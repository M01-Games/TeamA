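; Runs the two-stage weapon assembly minigame at a workbench: riveting the handle, then wrapping it.
; Riveting grades timing-bar hits by color zone, scores total hits against a perfect count, then attaches the handle and starts wrapping.
; Wrapping advances through either timed hits, scored on completion time, or alternating vertical mouse drags in Tick; both mark the weapon wrapped.
; A state enum tracks stages and lets unfinished riveting reset.
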(event Custom|StartMinigame%28%29
  (params (WorkBench :type Tyrell%20Workstation%20Object%20Reference) (Handle :type Handle%20BP%20Object%20Reference))
  (bind _output_get (Variables|Default|SetHandle Handle))
  (Rendering|SetVisibility (Variables|/Game/Tyrell_folder/Handle_BP.Handle_BP_C|GetNail_01 _output_get) true false)
  ;[0.15 0.15 0.15 0.5] This Is First Minigame
  (Rendering|SetVisibility (Variables|/Game/Tyrell_folder/Handle_BP.Handle_BP_C|GetNail_02 _output_get) true false)
  (Variables|Default|SetWork%20Bench WorkBench)
  (Variables|Default|SetCurrentState "NewEnumerator1")
  (bind _returnvalue (UserInterface|CreateWidget "/Game/Tyrell_folder/WBP_TimingBar.WBP_TimingBar_C" (Game|GetPlayerController 0)))
  (bind _output_get_2 (Variables|Default|SetTimingWidgetRef _returnvalue))
  (Variables|/Game/Tyrell_folder/WBP_TimingBar.WBP_TimingBar_C|SetHandleRef (Variables|Default|GetTimingWidgetRef) (Variables|Default|GetHandle))
  (UserInterface|Viewport|AddtoViewport _output_get_2 0)
  (Development|PrintString "add to viewport is runing"))

(event Custom|BeginRivet
  (params (Index :type Integer))
  (Variables|Default|SetCurrentRivetIndex Index)
  (Variables|Default|SetCurrentProgress 0)
  (Variables|Default|SetHitsThisRivet 0))

(event Custom|HandleWrapInput
  (bind _widgetwrappingref (Variables|Default|GetWidgetWrappingRef))
  (bind _widgetwrappingref_2 (Variables|Default|GetWidgetWrappingRef))
  (bind _work_bench (Variables|Default|GetWork%20Bench))
  (bind _weaponref (Variables|/Game/Blueprints/Tyrell_workstation.Tyrell_workstation_C|GetWeaponRef _work_bench))
  (if (Utilities|Enum|Equal(Enum) (Variables|Default|GetCurrentState) "NewEnumerator2")
    (Utilities|IsValid (Variables|Default|GetWidgetWrappingRef)
      (:Is%20Valid
        (bind _result (Default|EvaluateHit (Variables|Default|GetWidgetWrappingRef)))
        (switch Utilities|FlowControl|Switch|SwitchonEAccuracyZone _result
          (:NewEnumerator0
            (Variables|Default|SetPoints 10))
          (:NewEnumerator1
            (Variables|Default|SetPoints 20))
          (:NewEnumerator2
            (Variables|Default|SetPoints 50)))
        (bind _output_get (Variables|Default|SetCurrentProgress (+ (Variables|Default|GetCurrentProgress) (Variables|Default|GetPoints))))
        (Default|UpdateScoreUI (Variables|Default|GetWidgetWrappingRef))
        (Development|PrintString (Utilities|String|ToString(Integer) _output_get) true true "(R=0.501590,G=0.156199,B=1.000000,A=1.000000)" 2e+01)
        (bind _returnvalue (Actor|GetActorOfClass "/Game/Tyrell_folder/BPHandleAssembly.BPHandleAssembly_C"))
        (Default|UpDateMaterial _returnvalue)
        (if (>= (Variables|Default|GetCurrentProgress) 350)
          (Variables|/Game/Tyrell_folder/WBP_WrappingBar.WBP_WrappingBar_C|SetbGameActive (Variables|Default|GetWidgetWrappingRef) false)
          (Variables|Default|SetTimeRatio (Math|Float|Clamp(Float) (/ (- (Math|Conversions|ToFloat(Integer) (Variables|/Game/Tyrell_folder/WBP_WrappingBar.WBP_WrappingBar_C|GetSlowTime _widgetwrappingref_2)) (Variables|/Game/Tyrell_folder/WBP_WrappingBar.WBP_WrappingBar_C|GetTimeTaken _widgetwrappingref_2)) (- (Math|Conversions|ToFloat(Integer) (Variables|/Game/Tyrell_folder/WBP_WrappingBar.WBP_WrappingBar_C|GetSlowTime _widgetwrappingref)) (Math|Conversions|ToFloat(Integer) (Variables|/Game/Tyrell_folder/WBP_WrappingBar.WBP_WrappingBar_C|GetFastTime _widgetwrappingref))))))
          (bind _output_get_2 (Variables|Default|SetTimeScore (* (Variables|Default|GetTimeRatio) 1e+02)))
          (Development|PrintString (Utilities|String|ToString(Float) _output_get_2) true true "(R=1.000000,G=0.533699,B=0.063517,A=1.000000)" 2e+01)
          (Variables|Default|SetCurrentState "NewEnumerator3")
          (Variables|/Game/Connor_Folder/Blade/BP_BladeParent.BP_BladeParent_C|SetisBladeWrapped? _weaponref true)
          (Widget|RemovefromParent (Variables|Default|GetWidgetWrappingRef))
          (bind _output_get_3 (Variables|/Game/Connor_Folder/Blade/BP_BladeParent.BP_BladeParent_C|SetWrappingScore _weaponref (Math|Float|Truncate (Variables|Default|GetTimeScore))))
          (Development|PrintString (Utilities|String|ToString(Integer) _output_get_3) true true "(R=0.000000,G=1.000000,B=0.227971,A=1.000000)" 1e+02)))
      (:Is%20Not%20Valid
        (Development|PrintString "No Widget Ref")))))

(event Custom|HandleHitInput
  ;[0.15 0.15 0.15 0.5] this runs when i press P in widget WBP
  (if (not (Variables|/Game/Connor_Folder/Blade/BP_BladeParent.BP_BladeParent_C|GetIsBladeAttached? (Variables|/Game/Blueprints/Tyrell_workstation.Tyrell_workstation_C|GetWeaponRef (Variables|Default|GetWork%20Bench))))
    (Utilities|IsValid (Variables|Default|GetTimingWidgetRef)
      (:Is%20Valid
        (bind _result (Default|EvaluateHit (Variables|Default|GetTimingWidgetRef)))
        (switch Utilities|FlowControl|Switch|SwitchonEAccuracyZone _result
          (:NewEnumerator0
            (Variables|Default|SetPoints 1))
          (:NewEnumerator1
            (Variables|Default|SetPoints 3))
          (:NewEnumerator2
            (Variables|Default|SetPoints 5)))
        (Variables|Default|SetCurrentProgress (+ (Variables|Default|GetCurrentProgress) (Variables|Default|GetPoints)))
        (Variables|Default|SetHitsThisRivet (+ (Variables|Default|GetHitsThisRivet) 1))
        (if (>= (Variables|Default|GetCurrentProgress) 10)
          (Utilities|Array|Add (Variables|Default|GetRivetHits) (Variables|Default|GetHitsThisRivet))
          (Variables|Default|SetCurrentRivetIndex (+ (Variables|Default|GetCurrentRivetIndex) 1))
          (Variables|Default|SetCurrentProgress 0)
          (Variables|Default|SetHitsThisRivet 0)
          (if (>= (Variables|Default|GetCurrentRivetIndex) (Variables|Default|GetTotalRivets))
            (for _array_element (Variables|Default|GetRivetHits)
              (bind _output_get (Variables|Default|SetTotalSumOfHits (+ (Variables|Default|GetTotalSumOfHits) _array_element)))
              (Development|PrintString (Utilities|String|ToString(Integer) _output_get) true true "(R=1.000000,G=0.103228,B=0.208535,A=1.000000)" 2e+02))
            (Variables|Default|SetPerfectHits (* (Variables|Default|GetTotalRivets) 4))
            (Variables|Default|SetMaxHits (* (Variables|Default|GetTotalRivets) 10))
            (Variables|Default|SetErrorRatio (Math|Float|Clamp(Float) (/ (Math|Conversions|ToFloat(Integer) (- (Variables|Default|GetTotalSumOfHits) (Variables|Default|GetPerfectHits))) (Math|Conversions|ToFloat(Integer) (- (Variables|Default|GetMaxHits) (Variables|Default|GetPerfectHits))))))
            (Variables|Default|SetMinigameScore (Math|Conversions|ToFloat(Integer) (Class|KismetMathLibrary|ToInt64(Float) (Math|Float|Clamp(Float) (* (- 1.0 (Variables|Default|GetErrorRatio)) 1e+02) 0.0 1e+02))))
            (CallFunction|EndMinigame)
            (Default|AttachHandle (Variables|Default|GetWork%20Bench))
            (bind _returnvalue (Actor|GetActorOfClass "/Game/Tyrell_folder/BPHandleAssembly.BPHandleAssembly_C"))
            (Default|MaterialChange _returnvalue)
            (CallFunction|Wrappinggame)
            (else
              (Variables|Default|SetCurrentState "NewEnumerator1")))))
      (:Is%20Not%20Valid
        (Development|PrintString "No Widget Ref")))))

(event Custom|EndMinigame
  (Development|PrintString "Minigame is finished")
  (Development|PrintString (Utilities|String|ToString(Float) (Variables|Default|GetMinigameScore)))
  (Variables|Default|SetCurrentState "NewEnumerator2")
  (Widget|RemovefromParent (Variables|Default|GetTimingWidgetRef))
  (Variables|Default|SetCurrentRivetIndex 0)
  (Variables|Default|SetHitsThisRivet 0)
  (Variables|Default|SetCurrentProgress 0)
  (Variables|Default|SetTotalSumOfHits 0)
  (Utilities|Array|Clear (Variables|Default|GetRivetHits)))

(event Custom|Restart_minigame
  (bind _handle (Variables|Default|GetHandle))
  (if (Utilities|Enum|Equal(Enum) (Variables|Default|GetCurrentState) "NewEnumerator2")
    (Development|PrintString "User actually finished minigame")
    (else
      (Development|PrintString "Minigame didn't finish completely")
      (Variables|Default|SetCurrentState "NewEnumerator0")
      (Widget|RemovefromParent (Variables|Default|GetTimingWidgetRef))
      (Variables|Default|SetCurrentRivetIndex 0)
      (Variables|Default|SetHitsThisRivet 0)
      (Variables|Default|SetCurrentProgress 0)
      (Default|ResetAnimation (Variables|Default|GetHandle))
      (Rendering|SetVisibility (Variables|/Game/Tyrell_folder/Handle_BP.Handle_BP_C|GetNail_01 _handle) false false)
      (Rendering|SetVisibility (Variables|/Game/Tyrell_folder/Handle_BP.Handle_BP_C|GetNail_02 _handle) false false))))

(event Custom|AltF4
  (bind _widgetwrappingref (Variables|Default|GetWidgetWrappingRef))
  (bind _timingwidgetref (Variables|Default|GetTimingWidgetRef))
  (Utilities|IsValid _timingwidgetref
    (:Is%20Valid
      (Widget|RemovefromParent _timingwidgetref)
      (Utilities|IsValid _widgetwrappingref
        (:Is%20Valid
          (Widget|RemovefromParent _widgetwrappingref))))))

(event Custom|Wrappinggame
  (bind _returnvalue (Game|GetPlayerController 0))
  (Input|EnableInput _returnvalue)
  (Variables|Default|SetIsWrapping false)
  (Variables|Default|SetWrappingCurrentProgress 0.0)
  (Variables|/Script/Engine.PlayerController|SetbShowMouseCursor _returnvalue true)
  (Variables|Default|SetLastMouseY (.LocationY (Game|Player|GetMousePosition _returnvalue)))
  (bind _returnvalue_2 (UserInterface|CreateWidget "/Game/Tyrell_folder/WBP_WrappingBar.WBP_WrappingBar_C" (Game|GetPlayerController 0)))
  (bind _output_get (Variables|Default|SetWidgetWrappingRef _returnvalue_2))
  (UserInterface|Viewport|AddtoViewport _output_get 0)
  (Development|PrintString "WrappingMinigame now sarting"))

(event EventBeginPlay)

(event Collision|EventActorBeginOverlap
  (params (OtherActor :type Actor%20Object%20Reference)))

(event EventTick
  (params (DeltaSeconds :type Float%20%28single-precision%29))
  (bind _returnvalue (Game|GetPlayerController 0))
  (bind _returnvalue_2 (Game|GetPlayerController 0))
  (bind _work_bench (Variables|Default|GetWork%20Bench))
  (bind _work_bench_2 (Variables|Default|GetWork%20Bench))
  (bind _deltay (Class|PlayerController|GetInputMouseDelta _returnvalue))
  (bind _weaponref (Variables|/Game/Blueprints/Tyrell_workstation.Tyrell_workstation_C|GetWeaponRef _work_bench_2))
  (bind _weaponref_2 (Variables|/Game/Blueprints/Tyrell_workstation.Tyrell_workstation_C|GetWeaponRef _work_bench))
  (bind _returnvalue_3 (Math|Float|Absolute(Float) _deltay))
  (bind _returnvalue_4 (> _deltay 0.0))
  (Utilities|IsValid _work_bench_2
    (:Is%20Valid
      (Utilities|IsValid _weaponref
        (:Is%20Valid
          (if (not (Variables|/Game/Connor_Folder/Blade/BP_BladeParent.BP_BladeParent_C|GetisBladeWrapped? _weaponref))
            (Utilities|IsValid (Variables|Default|GetWidgetWrappingRef)
              (:Is%20Valid
                (Default|UpdateScoreUI (Variables|Default|GetWidgetWrappingRef)))
              (:Is%20Not%20Valid
                _))
            (if (>= (Variables|Default|GetWrappingCurrentProgress) 1.0)
              (Utilities|FlowControl|DoOnce false :!label _label
                (:Completed
                  (Input|DisableInput _returnvalue_2)
                  (Variables|/Script/Engine.PlayerController|SetbShowMouseCursor _returnvalue_2 false)
                  (Development|PrintString (Utilities|GetDisplayName _weaponref_2))
                  (Variables|/Game/Connor_Folder/Blade/BP_BladeParent.BP_BladeParent_C|SetisBladeWrapped? _weaponref_2 true)
                  (Widget|RemovefromParent (Variables|Default|GetWidgetWrappingRef))
                  (Utilities|FlowControl|Delay 0.2)
                  (Variables|Default|SetWrappingCurrentProgress 0.0)
                  (goto _label Reset)))
              (elif (Variables|Default|GetIsWrapping)
                (if (>= _returnvalue_3 (Variables|Default|GetMinDelta))
                  (if (== (Variables|Default|GetHasDirection) false)
                    (Variables|Default|SetWasMovingUp _returnvalue_4)
                    (Variables|Default|SetHasDirection true)
                    (elif (not (== _returnvalue_4 (Variables|Default|GetWasMovingUp)))
                      (Variables|Default|SetWasMovingUp _returnvalue_4)
                      (Variables|Default|SetWrappingCurrentProgress (Math|Float|Clamp(Float) (+ (Variables|Default|GetWrappingCurrentProgress) (* _returnvalue_3 (Variables|Default|GetProgressSpeed))))))))))))))))

(event Input|MouseEvents|LeftMouseButton
  (params (Key :type Key%20Structure :default "None"))
  (:Pressed
    (Variables|Default|SetIsWrapping true)
    (Variables|Default|SetLastMouseY (.LocationY (Game|Player|GetMousePosition (Game|GetPlayerController 0)))))
  (:Released
    (Variables|Default|SetIsWrapping false)))

(fn ConstructionScript)