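; Parent Blueprint for a craftable blade that is shaped by forging and sharpening and reports both results through GetBladeScore.
; The first morph target follows inverse ForgingProgress, while each remaining one is a sharpen point that accumulates clamped GrindPower.
; Construction creates dynamic materials for inner blade and edge from DT_Metal by MetalType.
; Tick re-reads the table and reapplies both materials, including heat, every frame.
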(event EventBeginPlay
  (bind _skeletalmesh (Variables|Default|GetSkeletalMesh))
  (bind _skeletalmeshasset (Variables|/Script/Engine.SkeletalMeshComponent|GetSkeletalMeshAsset _skeletalmesh))
  (Utilities|IsValid _skeletalmeshasset
    (:Is%20Valid
      (bind _output_get (Variables|Default|SetAllMorphTargets (Class|SkeletalMesh|GetAllMorphTargetNames _skeletalmeshasset)))
      (bind _output_get_2 (Variables|Default|SetForgeMorph (Utilities|Array|Get(acopy) _output_get)))
      (Components|SkeletalMesh|SetMorphTarget (Variables|Default|GetSkeletalMesh) (Utilities|String|StringToName _output_get_2) 1.0 true)
      (Utilities|Array|RemoveIndex _output_get)
      (for _array_element (Variables|Default|GetAllMorphTargets)
        (Utilities|Array|Add (Variables|Default|GetPoints) 0.0)))))

(event EventTick
  (params (DeltaSeconds :type Float%20%28single-precision%29))
  (CallFunction|SetInnerBladeInfofromDataTable)
  (CallFunction|ApplyInnerBladeInfofromDataTable)
  (CallFunction|SetBladeEdgeInfofromDataTable)
  (CallFunction|ApplyBladeEdgeInfofromDataTable))

(event EventForgeModel
  (Components|SkeletalMesh|SetMorphTarget (Variables|Default|GetSkeletalMesh) (Utilities|String|StringToName (Variables|Default|GetForgeMorph)) (- 1.0 (Variables|Default|GetforgingProgress)) true))

(event EventSharpen
  (params (GrindPower :type Float%20%28double-precision%29) (Index :type Integer))
  (bind _skeletalmesh (Variables|Default|GetSkeletalMesh))
  (Development|PrintString "Sharpened")
  (Utilities|IsValid (Variables|/Script/Engine.SkeletalMeshComponent|GetSkeletalMeshAsset _skeletalmesh)
    (:Is%20Valid
      (CallFunction|SharpenatPoint _skeletalmesh (Utilities|String|StringToName (Utilities|Array|Get(acopy) (Variables|Default|GetAllMorphTargets) Index)) Index GrindPower))))

(fn ConstructionScript
  (bind _skeletalmesh (Variables|Default|GetSkeletalMesh))
  (Utilities|FlowControl|Sequence
    (:then_0
      (bind _returnvalue (Rendering|Material|CreateDynamicMaterialInstance "/Game/Jack_Folder/Materials/Metal/MI_Metal_Default.MI_Metal_Default" "None" "None" :!class /Script/Engine.KismetMaterialLibrary))
      (Variables|Default|SetDMI%20Inner%20Blade _returnvalue)
      (Rendering|Material|SetMaterial (Variables|Default|GetSkeletalMesh) 2 (Variables|Default|GetDMI%20Inner%20Blade))
      (CallFunction|SetInnerBladeInfofromDataTable)
      (CallFunction|ApplyInnerBladeInfofromDataTable))
    (:then_1
      (bind _returnvalue_2 (Rendering|Material|CreateDynamicMaterialInstance "/Game/Jack_Folder/Materials/Metal/MI_Metal_Default.MI_Metal_Default" "None" "None" :!class /Script/Engine.KismetMaterialLibrary))
      (Variables|Default|SetDMI%20Blade%20Edge _returnvalue_2)
      (Rendering|Material|SetMaterial _skeletalmesh 0 (Variables|Default|GetDMI%20Blade%20Edge))
      (Rendering|Material|SetMaterial _skeletalmesh 1 (Variables|Default|GetDMI%20Blade%20Edge))
      (CallFunction|SetBladeEdgeInfofromDataTable)
      (CallFunction|ApplyBladeEdgeInfofromDataTable))))

(fn SharpenatPoint
  (params (Target :type Skeletal%20Mesh%20Component%20Object%20Reference) (MorphTargetName :type Name) (Index :type Integer) (GrindPower :type Float%20%28double-precision%29))
  (bind _points (Variables|Default|GetPoints))
  (bind _output (Utilities|Array|Get(acopy) _points Index))
  (bind _returnvalue (+ _output GrindPower))
  (bind _returnvalue_2 (Math|Float|Clamp(Float) _returnvalue 0.001))
  (Components|SkeletalMesh|SetMorphTarget Target MorphTargetName _returnvalue_2 true)
  (Utilities|Array|SetArrayElem (Variables|Default|GetPoints) Index _returnvalue_2))

(fn SetInnerBladeInfofromDataTable
  (bind _returnvalue (Utilities|GetDataTableRow "/Game/Jack_Folder/Materials/Metal/DT_Metal.DT_Metal" (Utilities|String|StringToName (Utilities|String|EnumtoString (Variables|Default|GetMetal%20Type))))
    (:then
      (bind _output_get (Variables|Default|SetMetal%20Data _returnvalue))
      (Variables|Default|SetMetallic (.metallic _output_get))
      (Variables|Default|SetRoughness (.roughness _output_get))
      (Variables|Default|SetInner%20Scratch%20Strength (.scratchstrength _output_get))
      (Variables|Default|SetScratch%20Tiling (.scratchtiling _output_get))
      (Variables|Default|SetScratch%20Colour%20Intensity (.scratchcolourintensity _output_get))
      (Variables|Default|SetGlow%20Boost (.glowboost _output_get))
      (Variables|Default|SetRim%20Light%20Intensity (.rimlightintensity _output_get))
      (Variables|Default|SetMetal%20Colour (.metalcolour _output_get))
      (Variables|Default|SetScratch%20Colour (.imperfectioncolour _output_get))
      (Variables|Default|SetRim%20Light%20Colour (.rimlightcolour _output_get)))
    (:RowNotFound
      (Development|PrintString "ROW NOT FOUND" true true "(R=1.000000,G=0.057958,B=0.000000,A=1.000000)" 1e+01))))

(fn ApplyInnerBladeInfofromDataTable
  (bind _dmi_inner_blade (Variables|Default|GetDMI%20Inner%20Blade))
  (Rendering|Material|SetScalarParameterValue _dmi_inner_blade "Metallic" (Variables|Default|GetMetallic) :!class /Script/Engine.MaterialInstanceDynamic)
  (Rendering|Material|SetScalarParameterValue _dmi_inner_blade "Roughness" (Variables|Default|GetRoughness) :!class /Script/Engine.MaterialInstanceDynamic)
  (Rendering|Material|SetScalarParameterValue _dmi_inner_blade "Scratch Strength" (Variables|Default|GetInner%20Scratch%20Strength) :!class /Script/Engine.MaterialInstanceDynamic)
  (Rendering|Material|SetScalarParameterValue _dmi_inner_blade "Scratch Tiling" (Variables|Default|GetScratch%20Tiling) :!class /Script/Engine.MaterialInstanceDynamic)
  (Rendering|Material|SetScalarParameterValue _dmi_inner_blade "Scratch Colour Intensity" (Variables|Default|GetScratch%20Colour%20Intensity) :!class /Script/Engine.MaterialInstanceDynamic)
  (Rendering|Material|SetScalarParameterValue _dmi_inner_blade "Heat Intensity" (Variables|Default|GetHeatIntensity) :!class /Script/Engine.MaterialInstanceDynamic)
  (Rendering|Material|SetScalarParameterValue _dmi_inner_blade "Glow Boost" (Variables|Default|GetGlow%20Boost) :!class /Script/Engine.MaterialInstanceDynamic)
  (Rendering|Material|SetScalarParameterValue _dmi_inner_blade "Rim Light Intensity" (Variables|Default|GetRim%20Light%20Intensity) :!class /Script/Engine.MaterialInstanceDynamic)
  (Rendering|Material|SetScalarParameterValue _dmi_inner_blade "Grain Strength" (Variables|Default|GetGrainStrength) :!class /Script/Engine.MaterialInstanceDynamic)
  (Rendering|Material|SetVectorParameterValue _dmi_inner_blade "Metal Colour" (Variables|Default|GetMetal%20Colour) :!class /Script/Engine.MaterialInstanceDynamic)
  (Rendering|Material|SetVectorParameterValue _dmi_inner_blade "Scratch Colour" (Variables|Default|GetScratch%20Colour) :!class /Script/Engine.MaterialInstanceDynamic)
  (Rendering|Material|SetVectorParameterValue _dmi_inner_blade "Rim Light Colour" (Variables|Default|GetRim%20Light%20Colour) :!class /Script/Engine.MaterialInstanceDynamic))

(fn ApplyBladeEdgeInfofromDataTable
  (bind _dmi_blade_edge (Variables|Default|GetDMI%20Blade%20Edge))
  (Rendering|Material|SetScalarParameterValue _dmi_blade_edge "Metallic" (Variables|Default|GetMetallic) :!class /Script/Engine.MaterialInstanceDynamic)
  (Rendering|Material|SetScalarParameterValue _dmi_blade_edge "Roughness" (Variables|Default|GetRoughness) :!class /Script/Engine.MaterialInstanceDynamic)
  (Rendering|Material|SetScalarParameterValue _dmi_blade_edge "Scratch Strength" (Variables|Default|GetBlade%20Scratch%20Strength) :!class /Script/Engine.MaterialInstanceDynamic)
  (Rendering|Material|SetScalarParameterValue _dmi_blade_edge "Scratch Tiling" (Variables|Default|GetScratch%20Tiling) :!class /Script/Engine.MaterialInstanceDynamic)
  (Rendering|Material|SetScalarParameterValue _dmi_blade_edge "Scratch Colour Intensity" (Variables|Default|GetScratch%20Colour%20Intensity) :!class /Script/Engine.MaterialInstanceDynamic)
  (Rendering|Material|SetScalarParameterValue _dmi_blade_edge "Heat Intensity" (Variables|Default|GetHeatIntensity) :!class /Script/Engine.MaterialInstanceDynamic)
  (Rendering|Material|SetScalarParameterValue _dmi_blade_edge "Glow Boost" (Variables|Default|GetGlow%20Boost) :!class /Script/Engine.MaterialInstanceDynamic)
  (Rendering|Material|SetScalarParameterValue _dmi_blade_edge "Rim Light Intensity" (Variables|Default|GetRim%20Light%20Intensity) :!class /Script/Engine.MaterialInstanceDynamic)
  (Rendering|Material|SetScalarParameterValue _dmi_blade_edge "Grain Strength" (Variables|Default|GetGrainStrength) :!class /Script/Engine.MaterialInstanceDynamic)
  (Rendering|Material|SetVectorParameterValue _dmi_blade_edge "Metal Colour" (Variables|Default|GetMetal%20Colour) :!class /Script/Engine.MaterialInstanceDynamic)
  (Rendering|Material|SetVectorParameterValue _dmi_blade_edge "Scratch Colour" (Variables|Default|GetScratch%20Colour) :!class /Script/Engine.MaterialInstanceDynamic)
  (Rendering|Material|SetVectorParameterValue _dmi_blade_edge "Rim Light Colour" (Variables|Default|GetRim%20Light%20Colour) :!class /Script/Engine.MaterialInstanceDynamic))

(fn SetBladeEdgeInfofromDataTable
  (bind _returnvalue (Utilities|GetDataTableRow "/Game/Jack_Folder/Materials/Metal/DT_Metal.DT_Metal" (Utilities|String|StringToName (Utilities|String|EnumtoString (Variables|Default|GetMetal%20Type))))
    (:then
      (bind _output_get (Variables|Default|SetMetal%20Data _returnvalue))
      (Variables|Default|SetMetallic (.metallic _output_get))
      (Variables|Default|SetRoughness (.roughness _output_get))
      (Variables|Default|SetScratch%20Tiling (.scratchtiling _output_get))
      (Variables|Default|SetScratch%20Colour%20Intensity (.scratchcolourintensity _output_get))
      (Variables|Default|SetGlow%20Boost (.glowboost _output_get))
      (Variables|Default|SetRim%20Light%20Intensity (.rimlightintensity _output_get))
      (Variables|Default|SetMetal%20Colour (.metalcolour _output_get))
      (Variables|Default|SetScratch%20Colour (.imperfectioncolour _output_get))
      (Variables|Default|SetRim%20Light%20Colour (.rimlightcolour _output_get)))
    (:RowNotFound
      (Development|PrintString "ROW NOT FOUND" true true "(R=1.000000,G=0.057958,B=0.000000,A=1.000000)" 1e+01))))

(fn GetBladeScore
  (return (Variables|Default|GetFinalForgeScore) (Variables|Default|GetPoints)))

(fn GetSpecificBlade
  (return 0))