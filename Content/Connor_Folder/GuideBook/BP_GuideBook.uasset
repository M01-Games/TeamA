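; Guide book actor that opens and closes through Enter and Exit events and lets the player flip through its pages.
; Enter and Exit toggle player input and play open or close animations, polling until any running open or close finishes.
; Horizontal IA_Move input steps a bounded page index, playing forward or backward animations from arrays.
; A DoOnce gate blocks further flips until a delay resets it.
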(event Custom|ResetAnim
  (bind _skeletalmesh (Variables|Default|GetSkeletalMesh))
  (bind _pages (Variables|Default|GetPages))
  (bind _pages_2 (Variables|Default|GetPages))
  (Utilities|FlowControl|DoOnce false) ; enters at Reset
)

(event Input|EnhancedActionEvents|EnhancedInputActionIA_Move
  (params (ActionValue :type Vector%202D%20Structure) (ElapsedSeconds :type Float%20%28double-precision%29) (TriggeredSeconds :type Float%20%28double-precision%29) (InputAction :type Input%20Action%20Object%20Reference :default "/Game/Input/Actions/IA_Move.IA_Move"))
  (bind _skeletalmesh (Variables|Default|GetSkeletalMesh))
  (bind _pages (Variables|Default|GetPages))
  (bind _pages_2 (Variables|Default|GetPages))
  (:Started
    (if (not (== (.x ActionValue) 0.0))
      (if (not (Variables|Default|GetInAnim))
        (Utilities|FlowControl|DoOnce false :!label _label
          (:Completed
            (Math|Float|CompareFloat (.x ActionValue) 0.0
              (:>
                (Development|PrintString (Utilities|String|ToString(Integer) (Variables|Default|GetPages)))
                (if (< _pages 4)
                  (Components|Animation|PlayAnimation _skeletalmesh (Utilities|Array|Get(acopy) (Variables|Default|GetForward) (Variables|Default|GetPages)) false)
                  (Math|Integer|IncrementInt _pages_2
                    (:%20%20
                      (Utilities|FlowControl|Delay 1.2 :!label _label_2)))))
              (:==
                (goto _label Reset))
              (:<
                (if (>= _pages 1)
                  (Components|Animation|PlayAnimation _skeletalmesh (Utilities|Array|Get(acopy) (Variables|Default|GetBackward) (- _pages 1)) false)
                  (Math|Integer|DecrementInt _pages_2
                    (:%20%20
                      (goto _label_2)))
                  (else
                    _))))
            (CallFunction|ResetAnim)))))))

(event EventEnter
  (params (Character :type Character%20Object%20Reference))
  (Variables|Default|SetEntered true)
  (Input|EnableInput (Game|GetPlayerController 0))
  (if (Variables|Default|GetInAnim) :!label _label
    (Utilities|FlowControl|RetriggerableDelay 0.05)
    (goto _label)
    (elif (and (Variables|Default|GetEntered) (not (Variables|Default|GetPlayedOpenA)))
      (Variables|Default|SetInAnim true)
      (Components|Animation|PlayAnimation (Variables|Default|GetSkeletalMesh) "/Game/Connor_Folder/GuideBook/NewBook/BOOKNEWOpen.BOOKNEWOpen" false)
      (Variables|Default|SetPlayedOpenA true)
      (Variables|Default|SetPages 0)
      (Utilities|FlowControl|Delay 0.6)
      (Variables|Default|SetInAnim false))))

(event EventExit
  (params (Character :type Character%20Object%20Reference))
  (Variables|Default|SetEntered false)
  (Input|DisableInput (Game|GetPlayerController 0))
  (if (Variables|Default|GetInAnim) :!label _label
    (Utilities|FlowControl|RetriggerableDelay 0.05)
    (goto _label)
    (elif (and (not (Variables|Default|GetEntered)) (Variables|Default|GetPlayedOpenA))
      (Variables|Default|SetInAnim true)
      (Components|Animation|PlayAnimation (Variables|Default|GetSkeletalMesh) "/Game/Connor_Folder/GuideBook/NewBook/BOOKNEWClose.BOOKNEWClose" false)
      (Variables|Default|SetPlayedOpenA false)
      (Utilities|FlowControl|Delay 0.6)
      (Variables|Default|SetInAnim false))))

(fn ConstructionScript)