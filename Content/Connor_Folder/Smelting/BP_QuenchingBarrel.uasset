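; Smelting quenching barrel that turns a full mould into the matching sword, axe or dagger blade, or a loose ingot.
; A half-second timer checks two child-actor item slots and accepts a mould only while the weapon slot is empty.
; Quenching triggers brief steam, deletes the mould and attaches any spawned blade to the weapon slot.
; DoOnce gates control re-triggering and restore slot positions, as the mould slot drops away after quenching.
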(event Custom|Checking
  (bind _mouldis (Variables|Default|GetMouldIS))
  (if (not (Variables|/Script/TeamA.ItemSlot|GetbIsOccupied (Variables|Default|GetWeaponIS)))
    (CallFunction|ResetMouldPos)
    (if (Variables|/Script/TeamA.ItemSlot|GetbIsOccupied _mouldis)
      (Utilities|FlowControl|DoOnce false :!label _label
        (:Completed
          (bind _asbp_mould (Utilities|Casting|CastToBP_Mould (Variables|/Script/TeamA.ItemSlot|GetAttachedItem _mouldis))
            (:then
              (if (Variables|/Game/Connor_Folder/PlaceHolder/BP_Mould.BP_Mould_C|GetFull _asbp_mould)
                (Components|Activation|Activate (Variables|Default|GetNS_SteamTest) true)
                (CallFunction|SpawnCorrectWeapon (Transformation|GetActorTransform) (Variables|/Game/Connor_Folder/PlaceHolder/BP_Mould.BP_Mould_C|GetMetal _asbp_mould) (Variables|/Game/Connor_Folder/PlaceHolder/BP_Mould.BP_Mould_C|GetMouldType _asbp_mould))
                (Transformation|SetRelativeLocation (Variables|Default|GetMould) "0.000000,0.000000,-1000.000000" false false)
                (Class|ItemSlot|DeleteItem (Variables|Default|GetMouldIS))
                (Utilities|FlowControl|Sequence
                  (:then_0
                    (goto _label Reset))
                  (:then_1
                    (Utilities|FlowControl|DoOnce false) ; enters at Reset
                  )
                  (:then_2
                    (Utilities|FlowControl|Delay 1.0)
                    (Components|Activation|Deactivate (Variables|Default|GetNS_SteamTest))))
                (else
                  (goto _label Reset))))
            (:CastFailed
              (goto _label Reset))))))))

(event Custom|Reset%20Mould%20Pos
  (Utilities|FlowControl|DoOnce false
    (:Completed
      (Transformation|SetRelativeLocation (Variables|Default|GetMould) "0, 0, 0" false false)
      (Transformation|SetRelativeLocation (Variables|Default|GetWeapon) "0, 0, 0" false false))))

(event Custom|SpawnCorrectWeapon
  (params (SpawnTransform :type Transform) (MetalType :type E_MetalType%20Enum :default "NewEnumerator0") (WeaponType :type WeaponTypes%20Enum :default "NewEnumerator0"))
  (bind (_location _rotation _scale) (Math|Transform|BreakTransform SpawnTransform))
  (switch Utilities|FlowControl|Switch|SwitchonWeaponTypes WeaponType
    (:NewEnumerator0
      (bind _returnvalue (Game|SpawnActorfromClass "/Game/Connor_Folder/Blade/BP_BladeSword.BP_BladeSword_C" SpawnTransform "AlwaysSpawn" "MultiplyWithRoot" 0 MetalType WeaponType 0))
      (Class|ItemSlot|AttachItem (Variables|Default|GetWeaponIS) _returnvalue))
    (:NewEnumerator1
      (bind _returnvalue_2 (Game|SpawnActorfromClass "/Game/Connor_Folder/PlaceHolder/BP_Blade.BP_Blade_C" SpawnTransform "AlwaysSpawn" "MultiplyWithRoot" 0 "" "" "NewEnumerator0" WeaponType 0))
      (Class|ItemSlot|AttachItem (Variables|Default|GetWeaponIS) _returnvalue_2)
      (Development|PrintString "Sorry. these dont exist"))
    (:NewEnumerator2
      (bind _returnvalue_3 (Game|SpawnActorfromClass "/Game/Connor_Folder/Blade/BP_BladeDagger.BP_BladeDagger_C" SpawnTransform "AlwaysSpawn" "MultiplyWithRoot" 0 MetalType WeaponType 0))
      (Class|ItemSlot|AttachItem (Variables|Default|GetWeaponIS) _returnvalue_3)
      (Transformation|SetRelativeLocation (Variables|Default|GetWeapon) "0.000000,0.000000,90.000000" false false))
    (:NewEnumerator3
      (Game|SpawnActorfromClass "/Game/Jack_Folder/Smelting/BP_Ore1.BP_Ore1_C" (Math|Transform|MakeTransform (+ _location "0.000000,0.000000,90.000000") _rotation _scale) "AlwaysSpawn" "MultiplyWithRoot" 0 MetalType true 0))))

(event EventBeginPlay
  (bind _asitem_slot (Utilities|Casting|CastToItemSlot (Variables|/Script/Engine.ChildActorComponent|GetChildActor (Variables|Default|GetMould))))
  (Variables|Default|SetMouldIS _asitem_slot)
  (bind _asitem_slot_2 (Utilities|Casting|CastToItemSlot (Variables|/Script/Engine.ChildActorComponent|GetChildActor (Variables|Default|GetWeapon))))
  (Variables|Default|SetWeaponIS _asitem_slot_2)
  (Utilities|Time|SetTimerbyEvent (delegate Custom|Checking) 0.5 true))

(fn ConstructionScript)