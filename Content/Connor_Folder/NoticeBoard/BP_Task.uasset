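; BP_Task is a notice board poster representing a job that can be picked up.
; On BeginPlay it creates a WB_OnBoardText widget from its Description and shows it on its widget component.
; SelectTask marks an untaken task as Taken and passes itself to the JobManager via PickUpPoster, printing a debug string either way.
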(event EventBeginPlay
  ;[0.15 0.15 0.15 0.5] Setting the text on the notice
  (bind _returnvalue (UserInterface|CreateWidget "/Game/Connor_Folder/NoticeBoard/WB_OnBoardText.WB_OnBoardText_C" 0 (Variables|Default|GetDescription)))
  (UserInterface|SetWidget (Variables|Default|GetWidget) _returnvalue))

(event EventSelectTask
  ;[0.15 0.15 0.15 0.5] Telling the job manager this job was selected
  (if (not (Variables|Default|GetTaken))
    (Variables|Default|SetTaken true)
    (Default|PickUpPoster (Variables|Default|GetJobManager) self)
    (Development|PrintString "YUP")
    (else
      (Development|PrintString "NOT"))))

(fn ConstructionScript)