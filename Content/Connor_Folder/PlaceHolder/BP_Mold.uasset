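; BP_Mold is a forgeable weapon piece whose skeletal mesh changes shape through morph targets as it is forged and sharpened.
; The first morph target fades out with ForgingProgress when ForgeModel runs.
; Sharpen accumulates clamped grind power per remaining morph target and lowers roughness on one of two dynamic edge materials.
; Tick, behind a two-second Delay, converts the weapon and metal selections into type strings.
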(event EventBeginPlay
  (bind _skeletalmesh (Variables|Default|GetSkeletalMesh))
  (bind _output_get (Variables|Default|SetAllMorphTargets (Class|SkeletalMesh|GetAllMorphTargetNames (Variables|/Script/Engine.SkeletalMeshComponent|GetSkeletalMeshAsset (Variables|Default|GetSkeletalMesh)))))
  (bind _output_get_2 (Variables|Default|SetForgeMorph (Utilities|Array|Get(acopy) _output_get)))
  (Components|SkeletalMesh|SetMorphTarget (Variables|Default|GetSkeletalMesh) (Utilities|String|StringToName _output_get_2) 1.0 true)
  (Utilities|Array|RemoveIndex _output_get)
  (for _array_element (Variables|Default|GetAllMorphTargets)
    (Utilities|Array|Add (Variables|Default|GetPoints) 0.0)
    (bind _returnvalue (Rendering|Material|CreateDynamicMaterialInstance _skeletalmesh 0 "/Game/Connor_Folder/PlaceHolder/Sword/MetalEdge.MetalEdge" "None" :!class /Script/Engine.PrimitiveComponent))
    (Variables|Default|SetEdgeMat1 _returnvalue)
    (bind _returnvalue_2 (Rendering|Material|CreateDynamicMaterialInstance _skeletalmesh 2 "/Game/Connor_Folder/PlaceHolder/Sword/MetalEdge.MetalEdge" "None" :!class /Script/Engine.PrimitiveComponent))
    (Variables|Default|SetEdgeMat2 _returnvalue_2)))

(event Collision|EventActorBeginOverlap
  (params (OtherActor :type Actor%20Object%20Reference)))

(event EventSharpen
  (params (GrindPower :type Float%20%28double-precision%29) (Index :type Integer))
  (CallFunction|AddtoMorphTargets (Variables|Default|GetSkeletalMesh) (Utilities|String|StringToName (Utilities|Array|Get(acopy) (Variables|Default|GetAllMorphTargets) Index)) Index GrindPower))

(event EventForgeModel
  (Components|SkeletalMesh|SetMorphTarget (Variables|Default|GetSkeletalMesh) (Utilities|String|StringToName (Variables|Default|GetForgeMorph)) (- 1.0 (Variables|Default|GetforgingProgress)) true))

(event EventTick
  (params (DeltaSeconds :type Float%20%28single-precision%29))
  (Utilities|FlowControl|Delay 2.0)
  (Utilities|FlowControl|Sequence
    (:then_0
      (switch Utilities|FlowControl|Switch|SwitchonWeaponTypes (Variables|Default|GetSetWeapon)
        (:NewEnumerator0
          (Variables|Default|SetWeaponType "Sword"))
        (:NewEnumerator1
          (Variables|Default|SetWeaponType "Axe"))
        (:NewEnumerator2
          (Variables|Default|SetWeaponType "Dagger"))))
    (:then_1
      (switch Utilities|FlowControl|Switch|SwitchonEnum_Metals (Variables|Default|GetSelectMetal)
        (:NewEnumerator0
          (Variables|Default|SetMetalType "Iron"))
        (:NewEnumerator1
          (Variables|Default|SetMetalType "Gold"))
        (:NewEnumerator2
          (Variables|Default|SetMetalType "Tungston"))
        (:NewEnumerator3
          (Variables|Default|SetMetalType "Copper"))))))

(fn ConstructionScript)

(fn AddtoMorphTargets
  (params (Target :type Skeletal%20Mesh%20Component%20Object%20Reference) (MorphTargetName :type Name) (Index :type Integer) (GrindPower :type Float%20%28double-precision%29))
  (bind _points (Variables|Default|GetPoints))
  (bind _output (Utilities|Array|Get(acopy) _points Index))
  (bind _returnvalue (+ _output GrindPower))
  (bind _returnvalue_2 (Math|Float|Clamp(Float) _returnvalue 0.001))
  (Components|SkeletalMesh|SetMorphTarget Target MorphTargetName _returnvalue_2 true)
  (Utilities|Array|SetArrayElem (Variables|Default|GetPoints) Index _returnvalue_2)
  (if (== Index 0)
    (LocalVariables|SetCurrent (Variables|Default|GetEdgeMat2))
    (else
      (LocalVariables|SetCurrent (Variables|Default|GetEdgeMat1))))
  (Rendering|Material|SetScalarParameterValue (LocalVariables|GetCurrent) "Roughness" (Math|Float|Lerp 0.4 0.25 (Math|Float|Clamp(Float) (/ (Utilities|Array|Get(acopy) _points Index) 1.0) 0.001)) :!class /Script/Engine.MaterialInstanceDynamic))