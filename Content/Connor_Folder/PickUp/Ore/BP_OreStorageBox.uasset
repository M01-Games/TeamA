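; BP_OreStorageBox is an ore storage box that dispenses one metal type from the player's owned ores.
; OreBox reads that type's count from InventoryManager.OresOwned, withdraws one if available, and returns the type, availability and spawn point.
; SpawnOre is a separate function that creates a BP_Ore at a given location.
; PickUp returns false, so the box itself cannot be picked up.
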(event EventBeginPlay)

(event Collision|EventActorBeginOverlap
  (params (OtherActor :type Actor%20Object%20Reference)))

(event EventTick
  (params (DeltaSeconds :type Float%20%28single-precision%29)))

(fn ConstructionScript)

(fn OreBox?
  (bind _whatboxisit_ (Variables|Default|GetWhatBoxIsIt?))
  (bind _inventorymanager (Variables|Default|GetInventoryManager))
  (bind _returnvalue (Utilities|String|EnumtoString _whatboxisit_))
  (bind _oresowned (Variables|/Game/Connor_Folder/PickUp/BP_InventoryManager.BP_InventoryManager_C|GetOresOwned _inventorymanager))
  (bind _keys (Utilities|Map|Keys _oresowned))
  (bind _values (Utilities|Map|Values _oresowned))
  (LocalVariables|SetCurrentInBox (Utilities|Array|Get(acopy) _values (Utilities|Array|FindItem _keys _returnvalue)))
  (if (> (LocalVariables|GetCurrentInBox) 0)
    (Class|BPIInventoryManager|TakeOutX(Message) (Variables|Default|GetInventoryManager) 1 _returnvalue))
  (return true _returnvalue (> (LocalVariables|GetCurrentInBox) 0) (Transformation|GetWorldLocation (Variables|Default|GetSpawnPoint))))

(fn PickUp
  (return false))

(fn SpawnOre
  (params (Ore :type String) (Location :type Vector :default "0, 0, 0"))
  (bind _returnvalue (Game|SpawnActorfromClass :Class "/Game/Connor_Folder/PickUp/Ore/BP_Ore.BP_Ore_C" :SpawnTransform (Math|Transform|MakeTransform Location "0, 0, 0" "1.000000,1.000000,1.000000") :CollisionHandlingOverride "AdjustIfPossibleButAlwaysSpawn" :TransformScaleMethod "MultiplyWithRoot" :Ore Ore :Instigator 0))
  (return _returnvalue))