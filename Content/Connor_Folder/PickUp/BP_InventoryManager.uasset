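; BP_InventoryManager is an inventory actor that tracks owned ores in the OresOwned map, keyed by metal name, and handles subtracting amounts.
; The TakeOutX event and RemoveOne function both subtract X by removing the key and re-adding it.
; Both use the value returned by Find as an index into the map's Values array, instead of as the count itself.
; RemoveOne computes the new amount before Remove, while TakeOutX computes it inline in Add.
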(event EventBeginPlay)

(event Collision|EventActorBeginOverlap
  (params (OtherActor :type Actor%20Object%20Reference)))

(event EventTick
  (params (DeltaSeconds :type Float%20%28single-precision%29)))

(event EventTakeOutX
  (params (X :type Integer) (MetalName :type String))
  (bind _oresowned (Variables|Default|GetOresOwned))
  (bind _values (Utilities|Map|Values _oresowned))
  (Utilities|Map|Remove _oresowned MetalName)
  (Utilities|Map|Add _oresowned MetalName (- (Utilities|Array|Get(acopy) _values (.Value (Utilities|Map|Find _oresowned MetalName))) X)))

(fn ConstructionScript)

(fn RemoveOne
  (params (Metal :type String) (X :type Integer))
  (bind _oresowned (Variables|Default|GetOresOwned))
  (bind _values (Utilities|Map|Values _oresowned))
  (LocalVariables|SetNewAmount (- (Utilities|Array|Get(acopy) _values (.Value (Utilities|Map|Find _oresowned Metal))) X))
  (Utilities|Map|Remove _oresowned Metal)
  (Utilities|Map|Add _oresowned Metal (LocalVariables|GetNewAmount)))