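; BP_MedievalLight is a light actor whose point light shows at night and hides during the day.
; On BeginPlay it finds the first BP_TimeManager in the level, binds ToggleLight to its OnDayNightStateChanged event and applies the current night state immediately.
; ToggleLight sets the point light's visibility from that state, so the light is event-driven and does not use Tick.
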(event Custom|ToggleLight
  (params (CurrentIsNight :type Boolean))
  (if CurrentIsNight
    (Rendering|SetVisibility (Variables|Default|GetPointLight) true false)
    (else
      (Rendering|SetVisibility (Variables|Default|GetPointLight) false false))))

(event EventBeginPlay
  (bind _outactors (Actor|GetAllActorsOfClass "/Game/Systems/Lighting/BP_TimeManager.BP_TimeManager_C"))
  (bind _output_get (Variables|Default|SetTimeManagerRef (Utilities|Array|Get(acopy) _outactors)))
  (EventDispatchers|BindEventtoOnDayNightStateChanged _output_get (delegate Custom|ToggleLight))
  (CallFunction|ToggleLight (Variables|/Game/Systems/Lighting/BP_TimeManager.BP_TimeManager_C|GetCurrentIsNight (Variables|Default|GetTimeManagerRef))))

(event Collision|EventActorBeginOverlap
  (params (OtherActor :type Actor%20Object%20Reference)))

(event EventTick
  (params (DeltaSeconds :type Float%20%28single-precision%29)))

(fn ConstructionScript)