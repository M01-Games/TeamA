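; BP_MetalTest is a test actor that previews data-driven metal looks on a cube.
; Its Construction Script creates a dynamic instance of MI_Metal_Default, then loads the DT_Metal row named by the MetalType enum.
; The loaded values drive surface, scratch, glow and rim light parameters on that instance.
; Scratch strength, heat intensity and grain strength come from Blueprint variables outside the table, and a missing row prints a warning.
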(event EventBeginPlay)

(fn ConstructionScript
  (bind _returnvalue (Rendering|Material|CreateDynamicMaterialInstance "/Game/Assets/Materials/Metal/MI_Metal_Default.MI_Metal_Default" "None" "None" :!class /Script/Engine.KismetMaterialLibrary))
  (bind _output_get (Variables|Default|SetMetal%20DMI _returnvalue))
  (Rendering|Material|SetMaterial (Variables|Default|GetCube) 0 _output_get)
  (CallFunction|SetMetalInfofromDataTable)
  (CallFunction|ApplyMetalInfofromDataTable))

(fn SetMetalInfofromDataTable
  (bind _returnvalue (Utilities|GetDataTableRow "/Game/Assets/Materials/Metal/DT_Metal.DT_Metal" (Utilities|String|StringToName (Utilities|String|EnumtoString (Variables|Default|GetMetal%20Type))))
    (:then
      (bind _output_get (Variables|Default|SetMetal%20Data _returnvalue))
      (Variables|Default|SetMetallic (.metallic _output_get))
      (Variables|Default|SetRoughness (.roughness _output_get))
      (Variables|Default|SetScratch%20Tiling (.scratchtiling _output_get))
      (Variables|Default|SetScratch%20Colour%20Intensity (.scratchcolourintensity _output_get))
      (Variables|Default|SetGlow%20Boost (.glowboost _output_get))
      (Variables|Default|SetRim%20Light%20Intensity (.rimlightintensity _output_get))
      (Variables|Default|SetMetal%20Colour (.metalcolour _output_get))
      (Variables|Default|SetScratch%20Colour (.imperfectioncolour _output_get))
      (Variables|Default|SetRim%20Light%20Colour (.rimlightcolour _output_get)))
    (:RowNotFound
      (Development|PrintString "ROW NOT FOUND" true true "(R=1.000000,G=0.057958,B=0.000000,A=1.000000)" 1e+01))))

(fn ApplyMetalInfofromDataTable
  (bind _metal_dmi (Variables|Default|GetMetal%20DMI))
  (Rendering|Material|SetScalarParameterValue _metal_dmi "Metallic" (Variables|Default|GetMetallic) :!class /Script/Engine.MaterialInstanceDynamic)
  (Rendering|Material|SetScalarParameterValue _metal_dmi "Roughness" (Variables|Default|GetRoughness) :!class /Script/Engine.MaterialInstanceDynamic)
  (Rendering|Material|SetScalarParameterValue _metal_dmi "Scratch Strength" (Variables|Default|GetScratch%20Strength) :!class /Script/Engine.MaterialInstanceDynamic)
  (Rendering|Material|SetScalarParameterValue _metal_dmi "Scratch Tiling" (Variables|Default|GetScratch%20Tiling) :!class /Script/Engine.MaterialInstanceDynamic)
  (Rendering|Material|SetScalarParameterValue _metal_dmi "Scratch Colour Intensity" (Variables|Default|GetScratch%20Colour%20Intensity) :!class /Script/Engine.MaterialInstanceDynamic)
  (Rendering|Material|SetScalarParameterValue _metal_dmi "Heat Intensity" (Variables|Default|GetHeat%20Intensity) :!class /Script/Engine.MaterialInstanceDynamic)
  (Rendering|Material|SetScalarParameterValue _metal_dmi "Glow Boost" (Variables|Default|GetGlow%20Boost) :!class /Script/Engine.MaterialInstanceDynamic)
  (Rendering|Material|SetScalarParameterValue _metal_dmi "Rim Light Intensity" (Variables|Default|GetRim%20Light%20Intensity) :!class /Script/Engine.MaterialInstanceDynamic)
  (Rendering|Material|SetScalarParameterValue _metal_dmi "Grain Strength" (Variables|Default|GetGrain%20Strength) :!class /Script/Engine.MaterialInstanceDynamic)
  (Rendering|Material|SetVectorParameterValue _metal_dmi "Metal Colour" (Variables|Default|GetMetal%20Colour) :!class /Script/Engine.MaterialInstanceDynamic)
  (Rendering|Material|SetVectorParameterValue _metal_dmi "Scratch Colour" (Variables|Default|GetScratch%20Colour) :!class /Script/Engine.MaterialInstanceDynamic)
  (Rendering|Material|SetVectorParameterValue _metal_dmi "Rim Light Colour" (Variables|Default|GetRim%20Light%20Colour) :!class /Script/Engine.MaterialInstanceDynamic))