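; OreContainer is a container actor that accepts one specific ore or item type through a BoxSlot child actor.
; The construction script writes the AcceptedSpecificType enum name to a TextRender label.
; On BeginPlay it casts the ChildActor to BoxSlot and passes AcceptedSpecificType to it.
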(event EventBeginPlay
  (bind _asbox_slot (Utilities|Casting|CastToBoxSlot (Variables|/Script/Engine.ChildActorComponent|GetChildActor (Variables|Default|GetChildActor))))
  (Variables|Default|SetAs%20Box%20Slot _asbox_slot)
  (Variables|/Script/TeamA.ItemSlot|SetAcceptedSpecificType (Variables|Default|GetAs%20Box%20Slot) (Variables|Default|GetAccepted%20Specific%20Type)))

(fn ConstructionScript
  (Rendering|Components|TextRender|SetText (Variables|Default|GetTextRender) (Utilities|Text|ToText(String) (Utilities|String|EnumtoString (Variables|Default|GetAccepted%20Specific%20Type)))))