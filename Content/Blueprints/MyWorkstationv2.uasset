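; An interactive workstation with a spinnable wheel and cursor-driven placement of an inventory item.
; Enter stores the character, enables input and shows the mouse cursor; Exit reverses the input and cursor changes.
; Jump input adds clamped spin, and a timeline rotates Spinny's roll, replaying itself with decreasing spin until it reaches zero.
; Mouse look moves the first inventory item's collision mesh to the cursor trace hit within range of the Arrow.
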(event Custom|ContinueSpin
  (Variables|Default|SetWheelRot (Transformation|GetWorldRotation (Variables|Default|GetSpinny)))
  (bind _alpha (Timeline|Timeline PlayFromStart)
    (:Update
      (Transformation|SetWorldRotation (Variables|Default|GetSpinny) (Math|Rotator|Lerp(Rotator) (Variables|Default|GetWheelRot) (Math|Rotator|MakeRotator (+ (.Roll (Math|Rotator|BreakRotator (Variables|Default|GetWheelRot))) (Variables|Default|GetSpinValue)) (.Pitch (Math|Rotator|BreakRotator (Variables|Default|GetWheelRot))) (.Yaw (Math|Rotator|BreakRotator (Variables|Default|GetWheelRot)))) _alpha true) false false))
    (:Finished
      (if (> (Variables|Default|GetSpinValue) 0.0)
        (Variables|Default|SetSpinValue (Math|Float|Clamp(Float) (- (Variables|Default|GetSpinValue) 1e+01) 0.0 1.7e+02))
        (CallFunction|ContinueSpin)))))

(event Input|EnhancedActionEvents|EnhancedInputActionIA_Jump
  (params (ActionValue :type Boolean) (ElapsedSeconds :type Float%20%28double-precision%29) (TriggeredSeconds :type Float%20%28double-precision%29) (InputAction :type Input%20Action%20Object%20Reference :default "/Game/Input/Actions/IA_Jump.IA_Jump"))
  (:Started
    (Development|PrintString "Hello")
    (Variables|Default|SetSpinValue (Math|Float|Clamp(Float) (+ (Variables|Default|GetSpinValue) 1e+01) 0.0 1.7e+02))
    (Variables|Default|SetWheelRot (Transformation|GetWorldRotation (Variables|Default|GetSpinny)))
    (bind _alpha (Timeline|Timeline PlayFromStart)
      (:Update
        (Transformation|SetWorldRotation (Variables|Default|GetSpinny) (Math|Rotator|Lerp(Rotator) (Variables|Default|GetWheelRot) (Math|Rotator|MakeRotator (+ (.Roll (Math|Rotator|BreakRotator (Variables|Default|GetWheelRot))) (Variables|Default|GetSpinValue)) (.Pitch (Math|Rotator|BreakRotator (Variables|Default|GetWheelRot))) (.Yaw (Math|Rotator|BreakRotator (Variables|Default|GetWheelRot)))) _alpha true) false false))
      (:Finished
        (if (> (Variables|Default|GetSpinValue) 0.0)
          (Variables|Default|SetSpinValue (Math|Float|Clamp(Float) (- (Variables|Default|GetSpinValue) 1e+01) 0.0 1.7e+02))
          (CallFunction|ContinueSpin))))))

(event Input|EnhancedActionEvents|EnhancedInputActionIA_MouseLook
  (params (ActionValue :type Vector%202D%20Structure) (ElapsedSeconds :type Float%20%28double-precision%29) (TriggeredSeconds :type Float%20%28double-precision%29) (InputAction :type Input%20Action%20Object%20Reference :default "/Game/Input/Actions/IA_MouseLook.IA_MouseLook"))
  (bind _returnvalue (Game|GetPlayerController 0))
  (bind _inventory (Variables|Default|GetInventory))
  (bind (_hitresult _returnvalue_2) (Game|Player|GetHitResultUnderCursorbyChannel _returnvalue "TraceTypeQuery1" true))
  (bind _output (Utilities|Array|Get(acopy) _inventory))
  (:Triggered
    (Utilities|IsValid _output
      (:Is%20Valid
        (if _returnvalue_2
          (if (not (> (Math|Vector|Distance(Vector) (.location _hitresult) (Transformation|GetWorldLocation (Variables|Default|GetArrow))) 4e+02))
            (Transformation|SetWorldLocation (Variables|/Script/TeamA.Pickup|GetCollisionMesh _output) (.location _hitresult) false false)))))))

(event Input|EnhancedActionEvents|EnhancedInputActionIA_Move
  (params (ActionValue :type Vector%202D%20Structure) (ElapsedSeconds :type Float%20%28double-precision%29) (TriggeredSeconds :type Float%20%28double-precision%29) (InputAction :type Input%20Action%20Object%20Reference :default "/Game/Input/Actions/IA_Move.IA_Move")))

(event EventBeginPlay)

(event Collision|EventActorBeginOverlap
  (params (OtherActor :type Actor%20Object%20Reference)))

(event EventTick
  (params (DeltaSeconds :type Float%20%28single-precision%29)))

(event EventEnter
  (params (Character :type Character%20Object%20Reference))
  (bind _returnvalue (Game|GetPlayerController 0))
  (Variables|Default|SetCharacter Character)
  (Development|PrintString (Utilities|GetDisplayName (Utilities|Array|Get(acopy) (Variables|Default|GetInventory))))
  (Input|EnableInput _returnvalue)
  (Variables|/Script/Engine.PlayerController|SetbShowMouseCursor _returnvalue true))

(event EventExit
  (params (Character :type Character%20Object%20Reference))
  (bind _returnvalue (Game|GetPlayerController 0))
  (Input|DisableInput _returnvalue)
  (Variables|/Script/Engine.PlayerController|SetbShowMouseCursor _returnvalue false))

(fn ConstructionScript)

(fn LowerSpinValue
  (params (Alpha :type Float%20%28double-precision%29)))