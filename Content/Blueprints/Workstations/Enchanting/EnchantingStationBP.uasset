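; EnchantingStationBP is an enchanting workstation Blueprint that so far contains only cursor-movement input handling.
; While IA_MoveMouse triggers, it offsets player 0's mouse position on X and Y by a scaled axis key value.
; The offset comes from GetInputAxisKeyValue with no key shown, rather than the action's value.
; A debug string prints on each trigger; other events and the construction script are empty.
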(event Input|EnhancedActionEvents|EnhancedInputActionIA_MoveMouse
  (params (ActionValue :type Boolean) (ElapsedSeconds :type Float%20%28double-precision%29) (TriggeredSeconds :type Float%20%28double-precision%29) (InputAction :type Input%20Action%20Object%20Reference :default "/Game/Input/Actions/IA_MoveMouse.IA_MoveMouse"))
  (bind _returnvalue (Game|GetPlayerController 0))
  (bind (_locationx _locationy) (Game|Player|GetMousePosition _returnvalue))
  (:Triggered
    (Development|PrintString "StillGoin" true true "(R=0.000000,G=0.660000,B=1.000000,A=1.000000)" 0.1)
    (Class|PlayerController|SetMouseLocation (Game|GetPlayerController 0) (Math|Float|Round (+ _locationx (* (Class|Actor|GetInputAxisKeyValue) 1e+01))) (Math|Float|Round (+ _locationy (* (Class|Actor|GetInputAxisKeyValue) 1e+01))))))

(event EventBeginPlay)

(event Collision|EventActorBeginOverlap
  (params (OtherActor :type Actor%20Object%20Reference)))

(event EventTick
  (params (DeltaSeconds :type Float%20%28single-precision%29)))

(fn ConstructionScript)