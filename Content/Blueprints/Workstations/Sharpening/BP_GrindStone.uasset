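; Grindstone workstation where the player pumps left/right inputs to spin the wheel and sharpen the blade placed on it.
; Entering shows a sharpen widget, starts a looping spin decay and lets a forged blade follow the cursor; move input flips it.
; A self-retriggering capsule trace, faster at higher spin, maps component tags to blade sections, sends SharpenMessage with spin-scaled power and activates sparks.
; Grinding near top speed adds blade scratches.
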(event Custom|ContinueSpin
  (Variables|Default|SetWheelRot (Transformation|GetWorldRotation (Variables|Default|GetSpinny)))
  (bind _alpha (Timeline|Timeline PlayFromStart)
    (:Update
      (Transformation|SetWorldRotation (Variables|Default|GetSpinny) (Math|Rotator|Lerp(Rotator) (Variables|Default|GetWheelRot) (Math|Rotator|MakeRotator (+ (.Roll (Math|Rotator|BreakRotator (Variables|Default|GetWheelRot))) (Variables|Default|GetSpinValue)) (.Pitch (Math|Rotator|BreakRotator (Variables|Default|GetWheelRot))) (.Yaw (Math|Rotator|BreakRotator (Variables|Default|GetWheelRot)))) _alpha true) false false))
    (:Finished
      (if (> (Variables|Default|GetSpinValue) 0.0)
        (CallFunction|ContinueSpin)))))

(event Custom|OpenGate
  (bind _returnvalue (Game|GetPlayerController 0))
  (bind _inventory (Variables|Default|GetInventory))
  (bind _blade (Variables|Default|GetBlade))
  (bind (_hitresult _returnvalue_2) (Game|Player|GetHitResultUnderCursorbyChannel _returnvalue "TraceTypeQuery1" true))
  (bind _output (Utilities|Array|Get(acopy) _inventory))
  (bind _interactionvolume (Variables|/Script/TeamA.Pickup|GetInteractionVolume _output))
  (Utilities|FlowControl|Gate true) ; enters at Open
)

(event Custom|CloseGate
  (bind _returnvalue (Game|GetPlayerController 0))
  (bind _inventory (Variables|Default|GetInventory))
  (bind _blade (Variables|Default|GetBlade))
  (bind (_hitresult _returnvalue_2) (Game|Player|GetHitResultUnderCursorbyChannel _returnvalue "TraceTypeQuery1" true))
  (bind _output (Utilities|Array|Get(acopy) _inventory))
  (bind _interactionvolume (Variables|/Script/TeamA.Pickup|GetInteractionVolume _output))
  (Utilities|FlowControl|Sequence
    (:then_0
      (Utilities|FlowControl|Gate true) ; enters at Close
    )
    (:then_1
      (Utilities|FlowControl|Delay 0.01)
      (Utilities|IsValid _output
        (:Is%20Valid
          (Transformation|SetWorldLocation _interactionvolume (Transformation|GetWorldLocation (Variables|Default|GetItem)) false false)
          (Transformation|SetWorldRotation _interactionvolume "0, 0, 0" false false)
          (Utilities|FlowControl|DoOnce false) ; enters at Reset
        )))))

(event Custom|Trigger%20Sharpen
  (Utilities|FlowControl|DoOnce true
    (:Completed
      (Utilities|FlowControl|Delay (Math|Float|Clamp(Float) (/ 4e+01 (Variables|Default|GetSpinValue)) 0.0 2.0))
      (if (> (Variables|Default|GetSpinValue) 0.0)
        (CallFunction|LineTraceGrind)
        (CallFunction|ResetSharpen)
        (CallFunction|TriggerSharpen)
        (Utilities|FlowControl|RetriggerableDelay 2.3)
        (Components|Activation|Deactivate (Variables|Default|GetSparks))
        (else
          (CallFunction|ResetSharpen))))))

(event Custom|ResetSharpen
  (Utilities|FlowControl|DoOnce true) ; enters at Reset
)

(event Custom|Turn
  (bind _inventory (Variables|Default|GetInventory))
  (bind _output (Utilities|Array|Get(acopy) _inventory))
  (Utilities|IsValid _output
    (:Is%20Valid
      (Variables|Default|SetInventRot (Transformation|GetActorRotation _output))
      (bind _alpha (Timeline|Timeline_0 PlayFromStart)
        (:Update
          (Utilities|IsValid _output
            (:Is%20Valid
              (Transformation|SetActorRotation _output (Math|Rotator|Lerp(Rotator) (Variables|Default|GetInventRot) (Math|Rotator|MakeRotator (.Roll (Math|Rotator|BreakRotator (Variables|Default|GetInventRot))) (+ (.Pitch (Math|Rotator|BreakRotator (Variables|Default|GetInventRot))) 1.8e+02) (.Yaw (Math|Rotator|BreakRotator (Variables|Default|GetInventRot)))) _alpha true)))))))))

(event Custom|Lower
  (Variables|Default|SetSpinValue (Math|Float|Clamp(Float) (- (Variables|Default|GetSpinValue) 0.3) 0.0 1.7e+02)))

(event Input|EnhancedActionEvents|EnhancedInputActionIA_Right
  (params (ActionValue :type Boolean) (ElapsedSeconds :type Float%20%28double-precision%29) (TriggeredSeconds :type Float%20%28double-precision%29) (InputAction :type Input%20Action%20Object%20Reference :default "/Game/Input/Actions/IA_Right.IA_Right"))
  (:Started
    (if (Variables|Default|GetA)
      (Variables|Default|SetA false)
      (Development|PrintString "Hello")
      (CallFunction|TriggerSharpen)
      (Utilities|FlowControl|Delay 0.1)
      (CallFunction|ResetSharpen)
      (Variables|Default|SetSpinValue (Math|Float|Clamp(Float) (+ (Variables|Default|GetSpinValue) 4.0) 0.0 1.7e+02))
      (Variables|Default|SetWheelRot (Transformation|GetWorldRotation (Variables|Default|GetSpinny)))
      (bind _alpha (Timeline|Timeline PlayFromStart)
        (:Update
          (Transformation|SetWorldRotation (Variables|Default|GetSpinny) (Math|Rotator|Lerp(Rotator) (Variables|Default|GetWheelRot) (Math|Rotator|MakeRotator (+ (.Roll (Math|Rotator|BreakRotator (Variables|Default|GetWheelRot))) (Variables|Default|GetSpinValue)) (.Pitch (Math|Rotator|BreakRotator (Variables|Default|GetWheelRot))) (.Yaw (Math|Rotator|BreakRotator (Variables|Default|GetWheelRot)))) _alpha true) false false))
        (:Finished
          (if (> (Variables|Default|GetSpinValue) 0.0)
            (CallFunction|ContinueSpin)))))))

(event Input|EnhancedActionEvents|EnhancedInputActionIA_Left
  (params (ActionValue :type Float%20%28double-precision%29) (ElapsedSeconds :type Float%20%28double-precision%29) (TriggeredSeconds :type Float%20%28double-precision%29) (InputAction :type Input%20Action%20Object%20Reference :default "/Game/Input/Actions/IA_Left.IA_Left"))
  (:Started
    (if (not (Variables|Default|GetA))
      (Variables|Default|SetA true)
      (Development|PrintString "Hello")
      (CallFunction|TriggerSharpen)
      (Utilities|FlowControl|Delay 0.1)
      (CallFunction|ResetSharpen)
      (Variables|Default|SetSpinValue (Math|Float|Clamp(Float) (+ (Variables|Default|GetSpinValue) 4.0) 0.0 1.7e+02))
      (Variables|Default|SetWheelRot (Transformation|GetWorldRotation (Variables|Default|GetSpinny)))
      (bind _alpha (Timeline|Timeline PlayFromStart)
        (:Update
          (Transformation|SetWorldRotation (Variables|Default|GetSpinny) (Math|Rotator|Lerp(Rotator) (Variables|Default|GetWheelRot) (Math|Rotator|MakeRotator (+ (.Roll (Math|Rotator|BreakRotator (Variables|Default|GetWheelRot))) (Variables|Default|GetSpinValue)) (.Pitch (Math|Rotator|BreakRotator (Variables|Default|GetWheelRot))) (.Yaw (Math|Rotator|BreakRotator (Variables|Default|GetWheelRot)))) _alpha true) false false))
        (:Finished
          (if (> (Variables|Default|GetSpinValue) 0.0)
            (CallFunction|ContinueSpin)))))))

(event Input|EnhancedActionEvents|EnhancedInputActionIA_Move
  (params (ActionValue :type Vector%202D%20Structure) (ElapsedSeconds :type Float%20%28double-precision%29) (TriggeredSeconds :type Float%20%28double-precision%29) (InputAction :type Input%20Action%20Object%20Reference :default "/Game/Input/Actions/IA_Move.IA_Move"))
  (:Started
    (Math|Float|CompareFloat (.Y (Math|Vector2D|BreakVector2D ActionValue)) 0.0
      (:>
        _)
      (:<
        _))
    (Utilities|FlowControl|DoOnce false :!label _label
      (:Completed
        (CallFunction|Turn)
        (Utilities|FlowControl|Delay 1.0)
        (goto _label Reset)))))

(event Input|EnhancedActionEvents|EnhancedInputActionIA_MoveMouse
  (params (ActionValue :type Boolean) (ElapsedSeconds :type Float%20%28double-precision%29) (TriggeredSeconds :type Float%20%28double-precision%29) (InputAction :type Input%20Action%20Object%20Reference :default "/Game/Input/Actions/IA_MoveMouse.IA_MoveMouse"))
  (bind _returnvalue (Game|GetPlayerController 0))
  (bind (_locationx _locationy) (Game|Player|GetMousePosition _returnvalue))
  (:Triggered
    (Class|PlayerController|SetMouseLocation (Game|GetPlayerController 0) (Math|Float|Round (+ _locationx (* (Class|Actor|GetInputAxisKeyValue) 1e+01))) (Math|Float|Round (+ _locationy (* (Class|Actor|GetInputAxisKeyValue) 1e+01))))))

(event EventBeginPlay
  (bind _asitem_slot (Utilities|Casting|CastToItemSlot (Variables|/Script/Engine.ChildActorComponent|GetChildActor (Variables|Default|GetItem))))
  (Variables|Default|SetAs%20Item%20Slot _asitem_slot))

(event EventEnter
  (params (Character :type Character%20Object%20Reference))
  (bind _returnvalue (Game|GetPlayerController 0))
  (bind _returnvalue_2 (Viewport|GetViewportSize))
  (bind _inventory (Variables|Default|GetInventory))
  (bind _output (Utilities|Array|Get(acopy) _inventory))
  (Variables|Default|SetCharacter Character)
  (Utilities|IsValid _output
    (:Is%20Valid
      (bind _asbp_blade_parent (Utilities|Casting|CastToBP_BladeParent _output))
      (Variables|Default|SetBlade _asbp_blade_parent))
    (:Is%20Not%20Valid
      _))
  (bind _returnvalue_3 (UserInterface|CreateWidget "/Game/Blueprints/Workstations/Sharpening/WB_Sharpen.WB_Sharpen_C" 0 self))
  (bind _output_get (Variables|Default|SetWB_Sharpen _returnvalue_3))
  (UserInterface|Viewport|AddtoViewport _output_get 0)
  (Input|EnableInput _returnvalue)
  (Variables|/Script/Engine.PlayerController|SetbShowMouseCursor _returnvalue false)
  (CallFunction|OpenGate)
  (bind _returnvalue_4 (Utilities|Time|SetTimerbyEvent (delegate Custom|Lower) 0.1 true))
  (Variables|Default|SetTimerHandle _returnvalue_4)
  (Class|PlayerController|SetMouseLocation (Game|GetPlayerController 0) (Math|Float|Truncate (/ (.x _returnvalue_2) 2.0)) (Math|Float|Truncate (/ (.y _returnvalue_2) 2.0))))

(event EventExit
  (params (Character :type Character%20Object%20Reference))
  (bind _returnvalue (Game|GetPlayerController 0))
  (Input|DisableInput _returnvalue)
  (Variables|/Script/Engine.PlayerController|SetbShowMouseCursor _returnvalue false)
  (CallFunction|CloseGate)
  (Widget|RemovefromParent (Variables|Default|GetWB_Sharpen)))

(event EventTick
  (params (DeltaSeconds :type Float%20%28single-precision%29))
  (bind _returnvalue (Game|GetPlayerController 0))
  (bind _inventory (Variables|Default|GetInventory))
  (bind _blade (Variables|Default|GetBlade))
  (bind (_hitresult _returnvalue_2) (Game|Player|GetHitResultUnderCursorbyChannel _returnvalue "TraceTypeQuery1" true))
  (bind _output (Utilities|Array|Get(acopy) _inventory))
  (bind _interactionvolume (Variables|/Script/TeamA.Pickup|GetInteractionVolume _output))
  (Utilities|FlowControl|Gate true
    (:Exit
      (Utilities|IsValid _blade
        (:Is%20Valid
          (if (Variables|/Script/TeamA.Project|GetbIsForged _blade)
            (Utilities|IsValid _output
              (:Is%20Valid
                (if _returnvalue_2
                  (if (not (> (Math|Vector|Distance(Vector) (.location _hitresult) (Transformation|GetWorldLocation (Variables|Default|GetArrow))) 4e+02))
                    (Transformation|SetWorldLocation _interactionvolume (.location _hitresult) false false)
                    (Utilities|FlowControl|DoOnce false
                      (:Completed
                        (Transformation|SetWorldRotation _interactionvolume "-30.000000,0.000000,0.000000" false false)))))))))))))

(fn ConstructionScript)

(fn RotateProject
  (params (X? :type Boolean) (Value :type Float%20%28double-precision%29))
  (bind _inventory (Variables|Default|GetInventory))
  (bind _output (Utilities|Array|Get(acopy) _inventory))
  (Utilities|IsValid _output
    (:Is%20Valid
      (if X?
        (Class|Actor|AddActorWorldRotation _output (Math|Rotator|MakeRotator 1.8e+02 0.0 (* (* 1.8e+02 Value) -1.0)))))))

(fn LineTraceGrind
  (bind _grindpoint (Variables|Default|GetGrindPoint))
  (bind _blade (Variables|Default|GetBlade))
  (bind _returnvalue (Transformation|GetWorldLocation _grindpoint))
  (bind _outhit (Class|KismetSystemLibrary|CapsuleTraceSingleforObjects _returnvalue _returnvalue 5.0 3e+01 (LocalVariables|GetObjects%20to%20look%20for) false 0 "None" true "(R=1.000000,G=0.000000,B=0.000000,A=1.000000)" "(R=0.000000,G=1.000000,B=0.000000,A=1.000000)" 0.15))
  (if (or (.bBlockingHit (Collision|BreakHitResult _outhit)) (.bInitialOverlap (Collision|BreakHitResult _outhit)))
    (bind _output_get (LocalVariables|SetTags (Variables|/Script/Engine.ActorComponent|GetComponentTags (.HitComponent (Collision|BreakHitResult _outhit)))))
    (switch name (Utilities|Array|Get(acopy) _output_get)
      (:1
        (LocalVariables|SetIndex 0))
      (:2
        (LocalVariables|SetIndex 1))
      (:3
        (LocalVariables|SetIndex 2))
      (:4
        (LocalVariables|SetIndex 3))
      (:5
        (LocalVariables|SetIndex 4))
      (:6
        (LocalVariables|SetIndex 5))
      (:7
        (LocalVariables|SetIndex 6)))
    (Class|BPISharpen|Sharpen(Message) (Components|GetOwner (.HitComponent (Collision|BreakHitResult _outhit))) (/ (Variables|Default|GetSpinValue) 5.1e+03) (LocalVariables|GetIndex) (Variables|Default|GetWB_Sharpen))
    (Components|Activation|Activate (Variables|Default|GetSparks) true)
    (if (> (/ (Variables|Default|GetSpinValue) 1.7e+02) 0.85)
      (Variables|/Game/Blueprints/Weapons/BP_BladeParent.BP_BladeParent_C|SetBlade%20Scratch%20Strength _blade (+ (Variables|/Game/Blueprints/Weapons/BP_BladeParent.BP_BladeParent_C|GetBlade%20Scratch%20Strength _blade) 0.3)))
    (else
      (Components|Activation|Deactivate (Variables|Default|GetSparks)))))