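; Runs the weapon polishing minigame, where the player holds left mouse and wipes across the weapon's PolishHitBox.
; Tick traces under the cursor, turning wipe distance into Progress that drives the PolishAmount material parameter and polishing widget.
; Fast wipes build Heat, which reduces efficiency past an overheat threshold.
; Completion stores a time-based score and marks the weapon polished; Start and Restart events handle setup, already-polished notices and resets.
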(event Custom|StartMinigame
  (params (CurrentWeaponRef :type BP%20Blade%20Parent%20Object%20Reference))
  (bind _returnvalue (Rendering|Material|CreateDynamicMaterialInstance (Variables|/Script/TeamA.Project|GetSkeletalMesh CurrentWeaponRef) 0 0 "None" :!class /Script/Engine.PrimitiveComponent))
  (Variables|/Game/Blueprints/Weapons/BP_BladeParent.BP_BladeParent_C|SetPolishMID CurrentWeaponRef _returnvalue)
  (if (Variables|/Game/Blueprints/Weapons/BP_BladeParent.BP_BladeParent_C|GetIsPolishingDone? CurrentWeaponRef)
    (Development|PrintString "weapon is done on enter")
    (bind _returnvalue_2 (UserInterface|CreateWidget "/Game/Blueprints/Workstations/Assembly/WBP_StageChecker.WBP_StageChecker_C" (Game|GetPlayerController 0)))
    (bind _output_get (Variables|/Game/Blueprints/Workstations/Polishing/Polishing_Workstation.Polishing_Workstation_C|SetStageText (Variables|Default|GetPolishingRef) _returnvalue_2))
    (Default|ChangeText _output_get "Weapon Is Already Polished")
    (UserInterface|Viewport|AddtoViewport _output_get 0)
    (else
      (Variables|Default|SetProgress 0.0)
      (Variables|Default|SetTimeTaken 0.0)
      (Variables|Default|SetHeat 0.0)
      (UserInterface|Viewport|AddtoViewport (Variables|Default|GetPolishingWidgetRef) 0)
      (bind _output_get_2 (Variables|Default|SetWeaponRef CurrentWeaponRef))
      (Development|PrintString (Utilities|GetDisplayName _output_get_2))
      (Input|EnableInput (Game|GetPlayerController 0))
      (Variables|Default|SetbMinigameActive true)
      (Collision|SetCollisionResponsetoChannel (Variables|/Game/Blueprints/Weapons/BP_BladeParent.BP_BladeParent_C|GetPolishHitBox (Variables|Default|GetWeaponRef)) "ECC_Visibility" "ECR_Block"))))

(event Custom|RestartMinigame
  (bind _polishingwidgetref (Variables|Default|GetPolishingWidgetRef))
  (Utilities|IsValid (Variables|Default|GetWeaponRef)
    (:Is%20Valid
      (Widget|RemovefromParent (Variables|Default|GetPolishingWidgetRef))
      (if (Variables|/Game/Blueprints/Weapons/BP_BladeParent.BP_BladeParent_C|GetIsPolishingDone? (Variables|Default|GetWeaponRef))
        (Development|PrintString "weapon is done on leave")
        (Collision|SetCollisionResponsetoChannel (Variables|/Game/Blueprints/Weapons/BP_BladeParent.BP_BladeParent_C|GetPolishHitBox (Variables|Default|GetWeaponRef)) "ECC_Visibility" "ECR_Ignore")
        (else
          (Variables|Default|SetbMinigameActive false :!label _label)
          (Variables|Default|SetProgress 0.0)
          (Variables|Default|SetTimeTaken 0.0)
          (Default|ProgressChecker _polishingwidgetref)
          (Default|HeatChecker _polishingwidgetref)
          (Widget|RemovefromParent (Variables|Default|GetPolishingWidgetRef))
          (Collision|SetCollisionResponsetoChannel (Variables|/Game/Blueprints/Weapons/BP_BladeParent.BP_BladeParent_C|GetPolishHitBox (Variables|Default|GetWeaponRef)) "ECC_Visibility" "ECR_Ignore"))))
    (:Is%20Not%20Valid
      (goto _label))))

(event EventBeginPlay
  (bind _returnvalue (Actor|GetActorOfClass "/Game/Blueprints/Workstations/Polishing/Polishing_Workstation.Polishing_Workstation_C"))
  (Variables|Default|SetPolishingRef _returnvalue)
  (bind _returnvalue_2 (UserInterface|CreateWidget "/Game/Blueprints/Workstations/Polishing/WBP_PolishingWidget.WBP_PolishingWidget_C"))
  (Variables|Default|SetPolishingWidgetRef _returnvalue_2))

(event Collision|EventActorBeginOverlap
  (params (OtherActor :type Actor%20Object%20Reference)))

(event EventTick
  (params (DeltaSeconds :type Float%20%28single-precision%29))
  (bind _returnvalue (Game|GetPlayerController 0))
  (bind (_hitresult _returnvalue_2) (Game|Player|GetHitResultUnderCursorbyChannel _returnvalue "TraceTypeQuery1" true))
  (bind (_bblockinghit _binitialoverlap _time _distance _location _impactpoint _normal _impactnormal _physmat _hitactor _hitcomponent) (Collision|BreakHitResult _hitresult))
  (if (Variables|Default|GetbMinigameActive)
    (Rendering|Material|SetScalarParameterValue (Variables|/Game/Blueprints/Weapons/BP_BladeParent.BP_BladeParent_C|GetPolishMID (Variables|Default|GetWeaponRef)) "PolishAmount" (Variables|Default|GetProgress) :!class /Script/Engine.MaterialInstanceDynamic)
    (Default|HeatChecker (Variables|Default|GetPolishingWidgetRef))
    (Variables|Default|SetTimeTaken (+ (Variables|Default|GetTimeTaken) DeltaSeconds))
    (if (Variables|Default|GetbIsHolding)
      (if _returnvalue_2
        (if (== _hitcomponent (Variables|/Game/Blueprints/Weapons/BP_BladeParent.BP_BladeParent_C|GetPolishHitBox (Variables|Default|GetWeaponRef)))
          (if (> (Math|Float|Clamp(Float) (Math|Vector|VectorLength (- _impactpoint (Variables|Default|GetLastHitLocation))) 0.0 (Variables|Default|GetMaxMovePerFrame)) (Variables|Default|GetFastWipeThreshold))
            (Variables|Default|SetHeat (Math|Float|Clamp(Float) (+ (Variables|Default|GetHeat) (* (Variables|Default|GetHeatGainRate) DeltaSeconds))))
            (else
              (Variables|Default|SetHeat (Math|Float|Clamp(Float) (- (Variables|Default|GetHeat) (* (Variables|Default|GetHeatCoolRate) DeltaSeconds))))))
          (Development|PrintString "Hitting Sword")
          (bind _output_get (Variables|Default|SetProgress (Math|Float|Clamp(Float) (+ (Variables|Default|GetProgress) (* (Math|Float|Clamp(Float) (Math|Vector|VectorLength (- _impactpoint (Variables|Default|GetLastHitLocation))) 0.0 (Variables|Default|GetMaxMovePerFrame)) (Variables|Default|GetCleanRate) (Math|Float|Lerp 1.0 (Variables|Default|GetMinEfficiency) (Math|Float|Clamp(Float) (/ (- (Variables|Default|GetHeat) (Variables|Default|GetOverheatThreshold)) (- 1.0 (Variables|Default|GetOverheatThreshold))))))))))
          (Development|PrintString (Utilities|String|ToString(Float) _output_get))
          (Default|ProgressChecker (Variables|Default|GetPolishingWidgetRef))
          (Default|HeatChecker (Variables|Default|GetPolishingWidgetRef))
          (Variables|Default|SetLastHitLocation _impactpoint)
          (Variables|Default|SetbHasLastHit true)
          (if (>= (Variables|Default|GetProgress) 1.0)
            (bind _output_get_2 (Variables|Default|SetTimeRatio (Math|Float|Clamp(Float) (/ (- (Variables|Default|Getslowtime) (Variables|Default|GetTimeTaken)) (- (Variables|Default|Getslowtime) (Variables|Default|GetFastTime))))))
            (Development|PrintString (Utilities|String|ToString(Float) (* _output_get_2 1e+02)) true true "(R=0.110123,G=1.000000,B=0.380221,A=1.000000)" 1e+02)
            (Variables|/Game/Blueprints/Weapons/BP_BladeParent.BP_BladeParent_C|SetPolishingScore (Variables|Default|GetWeaponRef) (Math|Float|Truncate (* _output_get_2 1e+02)))
            (Variables|/Game/Blueprints/Weapons/BP_BladeParent.BP_BladeParent_C|SetIsPolishingDone? (Variables|Default|GetWeaponRef) true)
            (Variables|Default|SetbMinigameActive false)
            (Variables|Default|SetbIsHolding false)
            (Input|DisableInput (Game|GetPlayerController 0)))
          (else
            (Variables|Default|SetbHasLastHit false)
            (Variables|Default|SetHeat (Math|Float|Clamp(Float) (- (Variables|Default|GetHeat) (* (Variables|Default|GetHeatCoolRate) DeltaSeconds)))))))
      (else
        (Variables|Default|SetHeat (Math|Float|Clamp(Float) (- (Variables|Default|GetHeat) (* (Variables|Default|GetHeatCoolRate) DeltaSeconds))))))))

(event Input|MouseEvents|LeftMouseButton
  (params (Key :type Key%20Structure :default "None"))
  (:Pressed
    (Variables|Default|SetbIsHolding true)
    (Variables|Default|SetbHasLastHit false))
  (:Released
    (Variables|Default|SetbIsHolding false)
    (Variables|Default|SetbHasLastHit false)))

(fn ConstructionScript)