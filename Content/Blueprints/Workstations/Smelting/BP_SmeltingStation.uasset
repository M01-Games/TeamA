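; Smelting station where the player melts crucible ore into metals or alloys and pours it into moulds.
; On entry it derives target temperature from the highest melting point and tolerance from ore margins.
; Looping timers drive heat: holding input raises heating power, which otherwise decays through a gate.
; Five seconds in range triggers DT_AlloyCalc matching by metal presence, with sludge for invalid mixes, enabling an animated pour costed per mould.
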(event Custom|Check%20Crucible%20Temperature
  (bind _smeltingui (Variables|Default|GetSmeltingUi))
  (bind _target_temperature (Variables|Default|GetTarget%20Temperature))
  (bind _marginoferror_per_side_ (Variables|Default|GetMarginOfError%28per%20side%29))
  (if (Math|Float|InRange(Float) (Variables|Default|GetCrucibleTemperature) (- _target_temperature _marginoferror_per_side_) (+ _target_temperature _marginoferror_per_side_))
    (Variables|Default|SetTimeInSmelter (Math|Float|Clamp(Float) (+ (Variables|Default|GetTimeInSmelter) 0.1) 0.0 5.0))
    (if (>= (Variables|Default|GetTimeInSmelter) 5.0)
      (Utilities|FlowControl|DoOnce false :!label _label
        (:Completed
          ;[0.15 0.15 0.15 0.5] Code For Melting, Alloys
          (CallFunction|AlloyCalculations)
          (Variables|Default|SetHottestSmelted (Variables|Default|GetTarget%20Temperature))
          (Default|Reset _smeltingui)
          (for _array_element (Variables|Default|GetSmelted)
            (Default|METALSIN _smeltingui _array_element))
          (Default|Show (Variables|Default|GetSmeltingUi) true)
          (goto _label_2 Reset))))
    (else
      (Variables|Default|SetTimeInSmelter (Math|Float|Clamp(Float) (- (Variables|Default|GetTimeInSmelter) 0.1) 0.0 5.0))
      (Utilities|FlowControl|DoOnce true :!label _label_2
        (:Completed
          (Default|Show (Variables|Default|GetSmeltingUi) false)
          (goto _label Reset))))))

(event Custom|Cool%20Crucible
  (Variables|Default|SetCrucibleTemperature (Math|Float|Clamp(Float) (- (Variables|Default|GetCrucibleTemperature) 1.0) 0.0 4e+03))
  (if (== (Variables|Default|GetCrucibleTemperature) 0.0)
    (Variables|Default|SetHeatingPower 0.0)
    (CallFunction|OpenLowerPower false)))

(event Custom|PourReset
  (bind _returnvalue (Game|GetPlayerController 0))
  (bind _smeltingui (Variables|Default|GetSmeltingUi))
  (bind _as_bp_mold (Variables|Default|GetAs%20BP%20Mold))
  (bind _metalpour1 (Variables|Default|GetMETALPOUR1))
  (bind _names_0 (Variables|Default|GetNames_0))
  (bind (_key _value) (Utilities|Map|GetKeyValueByIndex _names_0 0))
  (bind _weaponstruct (Variables|/Game/Blueprints/BP_Mould.BP_Mould_C|GetWeaponStruct _as_bp_mold))
  (Utilities|FlowControl|DoOnce false) ; enters at Reset
)

(event Custom|Heat%20Crucible
  (Variables|Default|SetCrucibleTemperature (Math|Float|Clamp(Float) (+ (Variables|Default|GetCrucibleTemperature) (Variables|Default|GetHeatingPower)) 0.0 4e+03))
  (if (== (Variables|Default|GetCrucibleTemperature) 0.0)
    (Variables|Default|SetHeatingPower 0.0)
    (CallFunction|OpenLowerPower false)))

(event Custom|FlickerLight
  (bind _newtrack_0 (Timeline|Timeline PlayFromStart)
    (:Update
      (CallFunction|LightFlicker _newtrack_0))
    (:Finished
      (CallFunction|FlickerLight))))

(event Custom|LowerPower
  (Utilities|FlowControl|Gate true
    (:Exit
      (Variables|Default|SetHeatingPower (Math|Float|Clamp(Float) (- (Variables|Default|GetHeatingPower) (/ (Math|Conversions|ToFloat(Integer) 1) (Math|Conversions|ToFloat(Integer) (Variables|Default|GetUpgradeLevel)))) -15.0 1e+01)))))

(event Custom|OpenLowerPower
  (params (Return :type Boolean))
  (if Return
    (Utilities|FlowControl|Gate true) ; enters at Open
    (else
      (Utilities|FlowControl|Gate true) ; enters at Close
    )))

(event Custom|CrucibleStuff
  (CallFunction|HeatCrucible))

(event Input|EnhancedActionEvents|EnhancedInputActionIA_Space
  (params (ActionValue :type Boolean) (ElapsedSeconds :type Float%20%28double-precision%29) (TriggeredSeconds :type Float%20%28double-precision%29) (InputAction :type Input%20Action%20Object%20Reference :default "/Game/Input/Actions/IA_Space.IA_Space"))
  ;[0.15 0.15 0.15 0.5] For now changed it to held. Can be changed
  (:Started
    (CallFunction|OpenLowerPower false :!label _label)
    (Variables|Default|SetHeatingPower (Math|Float|Clamp(Float) (+ (Variables|Default|GetHeatingPower) 0.05) -15.0 1e+01)))
  (:Ongoing
    (goto _label))
  (:Canceled
    (CallFunction|OpenLowerPower true :!label _label_2))
  (:Completed
    (goto _label_2)))

(event Input|EnhancedActionEvents|EnhancedInputActionIA_Down
  (params (ActionValue :type Float%20%28double-precision%29) (ElapsedSeconds :type Float%20%28double-precision%29) (TriggeredSeconds :type Float%20%28double-precision%29) (InputAction :type Input%20Action%20Object%20Reference :default "/Game/Input/Actions/IA_Down.IA_Down"))
  (bind _returnvalue (Game|GetPlayerController 0))
  (bind _smeltingui (Variables|Default|GetSmeltingUi))
  (bind _metalpour1 (Variables|Default|GetMETALPOUR1))
  (bind _names_0 (Variables|Default|GetNames_0))
  (bind _as_item_slot (Variables|Default|GetAs%20Item%20Slot))
  (bind (_key _value) (Utilities|Map|GetKeyValueByIndex _names_0 0))
  (if (and (<= ActionValue -0.1) (> ElapsedSeconds 0.1))
    (if (and (Variables|/Script/TeamA.ItemSlot|GetbIsOccupied _as_item_slot) (== (Variables|Default|GetTimeInSmelter) 5.0))
      (bind _asbp_mould (Utilities|Casting|CastToBP_Mould (Variables|/Script/TeamA.ItemSlot|GetAttachedItem _as_item_slot)))
      (bind _output_get (Variables|Default|SetAs%20BP%20Mold _asbp_mould))
      (if (and (not (Variables|/Game/Blueprints/BP_Mould.BP_Mould_C|GetFull _output_get)) (>= (Variables|Default|GetHowMuchOre) (.ingotcost (Variables|/Game/Blueprints/BP_Mould.BP_Mould_C|GetWeaponStruct (Variables|Default|GetAs%20BP%20Mold)))))
        (Utilities|FlowControl|DoOnce false
          (:Completed
            (bind _output_get_2 (Variables|Default|SetHowMuchOre (- (Variables|Default|GetHowMuchOre) (.ingotcost (Variables|/Game/Blueprints/BP_Mould.BP_Mould_C|GetWeaponStruct (Variables|Default|GetAs%20BP%20Mold))))))
            (Development|PrintString (Utilities|String|ToString(Float) _output_get_2))
            (Variables|/Game/Blueprints/BP_Mould.BP_Mould_C|SetMetal (Variables|Default|GetAs%20BP%20Mold) (Utilities|Array|Get(acopy) (Variables|Default|GetSmelted)))
            (for _index (range 1 (Math|Float|Truncate (.ingotcost (Variables|/Game/Blueprints/BP_Mould.BP_Mould_C|GetWeaponStruct (Variables|Default|GetAs%20BP%20Mold)))))
              (Utilities|Array|RemoveIndex (Variables|Default|GetSmelted))
              (Utilities|Map|Add _names_0 _key (- _value 1)))
            (Variables|/Game/Blueprints/BP_Mould.BP_Mould_C|SetFull (Variables|Default|GetAs%20BP%20Mold) true)
            (Default|Reset _smeltingui)
            (for _array_element (Variables|Default|GetSmelted)
              (Default|METALSIN _smeltingui _array_element))
            (for _array_element_2 (Variables|Default|GetOre)
              (Default|METALSIN _smeltingui (.metalname (Variables|/Game/Blueprints/BP_Ore1.BP_Ore1_C|GetMetal%20Info _array_element_2))))
            (Input|DisableInput (Variables|Default|GetCharacter) (Game|GetPlayerController 0))
            (Rendering|SetVisibility (Variables|Default|GetMETALPOUR1) true false)
            (Components|Animation|PlayAnimation (Variables|Default|GetCrucible1) "/Game/Assets/Buildings/BucketTurnDown.BucketTurnDown" false)
            (Components|Animation|PlayAnimation _metalpour1 "/Game/Assets/Workstations/Turn.Turn" false)
            (Utilities|FlowControl|Delay 1.2)
            (Components|Animation|PlayAnimation _metalpour1 "/Game/Assets/Workstations/Pour.Pour" false)
            (Utilities|FlowControl|Delay 3.0)
            (Input|EnableInput (Variables|Default|GetCharacter) _returnvalue)
            (Input|SetInputModeGameOnly _returnvalue true)
            (Rendering|SetVisibility (Variables|Default|GetMETALPOUR1) false false)
            (Components|Animation|PlayAnimation (Variables|Default|GetCrucible1) "/Game/Assets/Buildings/BucketTurnUp.BucketTurnUp" false)
            (CallFunction|PourReset))))
      (else
        (Development|PrintString "Metal not hot enough OR no mould")))))

(event Input|EnhancedActionEvents|EnhancedInputActionIA_Eject
  (params (ActionValue :type Boolean) (ElapsedSeconds :type Float%20%28double-precision%29) (TriggeredSeconds :type Float%20%28double-precision%29) (InputAction :type Input%20Action%20Object%20Reference :default "/Game/Input/Actions/IA_Eject.IA_Eject"))
  (:Started
    (Utilities|Array|Clear (Variables|Default|GetSmelted))
    (Class|ItemSlot|DetachItem (Variables|Default|GetAs%20Box%20Slot))
    (Utilities|Array|Clear (Variables|Default|GetOre))
    (Default|Reset (Variables|Default|GetSmeltingUi))))

(event EventBeginPlay
  (bind _returnvalue (Rendering|Material|CreateDynamicMaterialInstance "/Game/Assets/Lucas/Textures/Forge_Textures/M_Forge.M_Forge" "None" "None" :!class /Script/Engine.KismetMaterialLibrary))
  (bind _output_get (Variables|Default|SetForgeMat _returnvalue))
  (Rendering|Material|SetMaterial (Variables|Default|GetStaticMesh) 0 _output_get)
  (CallFunction|FlickerLight)
  (bind _asbox_slot (Utilities|Casting|CastToBoxSlot (Variables|/Script/Engine.ChildActorComponent|GetChildActor (Variables|Default|GetCrucibleContainer))))
  (Variables|Default|SetAs%20Box%20Slot _asbox_slot)
  (bind _asitem_slot (Utilities|Casting|CastToItemSlot (Variables|/Script/Engine.ChildActorComponent|GetChildActor (Variables|Default|GetMouldSpot))))
  (Variables|Default|SetAs%20Item%20Slot _asitem_slot)
  (Utilities|Time|SetTimerbyEvent (delegate Custom|LowerPower) 0.1 true true)
  (Utilities|Time|SetTimerbyEvent (delegate Custom|CrucibleStuff) 0.01 true true)
  (Utilities|Time|SetTimerbyEvent (delegate Custom|Check%20Crucible%20Temperature) 0.1 true true))

(event EventEnter
  (params (Character :type Character%20Object%20Reference))
  (bind _as_box_slot (Variables|Default|GetAs%20Box%20Slot))
  (bind _containeditems (Variables|/Script/TeamA.BoxSlot|GetContainedItems _as_box_slot))
  ;[0.15 0.15 0.15 0.5] Detecting Inventory On Entry (Will need to move Temp Func)
  (Variables|Default|SetCharacter Character)
  (Input|EnableInput (Game|GetPlayerController 0))
  (if (Utilities|Array|IsEmpty (Variables|Default|GetSmelted))
    (Variables|Default|SetTarget%20Temperature -999.0))
  (Development|PrintString (Utilities|String|ToString(Integer) (Utilities|Array|Length _containeditems)))
  (for _array_element _containeditems
    (bind _asbp_ore_1 (Utilities|Casting|CastToBP_Ore1 _array_element))
    (if (< (Utilities|Array|FindItem (Variables|Default|GetOre) _asbp_ore_1) 0)
      (Utilities|Array|Add (Variables|Default|GetOre) _asbp_ore_1)
      (Math|Float|IncrementFloat (Variables|Default|GetHowMuchOre)
        (:%20%20
          (Development|PrintString "Added")))
      (else
        (Development|PrintString "AlreadyIn"))))
  (for _array_element_2 (Variables|Default|GetOre)
    (if (< (Utilities|Array|FindItem (Variables|/Script/TeamA.BoxSlot|GetContainedItems (Variables|Default|GetAs%20Box%20Slot)) _array_element_2) 0)
      (Development|PrintString "Removed")
      (Utilities|Array|RemoveItem (Variables|Default|GetOre) _array_element_2)
      (Math|Float|DecrementFloat (Variables|Default|GetHowMuchOre))
      (else
        (CallFunction|HighestTemp (.meltingpoint (Variables|/Game/Blueprints/BP_Ore1.BP_Ore1_C|GetMetal%20Info _array_element_2))))))
  (Development|PrintString (Utilities|String|Append "Total: " (Utilities|String|ToString(Float) (Variables|Default|GetHowMuchOre))))
  (CallFunction|SetMarginOfError)
  (CallFunction|HighestTemp (Variables|Default|GetHottestSmelted))
  (bind _returnvalue (UserInterface|CreateWidget "/Game/Blueprints/Workstations/Smelting/SmeltingUI.SmeltingUI_C" 0 self))
  (bind _output_get (Variables|Default|SetSmeltingUi _returnvalue))
  (Variables|/Game/Blueprints/Workstations/Smelting/TempGague.TempGague_C|SetSmeltingStation (Variables|/Game/Blueprints/Workstations/Smelting/SmeltingUI.SmeltingUI_C|GetTempGague _output_get) self)
  (for _array_element_3 (Variables|Default|GetSmelted)
    (Default|METALSIN (Variables|Default|GetSmeltingUi) _array_element_3))
  (for _array_element_4 (Variables|Default|GetOre)
    (Default|METALSIN (Variables|Default|GetSmeltingUi) (.metalname (Variables|/Game/Blueprints/BP_Ore1.BP_Ore1_C|GetMetal%20Info _array_element_4)))
    (Development|PrintString (Utilities|String|EnumtoString (.metalname (Variables|/Game/Blueprints/BP_Ore1.BP_Ore1_C|GetMetal%20Info _array_element_4)))))
  (UserInterface|Viewport|AddtoViewport (Variables|Default|GetSmeltingUi) 0))

(event EventExit
  (params (Character :type Character%20Object%20Reference))
  (bind _smeltingui (Variables|Default|GetSmeltingUi))
  (Variables|Default|SetCharacter 0)
  (Input|DisableInput (Game|GetPlayerController 0))
  (Utilities|IsValid _smeltingui
    (:Is%20Valid
      (Widget|RemovefromParent _smeltingui)
      (Variables|/Script/Engine.PlayerController|SetbShowMouseCursor (Game|GetPlayerController 0) false)
      (CallFunction|OpenLowerPower true))))

(event Input|MouseEvents|MouseWheelDown
  (params (Key :type Key%20Structure :default "None"))
  (bind _returnvalue (Game|GetPlayerController 0))
  (bind _smeltingui (Variables|Default|GetSmeltingUi))
  (bind _metalpour1 (Variables|Default|GetMETALPOUR1))
  (bind _names_0 (Variables|Default|GetNames_0))
  (bind _as_item_slot (Variables|Default|GetAs%20Item%20Slot))
  (bind (_key _value) (Utilities|Map|GetKeyValueByIndex _names_0 0))
  (:Pressed
    (if (and (Variables|/Script/TeamA.ItemSlot|GetbIsOccupied _as_item_slot) (== (Variables|Default|GetTimeInSmelter) 5.0))
      (bind _asbp_mould (Utilities|Casting|CastToBP_Mould (Variables|/Script/TeamA.ItemSlot|GetAttachedItem _as_item_slot)))
      (bind _output_get (Variables|Default|SetAs%20BP%20Mold _asbp_mould))
      (if (and (not (Variables|/Game/Blueprints/BP_Mould.BP_Mould_C|GetFull _output_get)) (>= (Variables|Default|GetHowMuchOre) (.ingotcost (Variables|/Game/Blueprints/BP_Mould.BP_Mould_C|GetWeaponStruct (Variables|Default|GetAs%20BP%20Mold)))))
        (Utilities|FlowControl|DoOnce false
          (:Completed
            (bind _output_get_2 (Variables|Default|SetHowMuchOre (- (Variables|Default|GetHowMuchOre) (.ingotcost (Variables|/Game/Blueprints/BP_Mould.BP_Mould_C|GetWeaponStruct (Variables|Default|GetAs%20BP%20Mold))))))
            (Development|PrintString (Utilities|String|ToString(Float) _output_get_2))
            (Variables|/Game/Blueprints/BP_Mould.BP_Mould_C|SetMetal (Variables|Default|GetAs%20BP%20Mold) (Utilities|Array|Get(acopy) (Variables|Default|GetSmelted)))
            (for _index (range 1 (Math|Float|Truncate (.ingotcost (Variables|/Game/Blueprints/BP_Mould.BP_Mould_C|GetWeaponStruct (Variables|Default|GetAs%20BP%20Mold)))))
              (Utilities|Array|RemoveIndex (Variables|Default|GetSmelted))
              (Utilities|Map|Add _names_0 _key (- _value 1)))
            (Variables|/Game/Blueprints/BP_Mould.BP_Mould_C|SetFull (Variables|Default|GetAs%20BP%20Mold) true)
            (Default|Reset _smeltingui)
            (for _array_element (Variables|Default|GetSmelted)
              (Default|METALSIN _smeltingui _array_element))
            (for _array_element_2 (Variables|Default|GetOre)
              (Default|METALSIN _smeltingui (.metalname (Variables|/Game/Blueprints/BP_Ore1.BP_Ore1_C|GetMetal%20Info _array_element_2))))
            (Input|DisableInput (Variables|Default|GetCharacter) (Game|GetPlayerController 0))
            (Rendering|SetVisibility (Variables|Default|GetMETALPOUR1) true false)
            (Components|Animation|PlayAnimation (Variables|Default|GetCrucible1) "/Game/Assets/Buildings/BucketTurnDown.BucketTurnDown" false)
            (Components|Animation|PlayAnimation _metalpour1 "/Game/Assets/Workstations/Turn.Turn" false)
            (Utilities|FlowControl|Delay 1.2)
            (Components|Animation|PlayAnimation _metalpour1 "/Game/Assets/Workstations/Pour.Pour" false)
            (Utilities|FlowControl|Delay 3.0)
            (Input|EnableInput (Variables|Default|GetCharacter) _returnvalue)
            (Input|SetInputModeGameOnly _returnvalue true)
            (Rendering|SetVisibility (Variables|Default|GetMETALPOUR1) false false)
            (Components|Animation|PlayAnimation (Variables|Default|GetCrucible1) "/Game/Assets/Buildings/BucketTurnUp.BucketTurnUp" false)
            (CallFunction|PourReset))))
      (else
        (Development|PrintString "Metal not hot enough OR no mould")))))

(fn ConstructionScript)

(fn HighestTemp
  (params (MeltingPoint :type Float%20%28double-precision%29))
  (if (> MeltingPoint (Variables|Default|GetTarget%20Temperature))
    (Variables|Default|SetTarget%20Temperature MeltingPoint)))

(fn SetMarginOfError
  (bind _ore (Variables|Default|GetOre))
  (if (Utilities|Array|IsEmpty (Variables|Default|GetSmelted))
    (Variables|Default|SetMarginOfError%28per%20side%29 0.0))
  (if (not (Utilities|Array|IsEmpty _ore))
    (for _array_element _ore
      (Utilities|IsValid _array_element
        (:Is%20Valid
          (Variables|Default|SetMarginOfError%28per%20side%29 (+ (Variables|Default|GetMarginOfError%28per%20side%29) (.marginoferrorperside (Variables|/Game/Blueprints/BP_Ore1.BP_Ore1_C|GetMetal%20Info _array_element)))))))
    (Variables|Default|SetMarginOfError%28per%20side%29 (/ (Variables|Default|GetMarginOfError%28per%20side%29) (Utilities|Array|Length _ore)))))

(fn AlloyCalculations
  (bind _as_box_slot (Variables|Default|GetAs%20Box%20Slot))
  (bind _smelted (Variables|Default|GetSmelted))
  (bind _ore (Variables|Default|GetOre))
  (bind _names_0 (Variables|Default|GetNames_0))
  (bind _names_0_2 (Variables|Default|GetNames_0))
  (bind _smelted_2 (Variables|Default|GetSmelted))
  (bind _names_0_3 (Variables|Default|GetNames_0))
  (bind _returnvalue (Utilities|Array|Length _smelted_2))
  ;[0.15 0.15 0.15 0.5] For Now turn all to sludge
  (Utilities|IsValid (Utilities|Array|Get(acopy) _ore)
    (:Is%20Valid
      (Development|PrintString "Unknown combo. making Sludge")
      (for _array_element _ore
        (bind _keys (Utilities|Map|Keys (Variables|Default|GetNames_0)))
        (if (!= (Utilities|Array|FindItem _keys (.metalname (Variables|/Game/Blueprints/BP_Ore1.BP_Ore1_C|GetMetal%20Info _array_element))) -1)
          (bind _values (Utilities|Map|Values _names_0))
          (Utilities|Map|Add (Variables|Default|GetNames_0) (.metalname (Variables|/Game/Blueprints/BP_Ore1.BP_Ore1_C|GetMetal%20Info _array_element)) (+ (Utilities|Array|Get(acopy) _values (Utilities|Array|FindItem _keys (.metalname (Variables|/Game/Blueprints/BP_Ore1.BP_Ore1_C|GetMetal%20Info _array_element)))) 1))
          (else
            (Utilities|Map|Add _names_0 (.metalname (Variables|/Game/Blueprints/BP_Ore1.BP_Ore1_C|GetMetal%20Info _array_element)) 1))))
      (bind _outrownames (DataTable|GetDataTableRowNames "/Game/Data/SmeltingData/DT_AlloyCalc.DT_AlloyCalc"))
      (for _array_element_2 _outrownames
        (bind _returnvalue_2 (Utilities|GetDataTableRow "/Game/Data/SmeltingData/DT_AlloyCalc.DT_AlloyCalc" _array_element_2)
          (:then
            (bind _keys_2 (Utilities|Map|Keys (.alloyratio _returnvalue_2)))
            (LocalVariables|SetPossible false)
            (bind _array_element_3 (Utilities|Array|ForEachLoopwithBreak _keys_2 :!label _label)
              (:LoopBody
                (if (Utilities|Map|Contains (Variables|Default|GetNames_0) _array_element_3)
                  (LocalVariables|SetPossible true)
                  (else
                    (LocalVariables|SetPossible false)
                    (goto _label Break))))
              (:Completed
                (if (LocalVariables|GetPossible)
                  (Utilities|Array|Add (LocalVariables|GetPossibleAlloys) (.alloy _returnvalue_2))))))))
      (bind _keys_3 (Utilities|Map|Keys _names_0_2))
      (LocalVariables|SetOresIn _keys_3)
      (bind _values_2 (Utilities|Map|Values _names_0_2))
      (LocalVariables|SetNumberOfMetaliN _values_2)
      (Utilities|Array|Clear (Variables|Default|GetSmelted))
      (if (or (> (Utilities|Array|Length (LocalVariables|GetPossibleAlloys)) 1) (> (Utilities|Map|Length (Variables|Default|GetNames_0)) 2))
        (for _array_element_4 (LocalVariables|GetNumberOfMetaliN) :!label _label_2
          (for _index (range 1 _array_element_4)
            (Utilities|Array|Add (Variables|Default|GetSmelted) "NewEnumerator9")))
        (elif (and (< (Utilities|Array|Length (LocalVariables|GetPossibleAlloys)) 1) (> (Utilities|Map|Length (Variables|Default|GetNames_0)) 1))
          (goto _label_2)
          (elif (< (Utilities|Array|Length (LocalVariables|GetPossibleAlloys)) 1)
            (for _array_element_5 (LocalVariables|GetNumberOfMetaliN)
              (for _index_2 (range 1 _array_element_5)
                (Utilities|Array|Add (Variables|Default|GetSmelted) (Utilities|Array|Get(acopy) (LocalVariables|GetOresIn)))))
            (else
              (for _array_element_6 (LocalVariables|GetNumberOfMetaliN)
                (for _index_3 (range 1 _array_element_6)
                  (Utilities|Array|Add (Variables|Default|GetSmelted) (Utilities|Array|Get(acopy) (LocalVariables|GetPossibleAlloys)))))))))
      (Class|BoxSlot|DeleteAll _as_box_slot)
      (Variables|Default|SetHowMuchOre (Math|Conversions|ToFloat(Integer) _returnvalue))
      (Variables|/Script/TeamA.BoxSlot|SetItemMax _as_box_slot (- 5 _returnvalue))
      (Utilities|Array|Clear (Variables|Default|GetOre))
      (Utilities|Map|Clear _names_0_3)
      (Utilities|Map|Add _names_0_3 (Utilities|Array|Get(acopy) _smelted) (Utilities|Array|Length _smelted)))
    (:Is%20Not%20Valid
      (Development|PrintString "NoOre"))))

(fn LightFlicker
  (params (NewParam :type Float%20%28double-precision%29))
  (Rendering|Material|SetScalarParameterValue (Variables|Default|GetForgeMat) "Noise" (* NewParam 1e+01) :!class /Script/Engine.MaterialInstanceDynamic)
  (Rendering|Components|Light|SetIntensity (Variables|Default|GetPointLight) (Math|Float|Lerp 5e+02 1e+03 NewParam)))