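; BP_Mould is a mould actor for a weapon type, set through its MouldType enum.
; The construction script maps Sword, Dagger or Battle Axe to the matching blade or axe class in MyActor.
; On BeginPlay it uses the enum name as the DT_Weapons row key, stores the row in WeaponStruct and shows the type name on a TextRender.
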(event EventBeginPlay
  (bind _mouldtype (Variables|Default|GetMouldType))
  (bind _returnvalue (Utilities|String|EnumtoString _mouldtype))
  (bind _returnvalue_2 (Utilities|GetDataTableRow "/Game/Data/QuestData/DT_Weapons.DT_Weapons" (Utilities|String|StringToName _returnvalue))
    (:then
      (Variables|Default|SetWeaponStruct _returnvalue_2)
      (Rendering|Components|TextRender|SetText (Variables|Default|GetTextRender) (Utilities|Text|ToText(String) _returnvalue)))))

(fn ConstructionScript
  (switch Utilities|FlowControl|Switch|SwitchonWeaponTypes (Variables|Default|GetMouldType)
    (:NewEnumerator0
      (Variables|Default|SetMy%20Actor "/Game/Blueprints/Weapons/BP_BladeSword1.BP_BladeSword1_C"))
    (:NewEnumerator2
      (Variables|Default|SetMy%20Actor "/Game/Blueprints/Weapons/BP_BladeDagger1.BP_BladeDagger1_C"))
    (:NewEnumerator1
      (Variables|Default|SetMy%20Actor "/Game/Blueprints/Weapons/BP_Axe.BP_Axe_C"))))