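; BP_Ore1 is a metal ore piece or ingot whose look and type follow an editor-selectable MetalType enum.
; The construction script swaps in a cube mesh for ingots, creates a dynamic material and sets SpecificType.
; It applies DT_Metal colours and surface values alongside variables not read from the table, such as Metallic and Roughness.
; BeginPlay separately caches a row from another table, DT_Metals, into MetalInfo.
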(event EventBeginPlay
  (bind _returnvalue (Utilities|GetDataTableRow "/Game/Data/QuestData/DT_Metals.DT_Metals" (Utilities|String|StringToName (Utilities|String|EnumtoString (Variables|Default|GetMetal%20Type))))
    (:then
      (bind _output_get (Variables|Default|SetMetal%20Info _returnvalue)))))

(fn ConstructionScript
  (if (Variables|Default|GetIsIngot)
    (Variables|Default|SetElement%20Index 0)
    (Components|StaticMesh|SetStaticMesh (Variables|Default|GetOre) "/Game/LevelPrototyping/Meshes/SM_ChamferCube.SM_ChamferCube")
    (else
      (Variables|Default|SetElement%20Index 1)))
  (bind _returnvalue (Rendering|Material|CreateDynamicMaterialInstance "/Game/Assets/Materials/Metal/MI_Metal_Default.MI_Metal_Default" "None" "None" :!class /Script/Engine.KismetMaterialLibrary))
  (bind _output_get (Variables|Default|SetMetal%20DMI _returnvalue))
  (Rendering|Material|SetMaterial (Variables|Default|GetOre) (Variables|Default|GetElement%20Index) _output_get)
  (CallFunction|SetMetalInfofromDataTable)
  (CallFunction|ApplyMetalInfofromDataTable)
  (switch Utilities|FlowControl|Switch|SwitchonE_MetalType (Variables|Default|GetMetal%20Type)
    (:NewEnumerator0
      (Variables|Default|SetSpecificType "Gold"))
    (:NewEnumerator1
      (Variables|Default|SetSpecificType "Iron"))
    (:NewEnumerator2
      (Variables|Default|SetSpecificType "Copper"))
    (:NewEnumerator3
      (Variables|Default|SetSpecificType "Tungsten"))
    (:NewEnumerator5
      (Variables|Default|SetSpecificType "Zinc"))
    (:NewEnumerator8
      (Variables|Default|SetSpecificType "Silver"))))

(fn SetMetalInfofromDataTable
  (bind _returnvalue (Utilities|GetDataTableRow "/Game/Assets/Materials/Metal/DT_Metal.DT_Metal" (Utilities|String|StringToName (Utilities|String|EnumtoString (Variables|Default|GetMetal%20Type))))
    (:then
      (bind _output_get (Variables|Default|SetMetal%20Data _returnvalue))
      (Variables|Default|SetScratch%20Tiling (.scratchtiling _output_get))
      (Variables|Default|SetScratch%20Colour%20Intensity (.scratchcolourintensity _output_get))
      (Variables|Default|SetGlow%20Boost (.glowboost _output_get))
      (Variables|Default|SetRim%20Light%20Intensity (.rimlightintensity _output_get))
      (Variables|Default|SetMetal%20Colour (.metalcolour _output_get))
      (Variables|Default|SetScratch%20Colour (.imperfectioncolour _output_get))
      (Variables|Default|SetRim%20Light%20Colour (.rimlightcolour _output_get)))
    (:RowNotFound
      (Development|PrintString "ROW NOT FOUND" true true "(R=1.000000,G=0.057958,B=0.000000,A=1.000000)" 1e+01))))

(fn ApplyMetalInfofromDataTable
  (bind _metal_dmi (Variables|Default|GetMetal%20DMI))
  (Rendering|Material|SetScalarParameterValue _metal_dmi "Metallic" (Variables|Default|GetMetallic) :!class /Script/Engine.MaterialInstanceDynamic)
  (Rendering|Material|SetScalarParameterValue _metal_dmi "Roughness" (Variables|Default|GetRoughness) :!class /Script/Engine.MaterialInstanceDynamic)
  (Rendering|Material|SetScalarParameterValue _metal_dmi "Scratch Strength" (Variables|Default|GetScratch%20Strength) :!class /Script/Engine.MaterialInstanceDynamic)
  (Rendering|Material|SetScalarParameterValue _metal_dmi "Scratch Tiling" (Variables|Default|GetScratch%20Tiling) :!class /Script/Engine.MaterialInstanceDynamic)
  (Rendering|Material|SetScalarParameterValue _metal_dmi "Scratch Colour Intensity" (Variables|Default|GetScratch%20Colour%20Intensity) :!class /Script/Engine.MaterialInstanceDynamic)
  (Rendering|Material|SetScalarParameterValue _metal_dmi "Heat Intensity" (Variables|Default|GetHeat%20Intensity) :!class /Script/Engine.MaterialInstanceDynamic)
  (Rendering|Material|SetScalarParameterValue _metal_dmi "Glow Boost" (Variables|Default|GetGlow%20Boost) :!class /Script/Engine.MaterialInstanceDynamic)
  (Rendering|Material|SetScalarParameterValue _metal_dmi "Rim Light Intensity" (Variables|Default|GetRim%20Light%20Intensity) :!class /Script/Engine.MaterialInstanceDynamic)
  (Rendering|Material|SetScalarParameterValue _metal_dmi "Grain Strength" (Variables|Default|GetGrain%20Strength) :!class /Script/Engine.MaterialInstanceDynamic)
  (Rendering|Material|SetVectorParameterValue _metal_dmi "Metal Colour" (Variables|Default|GetMetal%20Colour) :!class /Script/Engine.MaterialInstanceDynamic)
  (Rendering|Material|SetVectorParameterValue _metal_dmi "Scratch Colour" (Variables|Default|GetScratch%20Colour) :!class /Script/Engine.MaterialInstanceDynamic)
  (Rendering|Material|SetVectorParameterValue _metal_dmi "Rim Light Colour" (Variables|Default|GetRim%20Light%20Colour) :!class /Script/Engine.MaterialInstanceDynamic))