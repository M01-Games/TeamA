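; Shared helper functions for player interaction and sword-order checks on metal and rarity.
; LineTraceFromCamera, when not grabbing, traces the Visibility channel along the camera's forward vector and sends SelectTaskMessage and OpenMessage to the hit actor.
; RequiredToEmetal converts a required-metal enum to the Emetal enum.
; CalculateRareAccept passes swords meeting or exceeding the required rarity, but always rejects Poor ones.
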(fn LineTracefromCamera
  (params (Grabbing :type Boolean) (Camera :type Camera%20Component%20Object%20Reference) (reachDistance :type Float%20%28double-precision%29) (PhysicsHandle :type Physics%20Handle%20Component%20Object%20Reference) (TimerHandle :type Timer%20Handle%20Structure))
  (bind _returnvalue (Transformation|GetWorldLocation Camera))
  ;[0.15 0.15 0.15 0.5] Subject to change. going to try change this is i can do it outside of the FPS  Player
  ;;[0.15 0.15 0.15 0.5] Line Tracing for intteraction
  (if (not Grabbing)
    (bind _outhit (Collision|LineTraceByChannel 0 _returnvalue (+ _returnvalue (* (Math|Vector|GetForwardVector Camera) reachDistance)) "TraceTypeQuery1" false 0 "None"))
    (if (or (.bblockinghit _outhit) (.binitialoverlap _outhit))
      ;;[0.15 0.15 0.15 0.5 14] If task has This BPI
      ;; it is a task and is selected
      (Class|BPITask|SelectTask(Message) (.hitactor _outhit))
      (Class|BPIDelivery|Open(Message) (.hitactor _outhit)))))

(fn RequiredtoEmetal
  (params (RM :type RequiredMetal%20Enum :default "NewEnumerator0"))
  (switch Utilities|FlowControl|Switch|SwitchonRequiredMetal RM
    (:NewEnumerator0
      (LocalVariables|SetEmetal "NewEnumerator0"))
    (:NewEnumerator1
      (LocalVariables|SetEmetal "NewEnumerator1"))
    (:NewEnumerator2
      (LocalVariables|SetEmetal "NewEnumerator2"))
    (:NewEnumerator3
      (LocalVariables|SetEmetal "NewEnumerator5"))
    (:NewEnumerator4
      (LocalVariables|SetEmetal "NewEnumerator6"))
    (:NewEnumerator5
      (LocalVariables|SetEmetal "NewEnumerator7"))
    (:NewEnumerator6
      (LocalVariables|SetEmetal "NewEnumerator4"))
    (:NewEnumerator7
      (LocalVariables|SetEmetal "NewEnumerator3"))
    (:NewEnumerator8
      (LocalVariables|SetEmetal "NewEnumerator8")))
  (return (LocalVariables|GetEmetal)))

(fn CalculateRareAccept
  (params (Required%20Rarity :type RequiredRarety%20Enum :default "NewEnumerator7") (SwordRarety :type RequiredRarety%20Enum :default "NewEnumerator7"))
  (bind _returnvalue (Utilities|Enum|Equal(Enum) SwordRarety "NewEnumerator7"))
  (if (Utilities|Enum|NotEqual(Enum) SwordRarety "NewEnumerator11")
    (switch Utilities|FlowControl|Switch|SwitchonRequiredRarety Required%20Rarity
      (:NewEnumerator7
        (LocalVariables|SetPassing true))
      (:NewEnumerator8
        (if _returnvalue
          (LocalVariables|SetPassing false)
          (else
            (LocalVariables|SetPassing true))))
      (:NewEnumerator9
        (if (or _returnvalue (Utilities|Enum|Equal(Enum) SwordRarety "NewEnumerator8"))
          (LocalVariables|SetPassing false)
          (else
            (LocalVariables|SetPassing true))))
      (:NewEnumerator10
        (if (Utilities|Enum|Equal(Enum) SwordRarety "NewEnumerator10")
          (LocalVariables|SetPassing true)
          (else
            (LocalVariables|SetPassing false))))
      (:NewEnumerator11
        (LocalVariables|SetPassing true)))
    (else
      (LocalVariables|SetPassing false)))
  (return (LocalVariables|GetPassing)))