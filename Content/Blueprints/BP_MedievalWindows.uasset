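; BP_MedievalWindows is a window actor that switches its Cube material between lit and dark as day turns to night.
; On BeginPlay it creates a dynamic instance of the Light material, binds ToggleLight to BP_TimeManager's day/night event and applies the current state.
; Each toggle waits a random delay of up to three seconds, so window instances can change out of sync.
; A RandomSeed is rolled but unused in these graphs.
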(event Custom|ToggleLight
  (params (CurrentIsNight :type Boolean))
  (bind _cube (Variables|Default|GetCube))
  (Utilities|FlowControl|Delay (Math|Random|RandomFloatinRange 0.0 3.0))
  (if CurrentIsNight
    (Rendering|Material|SetMaterial _cube 0 (Variables|Default|GetLight))
    (else
      (Rendering|Material|SetMaterial _cube 0 "/Game/Assets/Environment/Dark.Dark"))))

(event EventBeginPlay
  (bind _returnvalue (Rendering|Material|CreateDynamicMaterialInstance "/Game/Assets/Environment/Light.Light" "None" "None" :!class /Script/Engine.KismetMaterialLibrary))
  (Variables|Default|SetLight _returnvalue)
  (Variables|Default|SetRandomSeed (Math|Random|RandomFloatinRange 0.0 1e+03))
  (bind _returnvalue_2 (Actor|GetActorOfClass "/Game/LightingSYS/Lighting/Blueprints/BP_TimeManager.BP_TimeManager_C"))
  (Variables|Default|SetTimeRef _returnvalue_2)
  (EventDispatchers|BindEventtoOnDayNightStateChanged (Variables|Default|GetTimeRef) (delegate Custom|ToggleLight))
  (CallFunction|ToggleLight (Variables|/Game/LightingSYS/Lighting/Blueprints/BP_TimeManager.BP_TimeManager_C|GetCurrentIsNight (Variables|Default|GetTimeRef))))

(event Collision|EventActorBeginOverlap
  (params (OtherActor :type Actor%20Object%20Reference)))

(fn ConstructionScript)