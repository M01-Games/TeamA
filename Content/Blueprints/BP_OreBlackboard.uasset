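; BP_OreBlackboard is a board that displays how many iron, copper, gold and tungsten items the level's ore containers hold.
; Shortly after BeginPlay it caches all OreContainer actors and sets each ore's text from the matching container's item count, so same-type containers overwrite rather than sum.
; Tick reruns that loop through a half-second Delay, a polling approach marked for replacement.
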(event EventBeginPlay
  (Utilities|FlowControl|Delay 0.2)
  (bind _outactors (Actor|GetAllActorsOfClass "/Game/Blueprints/OreContainer.OreContainer_C"))
  (bind _output_get (Variables|Default|SetContainers _outactors))
  (for _array_element _output_get
    (switch Utilities|FlowControl|Switch|SwitchonESpecificTypes (Variables|/Game/Blueprints/OreContainer.OreContainer_C|GetAccepted%20Specific%20Type _array_element)
      (:Iron
        (Rendering|Components|TextRender|SetText (Variables|Default|GetIron1) (Utilities|Text|ToText(Integer) (Utilities|Array|Length (Variables|/Script/TeamA.BoxSlot|GetContainedItems (Variables|/Game/Blueprints/OreContainer.OreContainer_C|GetAs%20Box%20Slot _array_element))))))
      (:Copper
        (Rendering|Components|TextRender|SetText (Variables|Default|GetCopper1) (Utilities|Text|ToText(Integer) (Utilities|Array|Length (Variables|/Script/TeamA.BoxSlot|GetContainedItems (Variables|/Game/Blueprints/OreContainer.OreContainer_C|GetAs%20Box%20Slot _array_element))))))
      (:Gold
        (Rendering|Components|TextRender|SetText (Variables|Default|GetGold1) (Utilities|Text|ToText(Integer) (Utilities|Array|Length (Variables|/Script/TeamA.BoxSlot|GetContainedItems (Variables|/Game/Blueprints/OreContainer.OreContainer_C|GetAs%20Box%20Slot _array_element))))))
      (:Tungsten
        (Rendering|Components|TextRender|SetText (Variables|Default|GetTungsten1) (Utilities|Text|ToText(Integer) (Utilities|Array|Length (Variables|/Script/TeamA.BoxSlot|GetContainedItems (Variables|/Game/Blueprints/OreContainer.OreContainer_C|GetAs%20Box%20Slot _array_element)))))))))

(event EventTick
  (params (DeltaSeconds :type Float%20%28single-precision%29))
  ;[0.15 0.15 0.15 0.5] REMOVE AND FIND A WAY
  (Utilities|FlowControl|Delay 0.5)
  (for _array_element (stale EventBeginPlay _output_get)
    (switch Utilities|FlowControl|Switch|SwitchonESpecificTypes (Variables|/Game/Blueprints/OreContainer.OreContainer_C|GetAccepted%20Specific%20Type _array_element)
      (:Iron
        (Rendering|Components|TextRender|SetText (Variables|Default|GetIron1) (Utilities|Text|ToText(Integer) (Utilities|Array|Length (Variables|/Script/TeamA.BoxSlot|GetContainedItems (Variables|/Game/Blueprints/OreContainer.OreContainer_C|GetAs%20Box%20Slot _array_element))))))
      (:Copper
        (Rendering|Components|TextRender|SetText (Variables|Default|GetCopper1) (Utilities|Text|ToText(Integer) (Utilities|Array|Length (Variables|/Script/TeamA.BoxSlot|GetContainedItems (Variables|/Game/Blueprints/OreContainer.OreContainer_C|GetAs%20Box%20Slot _array_element))))))
      (:Gold
        (Rendering|Components|TextRender|SetText (Variables|Default|GetGold1) (Utilities|Text|ToText(Integer) (Utilities|Array|Length (Variables|/Script/TeamA.BoxSlot|GetContainedItems (Variables|/Game/Blueprints/OreContainer.OreContainer_C|GetAs%20Box%20Slot _array_element))))))
      (:Tungsten
        (Rendering|Components|TextRender|SetText (Variables|Default|GetTungsten1) (Utilities|Text|ToText(Integer) (Utilities|Array|Length (Variables|/Script/TeamA.BoxSlot|GetContainedItems (Variables|/Game/Blueprints/OreContainer.OreContainer_C|GetAs%20Box%20Slot _array_element)))))))))

(fn ConstructionScript)