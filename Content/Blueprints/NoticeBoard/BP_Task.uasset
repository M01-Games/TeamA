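; A notice board task poster that displays a job description and reports to the job manager when selected.
; On BeginPlay it creates a WB_OnBoardText widget from its Description and assigns it to its Widget component.
; SelectTask calls PickUpPoster on JobManager, passing itself and whether the job was already taken.
; The first selection latches the Taken flag and prints a debug string.
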(event EventBeginPlay
  ;[0.15 0.15 0.15 0.5] Setting the text on the notice
  (bind _returnvalue (UserInterface|CreateWidget "/Game/Blueprints/NoticeBoard/WB_OnBoardText.WB_OnBoardText_C" 0 (Variables|Default|GetDescription)))
  (UserInterface|SetWidget (Variables|Default|GetWidget) _returnvalue))

(event EventSelectTask
  (bind _self self)
  (bind _jobmanager (Variables|Default|GetJobManager))
  ;[0.15 0.15 0.15 0.5] Telling the job manager this job was selected
  (if (not (Variables|Default|GetTaken))
    (Variables|Default|SetTaken true)
    (Default|PickUpPoster _jobmanager _self false)
    (Development|PrintString "YUP")
    (else
      (Default|PickUpPoster _jobmanager _self true))))

(fn ConstructionScript)