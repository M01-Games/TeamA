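; Weapon assembly workstation where a handle is fitted to a blade and wrapped through BP_AssemblyMinigame.
; Enter reads the handle and project ItemSlot child actors, then uses inventory count and blade state to start assembly or wrapping.
; AttachHandle replaces the handle item with a BPHandleAssembly on the blade's HandlePoint and stores the minigame score.
; Exit ends or restarts the minigame and returns the handle to its slot.
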(event Custom|AttachHandle
  (Variables|/Game/Connor_Folder/Blade/BP_BladeParent.BP_BladeParent_C|SetIsBladeAttached? (Variables|Default|GetWeaponRef) true)
  (bind _ashandle_bp (Utilities|Casting|CastToHandle_BP (Variables|/Script/TeamA.ItemSlot|GetAttachedItem (Variables|Default|GetHandleItemSlot))))
  (bind _output_get (Variables|Default|SetAs%20Handle%20BP _ashandle_bp))
  (bind _returnvalue (Game|SpawnActorfromClass "/Game/Tyrell_folder/BPHandleAssembly.BPHandleAssembly_C" (Transformation|GetActorTransform _output_get) "AlwaysSpawn" "MultiplyWithRoot" 0 0.0 0))
  (bind _output_get_2 (Variables|/Game/Connor_Folder/Blade/BP_BladeParent.BP_BladeParent_C|SetAssemblyScore (Variables|Default|GetWeaponRef) (Math|Float|Truncate (Variables|/Game/Tyrell_folder/BP_AssemblyMinigame.BP_AssemblyMinigame_C|GetMinigameScore (Variables|Default|GetMiniGame)))))
  (Development|PrintString (Utilities|String|ToString(Integer) _output_get_2) true true "(R=1.000000,G=0.061260,B=0.801450,A=1.000000)" 1e+02)
  (Transformation|AttachComponentToComponent _returnvalue (Variables|/Game/Connor_Folder/Blade/BP_BladeParent.BP_BladeParent_C|GetHandlePoint (Variables|Default|GetWeaponRef)) "None" "SnapToTarget" "KeepWorld" "KeepWorld" true)
  (Class|ItemSlot|DeleteItem (Variables|Default|GetHandleItemSlot)))

(event Collision|EventActorBeginOverlap
  (params (OtherActor :type Actor%20Object%20Reference)))

(event EventTick
  (params (DeltaSeconds :type Float%20%28single-precision%29)))

(event EventEnter
  (params (Character :type Character%20Object%20Reference))
  (bind _inventory (Variables|Default|GetInventory))
  (bind _returnvalue (Utilities|Array|LastIndex _inventory))
  (bind _asitem_slot (Utilities|Casting|CastToItemSlot (Variables|/Script/Engine.ChildActorComponent|GetChildActor (Variables|Default|GetHandleBox))))
  (Variables|Default|SetHandleItemSlot _asitem_slot)
  (bind _asitem_slot_2 (Utilities|Casting|CastToItemSlot (Variables|/Script/Engine.ChildActorComponent|GetChildActor (Variables|Default|GetProjectBox))))
  (Variables|Default|SetProjectItemSlot _asitem_slot_2)
  (bind _asbp_blade_parent (Utilities|Casting|CastToBP_BladeParent (Variables|/Script/TeamA.ItemSlot|GetAttachedItem (Variables|Default|GetProjectItemSlot))))
  (Variables|Default|SetWeaponRef _asbp_blade_parent)
  (if (and (== (Utilities|Array|LastIndex (Variables|Default|GetInventory)) 0) (== (Variables|/Game/Connor_Folder/Blade/BP_BladeParent.BP_BladeParent_C|GetIsBladeAttached? (Variables|Default|GetWeaponRef)) true))
    (Development|PrintString "wrapping issue is true")
    (if (not (== (Variables|/Game/Connor_Folder/Blade/BP_BladeParent.BP_BladeParent_C|GetisBladeWrapped? (Variables|Default|GetWeaponRef)) true))
      (Default|Wrappinggame (Variables|Default|GetMiniGame)))
    (else
      (Development|PrintString "wrapping issue is false")
      ;[0.15 0.15 0.15 0.5] Please Note, this only works if only one item can be place on they, if it can't please re-evaluate the index so the conditions are correct
      (Development|PrintString (Utilities|String|ToString(Integer) _returnvalue))
      (if (== _returnvalue 1)
        (bind _asitem_slot_3 (Utilities|Casting|CastToItemSlot (Variables|/Script/Engine.ChildActorComponent|GetChildActor (Variables|Default|GetHandleBox))))
        (Variables|Default|SetHandleItemSlot _asitem_slot_3)
        (bind _asitem_slot_4 (Utilities|Casting|CastToItemSlot (Variables|/Script/Engine.ChildActorComponent|GetChildActor (Variables|Default|GetProjectBox))))
        (Variables|Default|SetProjectItemSlot _asitem_slot_4)
        (bind _ashandle_bp (Utilities|Casting|CastToHandle_BP (Variables|/Script/TeamA.ItemSlot|GetAttachedItem (Variables|Default|GetHandleItemSlot))))
        (Variables|Default|SetAs%20Handle%20BP _ashandle_bp)
        (Utilities|IsValid (Variables|/Script/TeamA.ItemSlot|GetAttachedItem (Variables|Default|GetProjectItemSlot))
          (:Is%20Valid
            (bind _asbp_blade_parent_2 (Utilities|Casting|CastToBP_BladeParent (Variables|/Script/TeamA.ItemSlot|GetAttachedItem (Variables|Default|GetProjectItemSlot))))
            (bind _output_get (Variables|Default|SetWeaponRef _asbp_blade_parent_2))
            (if (== (Variables|/Game/Connor_Folder/Blade/BP_BladeParent.BP_BladeParent_C|GetIsBladeAttached? _output_get) true)
              (Development|PrintString "we finally did it")
              (else
                (Transformation|SetActorLocation (Variables|Default|GetAs%20Handle%20BP) (Transformation|GetWorldLocation (Variables|/Game/Connor_Folder/Blade/BP_BladeParent.BP_BladeParent_C|GetHandlePoint (Variables|Default|GetWeaponRef))) false false)
                (Default|StartMinigame() (Variables|Default|GetMiniGame) self (Variables|Default|GetAs%20Handle%20BP)))))
          (:Is%20Not%20Valid
            (Development|PrintString "No item in slot")))))))

(event EventExit
  (params (Character :type Character%20Object%20Reference))
  (bind _inventory (Variables|Default|GetInventory))
  (bind _as_handle_bp (Variables|Default|GetAs%20Handle%20BP))
  (bind _returnvalue (Utilities|Array|LastIndex _inventory))
  (Variables|/Script/Engine.PlayerController|SetbShowMouseCursor (Game|GetPlayerController 0) false)
  (if (Utilities|Enum|Equal(Enum) (Variables|/Game/Tyrell_folder/BP_AssemblyMinigame.BP_AssemblyMinigame_C|GetCurrentState (Variables|Default|GetMiniGame)) "NewEnumerator2")
    (Default|EndMinigame (Variables|Default|GetMiniGame))
    ;[0.15 0.15 0.15 0.5] Please Note, this only works if only one item can be place on they, if it can't please re-evaluate the index so the conditions are correct
    (bind _returnvalue_2 (Actor|GetActorOfClass "/Game/Tyrell_folder/BPHandleAssembly.BPHandleAssembly_C"))
    (Variables|/Game/Tyrell_folder/BPHandleAssembly.BPHandleAssembly_C|SetWrapProgress _returnvalue_2 0.0)
    (Default|AltF4 (Variables|Default|GetMiniGame)))
  (if (or (== _returnvalue -1) (== _returnvalue 0))
    (Development|PrintString "Not enough items placed")
    (else
      (bind _outactors (Actor|GetAllActorsOfClass "/Game/Tyrell_folder/BP_AssemblyMinigame.BP_AssemblyMinigame_C"))
      (Default|RestartMinigame (Utilities|Array|Get(acopy) _outactors))))
  (Utilities|IsValid _as_handle_bp
    (:Is%20Valid
      (Transformation|SetActorLocation _as_handle_bp (Transformation|GetWorldLocation (Variables|/Script/Engine.Actor|GetRootComponent (Variables|Default|GetHandleItemSlot))) false false))))

(event EventBeginPlay
  (bind _returnvalue (Actor|GetActorOfClass "/Game/Tyrell_folder/BP_AssemblyMinigame.BP_AssemblyMinigame_C"))
  (Variables|Default|SetMiniGame _returnvalue)
  (bind _returnvalue_2 (Actor|GetActorOfClass "/Game/Connor_Folder/Blade/BP_BladeParent.BP_BladeParent_C"))
  (Variables|Default|SetWeaponRef _returnvalue_2)
  (bind _returnvalue_3 (Actor|GetActorOfClass "/Game/Tyrell_folder/BPHandleAssembly.BPHandleAssembly_C"))
  (Variables|Default|SetHandleAssemblyRef _returnvalue_3))

(fn ConstructionScript)