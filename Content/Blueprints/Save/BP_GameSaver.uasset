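; BP_GameSaver saves and restores forging-game progress through a single BP_GameSave slot.
; BeginPlay loads the slot after a short delay, or creates it with a player-and-poster-only first save.
; SaveGame records player, storage counts, weapons, jobs, deliveries and posters from actors found by class.
; Load respawns items into their containers and rebuilds blades and job posters, relying on GetAllActorsOfClass order to identify weapon holders.
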(event Custom|DoesGameSaveExist
  (bind _returnvalue (SaveGame|DoesSaveGameExist "SlotA"))
  (if _returnvalue
    (bind _returnvalue_2 (SaveGame|LoadGamefromSlot "SlotA"))
    (bind _asbp_game_save (Utilities|Casting|CastToBP_GameSave _returnvalue_2))
    (Variables|Default|SetGameSave _asbp_game_save)
    (Utilities|FlowControl|Delay 0.2)
    (CallFunction|Load)
    (else
      (bind _returnvalue_3 (SaveGame|CreateSaveGameObject "/Game/Blueprints/Save/BP_GameSave.BP_GameSave_C"))
      (bind _output_get (Variables|Default|SetGameSave _returnvalue_3))
      (SaveGame|SaveGametoSlot _output_get "SlotA")
      (CallFunction|Save true)
      (SaveGame|SaveGametoSlot (Variables|Default|GetGameSave) "SlotA"))))

(event Custom|SaveGame
  (CallFunction|Save false)
  (SaveGame|SaveGametoSlot (Variables|Default|GetGameSave) "SlotA"))

(event EventBeginPlay
  (CallFunction|DoesGameSaveExist))

(fn ConstructionScript)

(fn Save
  (params (First? :type Boolean))
  (bind _gamesave (Variables|Default|GetGameSave))
  (bind _gamesave_2 (Variables|Default|GetGameSave))
  (bind _oresinstorage (Variables|/Game/Blueprints/Save/BP_GameSave.BP_GameSave_C|GetOresInStorage _gamesave_2))
  (bind _asbp_first_person_character (Utilities|Casting|CastToBP_FirstPersonCharacter (Game|Player|GetPlayerPawn 0)))
  (Variables|/Game/Blueprints/Save/BP_GameSave.BP_GameSave_C|SetPlayerTransform _gamesave (Transformation|GetActorTransform _asbp_first_person_character))
  (bind _returnvalue (Actor|GetActorOfClass "/Game/Blueprints/XP/BP_RepPlaque.BP_RepPlaque_C"))
  (Variables|/Game/Blueprints/Save/BP_GameSave.BP_GameSave_C|SetPlayerData _gamesave (Utilities|Struct|MakePlayerData (Variables|/Game/Blueprints/BP_FirstPersonCharacter.BP_FirstPersonCharacter_C|GetG _asbp_first_person_character) (Variables|/Game/Blueprints/XP/BP_RepPlaque.BP_RepPlaque_C|GetLevel _returnvalue) (Variables|/Game/Blueprints/XP/BP_RepPlaque.BP_RepPlaque_C|GetXP _returnvalue)))
  (bind _returnvalue_2 (Actor|GetActorOfClass "/Game/Blueprints/BP_WallPoster.BP_WallPoster_C"))
  (Variables|/Game/Blueprints/Save/BP_GameSave.BP_GameSave_C|SetPosterEnchants (Variables|Default|GetGameSave) (Variables|/Game/Blueprints/BP_WallPoster.BP_WallPoster_C|GetNewVar _returnvalue_2))
  (if (not First?)
    (bind _outactors (Actor|GetAllActorsOfClass "/Game/Blueprints/OreContainer.OreContainer_C"))
    (for _array_element _outactors
      (Utilities|Map|Add _oresinstorage (Variables|/Game/Blueprints/OreContainer.OreContainer_C|GetAccepted%20Specific%20Type _array_element) (Utilities|Array|Length (Variables|/Script/TeamA.BoxSlot|GetContainedItems (Variables|/Game/Blueprints/OreContainer.OreContainer_C|GetAs%20Box%20Slot _array_element))))
      (bind (_keypin _valuepin) (Utilities|Map|ForEachLoop(Map) _oresinstorage)
        (:then
          (Development|PrintString (Utilities|String|Append (Utilities|String|ToString(Integer) _valuepin) (Utilities|String|EnumtoString _keypin))))))
    (Utilities|Array|Clear (Variables|/Game/Blueprints/Save/BP_GameSave.BP_GameSave_C|GetJobData (Variables|Default|GetGameSave)))
    (Utilities|Array|Clear (Variables|/Game/Blueprints/Save/BP_GameSave.BP_GameSave_C|GetweaponData (Variables|Default|GetGameSave)))
    (bind _outactors_2 (Actor|GetAllActorsOfClass "/Game/Blueprints/NoticeBoard/JobCompletion/WeaponHolder.WeaponHolder_C"))
    (for (_array_element_2 _array_index) _outactors_2
      (if (Variables|/Script/TeamA.ItemSlot|GetbIsOccupied (Variables|/Game/Blueprints/NoticeBoard/JobCompletion/WeaponHolder.WeaponHolder_C|GetItemSlot _array_element_2))
        (Utilities|IsValid (Variables|/Game/Blueprints/NoticeBoard/JobCompletion/WeaponHolder.WeaponHolder_C|GetBlade _array_element_2)
          (:Is%20Valid
            (Development|PrintString "Saving WeaponInfo")
            (Utilities|Array|Add (Variables|/Game/Blueprints/Save/BP_GameSave.BP_GameSave_C|GetweaponData (Variables|Default|GetGameSave)) (Utilities|Struct|MakeWeaponData _array_index (Utilities|Struct|MakeForgingData (Variables|/Script/TeamA.Project|GetbIsForged (Variables|/Game/Blueprints/NoticeBoard/JobCompletion/WeaponHolder.WeaponHolder_C|GetBlade _array_element_2)) (Variables|/Script/TeamA.Project|GetforgingProgress (Variables|/Game/Blueprints/NoticeBoard/JobCompletion/WeaponHolder.WeaponHolder_C|GetBlade _array_element_2)) (Variables|/Script/TeamA.Project|GetTotalForgeScore (Variables|/Game/Blueprints/NoticeBoard/JobCompletion/WeaponHolder.WeaponHolder_C|GetBlade _array_element_2)) (Variables|/Script/TeamA.Project|GetTotalForgeHits (Variables|/Game/Blueprints/NoticeBoard/JobCompletion/WeaponHolder.WeaponHolder_C|GetBlade _array_element_2)) (Variables|/Script/TeamA.Project|GetFinalForgeScore (Variables|/Game/Blueprints/NoticeBoard/JobCompletion/WeaponHolder.WeaponHolder_C|GetBlade _array_element_2)) (Variables|/Script/TeamA.Project|GetGrainStrength (Variables|/Game/Blueprints/NoticeBoard/JobCompletion/WeaponHolder.WeaponHolder_C|GetBlade _array_element_2))) (Utilities|Struct|MakeNonCodeData (Variables|/Game/Blueprints/Weapons/BP_BladeParent.BP_BladeParent_C|GetPoints (Variables|/Game/Blueprints/NoticeBoard/JobCompletion/WeaponHolder.WeaponHolder_C|GetBlade _array_element_2)) (Variables|/Game/Blueprints/Weapons/BP_BladeParent.BP_BladeParent_C|GetMetal%20Type (Variables|/Game/Blueprints/NoticeBoard/JobCompletion/WeaponHolder.WeaponHolder_C|GetBlade _array_element_2)) (Variables|/Game/Blueprints/Weapons/BP_BladeParent.BP_BladeParent_C|GetBlade%20Scratch%20Strength (Variables|/Game/Blueprints/NoticeBoard/JobCompletion/WeaponHolder.WeaponHolder_C|GetBlade _array_element_2)) (Variables|/Game/Blueprints/Weapons/BP_BladeParent.BP_BladeParent_C|GetAssemblyScore (Variables|/Game/Blueprints/NoticeBoard/JobCompletion/WeaponHolder.WeaponHolder_C|GetBlade _array_element_2)) (Variables|/Game/Blueprints/Weapons/BP_BladeParent.BP_BladeParent_C|GetIsBladeAttached? (Variables|/Game/Blueprints/NoticeBoard/JobCompletion/WeaponHolder.WeaponHolder_C|GetBlade _array_element_2)) (Variables|/Game/Blueprints/Weapons/BP_BladeParent.BP_BladeParent_C|GetWrappingScore (Variables|/Game/Blueprints/NoticeBoard/JobCompletion/WeaponHolder.WeaponHolder_C|GetBlade _array_element_2)) (Variables|/Game/Blueprints/Weapons/BP_BladeParent.BP_BladeParent_C|GetIsBladeWrapped? (Variables|/Game/Blueprints/NoticeBoard/JobCompletion/WeaponHolder.WeaponHolder_C|GetBlade _array_element_2)) (Utilities|GetClass (Variables|/Game/Blueprints/Weapons/BP_BladeParent.BP_BladeParent_C|GetHandle (Variables|/Game/Blueprints/NoticeBoard/JobCompletion/WeaponHolder.WeaponHolder_C|GetBlade _array_element_2))) (Variables|/Game/Blueprints/Weapons/BP_BladeParent.BP_BladeParent_C|GetAcceptableHandleType (Variables|/Game/Blueprints/NoticeBoard/JobCompletion/WeaponHolder.WeaponHolder_C|GetBlade _array_element_2)) (Utilities|GetClass (Variables|/Game/Blueprints/NoticeBoard/JobCompletion/WeaponHolder.WeaponHolder_C|GetBlade _array_element_2)) (Variables|/Game/Blueprints/Weapons/BP_BladeParent.BP_BladeParent_C|GetWeaponType (Variables|/Game/Blueprints/NoticeBoard/JobCompletion/WeaponHolder.WeaponHolder_C|GetBlade _array_element_2))))))
          (:Is%20Not%20Valid
            _)))
      (bind _returnvalue_3 (Actor|GetActorOfClass "/Game/Blueprints/NoticeBoard/BP_jobManager.BP_jobManager_C"))
      (if (Variables|/Game/Blueprints/NoticeBoard/JobCompletion/WeaponHolder.WeaponHolder_C|GetTaken _array_element_2)
        (Utilities|Array|Add (Variables|/Game/Blueprints/Save/BP_GameSave.BP_GameSave_C|GetJobData (Variables|Default|GetGameSave)) (Utilities|Struct|MakeJobdatasaveStruct (Variables|/Game/Blueprints/NoticeBoard/JobCompletion/WeaponHolder.WeaponHolder_C|GetRelatedJob _array_element_2) (Variables|/Game/Blueprints/NoticeBoard/WB_Poster.WB_Poster_C|GetDescriptions (Utilities|Array|Get(acopy) (Variables|/Game/Blueprints/NoticeBoard/BP_jobManager.BP_jobManager_C|GetJobWidgets _returnvalue_3) (Utilities|Array|FindItem (Variables|/Game/Blueprints/NoticeBoard/BP_jobManager.BP_jobManager_C|GetJobs _returnvalue_3) (Variables|/Game/Blueprints/NoticeBoard/JobCompletion/WeaponHolder.WeaponHolder_C|GetRelatedJob _array_element_2))))))))
    (bind _returnvalue_4 (Actor|GetActorOfClass "/Game/Blueprints/CrystalContainer.CrystalContainer_C"))
    (Variables|/Game/Blueprints/Save/BP_GameSave.BP_GameSave_C|SetAmethistAmmount (Variables|Default|GetGameSave) (Utilities|Array|Length (Variables|/Script/TeamA.BoxSlot|GetContainedItems (Variables|/Game/Blueprints/CrystalContainer.CrystalContainer_C|GetAs%20Box%20Slot _returnvalue_4))))
    (bind _outactors_3 (Actor|GetAllActorsOfClass "/Game/Blueprints/MouldHoulder.MouldHoulder_C"))
    (for _array_element_3 _outactors_3
      (Utilities|Map|Add (Variables|/Game/Blueprints/Save/BP_GameSave.BP_GameSave_C|GetMouldsInStorage (Variables|Default|GetGameSave)) (Variables|/Game/Blueprints/MouldHoulder.MouldHoulder_C|GetAccepted%20Specific%20Type _array_element_3) (Utilities|Array|Length (Variables|/Script/TeamA.BoxSlot|GetContainedItems (Variables|/Game/Blueprints/MouldHoulder.MouldHoulder_C|GetAs%20Box%20Slot _array_element_3)))))
    (bind _outactors_4 (Actor|GetAllActorsOfClass "/Game/Blueprints/HandlesBox.HandlesBox_C"))
    (for _array_element_4 _outactors_4
      (Utilities|Map|Add (Variables|/Game/Blueprints/Save/BP_GameSave.BP_GameSave_C|GetHandlesInStorage (Variables|Default|GetGameSave)) (Variables|/Game/Blueprints/HandlesBox.HandlesBox_C|GetAccepted%20Specific%20Type _array_element_4) (Utilities|Array|Length (Variables|/Script/TeamA.BoxSlot|GetContainedItems (Variables|/Game/Blueprints/HandlesBox.HandlesBox_C|GetAs%20Box%20Slot _array_element_4)))))
    (bind _returnvalue_5 (Actor|GetActorOfClass "/Game/Blueprints/Workstations/Ordering/UI/DeliveryPoint.DeliveryPoint_C"))
    (Variables|/Game/Blueprints/Save/BP_GameSave.BP_GameSave_C|SetDeliveryData (Variables|Default|GetGameSave) (Variables|/Game/Blueprints/Workstations/Ordering/UI/DeliveryPoint.DeliveryPoint_C|GetDeliveries _returnvalue_5))
    (bind _returnvalue_6 (Actor|GetActorOfClass "/Game/Blueprints/BP_AlloyPoster.BP_AlloyPoster_C"))
    (Variables|/Game/Blueprints/Save/BP_GameSave.BP_GameSave_C|SetPosterAlloy (Variables|Default|GetGameSave) (Variables|/Game/Blueprints/BP_AlloyPoster.BP_AlloyPoster_C|GetAlloys _returnvalue_6))))

(fn Load
  (bind _gamesave (Variables|Default|GetGameSave))
  (bind _gamesave_2 (Variables|Default|GetGameSave))
  (bind _gamesave_3 (Variables|Default|GetGameSave))
  (bind _gamesave_4 (Variables|Default|GetGameSave))
  (bind _playerdata (Variables|/Game/Blueprints/Save/BP_GameSave.BP_GameSave_C|GetPlayerData _gamesave))
  (bind _amethistammount (Variables|/Game/Blueprints/Save/BP_GameSave.BP_GameSave_C|GetAmethistAmmount _gamesave_2))
  (bind _deliverydata (Variables|/Game/Blueprints/Save/BP_GameSave.BP_GameSave_C|GetDeliveryData _gamesave_4))
  (bind _playertransform (Variables|/Game/Blueprints/Save/BP_GameSave.BP_GameSave_C|GetPlayerTransform _gamesave_3))
  (bind (_g _rep _xp) (Utilities|Struct|BreakPlayerData _playerdata))
  (bind _returnvalue (Actor|GetActorOfClass "/Game/Blueprints/XP/BP_RepPlaque.BP_RepPlaque_C"))
  (Variables|/Game/Blueprints/XP/BP_RepPlaque.BP_RepPlaque_C|SetLevel _returnvalue _rep)
  (Variables|/Game/Blueprints/XP/BP_RepPlaque.BP_RepPlaque_C|SetXP _returnvalue _xp)
  (Default|Started _returnvalue)
  (bind _returnvalue_2 (Actor|GetActorOfClass "/Game/Blueprints/BP_WallPoster.BP_WallPoster_C"))
  (Variables|/Game/Blueprints/BP_WallPoster.BP_WallPoster_C|SetNewVar _returnvalue_2 (Variables|/Game/Blueprints/Save/BP_GameSave.BP_GameSave_C|GetPosterEnchants (Variables|Default|GetGameSave)))
  (bind _asbp_first_person_character (Utilities|Casting|CastToBP_FirstPersonCharacter (Game|Player|GetPlayerPawn 0)))
  (Variables|/Game/Blueprints/BP_FirstPersonCharacter.BP_FirstPersonCharacter_C|SetG _asbp_first_person_character _g)
  (Transformation|SetActorTransform _asbp_first_person_character _playertransform false true)
  (Pawn|SetControlRotation (Game|GetPlayerController 0) (.Rotation (Math|Transform|BreakTransform _playertransform)))
  (bind _outactors (Actor|GetAllActorsOfClass "/Game/Blueprints/OreContainer.OreContainer_C"))
  (LocalVariables|SetOreStorage _outactors)
  (bind (_keypin _valuepin) (Utilities|Map|ForEachLoop(Map) (Variables|/Game/Blueprints/Save/BP_GameSave.BP_GameSave_C|GetOresInStorage (Variables|Default|GetGameSave)))
    (:then
      (if (> _valuepin 0)
        (bind _array_element (Utilities|Array|ForEachLoopwithBreak (LocalVariables|GetOreStorage) :!label _label)
          (:LoopBody
            (if (Utilities|Enum|Equal(Enum) _keypin (Variables|/Game/Blueprints/OreContainer.OreContainer_C|GetAccepted%20Specific%20Type _array_element))
              (for _index (range 1 _valuepin)
                (bind _returnvalue_3 (Game|SpawnActorfromClass :Class "/Game/Blueprints/BP_Ore1.BP_Ore1_C" :CollisionHandlingOverride "AlwaysSpawn" :TransformScaleMethod "MultiplyWithRoot" :Metal%20Type (CallFunction|SpecifictoEmetal _keypin) :Instigator 0))
                (Class|ItemSlot|AttachItem (Variables|/Game/Blueprints/OreContainer.OreContainer_C|GetAs%20Box%20Slot _array_element) _returnvalue_3)
                (Development|PrintString "Hello"))
              (goto _label Break))))))
    (:CompletedPin
      (Development|PrintString "Trying to load Weapon")
      (for _array_element_2 (Variables|/Game/Blueprints/Save/BP_GameSave.BP_GameSave_C|GetweaponData (Variables|Default|GetGameSave))
        (bind _outactors_2 (Actor|GetAllActorsOfClass "/Game/Blueprints/NoticeBoard/JobCompletion/WeaponHolder.WeaponHolder_C"))
        (Development|PrintString "DataHasBeenFound")
        (switch Utilities|FlowControl|Switch|SwitchonWeaponTypes (.Type (Utilities|Struct|BreakNonCodeData (.AllElse (Utilities|Struct|BreakWeaponData _array_element_2))))
          (:NewEnumerator0
            (LocalVariables|SetClass "/Game/Blueprints/Weapons/BP_BladeSword1.BP_BladeSword1_C"))
          (:NewEnumerator2
            (LocalVariables|SetClass "/Game/Blueprints/Weapons/BP_BladeDagger1.BP_BladeDagger1_C"))
          (:NewEnumerator1
            (LocalVariables|SetClass "/Game/Blueprints/Weapons/BP_Axe.BP_Axe_C")))
        (bind _returnvalue_4 (Game|SpawnActorfromClass (LocalVariables|GetClass) (Math|Transform|MakeTransform "0, 0, 0" "0, 0, 0" "1.000000,1.000000,1.000000") "AlwaysSpawn" "MultiplyWithRoot" 0 0))
        (Development|PrintString "SHOULD HAVE SPAWNED")
        (bind _asbp_blade_parent (Utilities|Casting|CastToBP_BladeParent _returnvalue_4)
          (:then
            (bind _output_get (LocalVariables|SetCurrentBlade _asbp_blade_parent))
            (CallFunction|SetWeaponStats _output_get (.IsForged (Utilities|Struct|BreakForgingData (.ForgingData (Utilities|Struct|BreakWeaponData _array_element_2)))) (.ForgingProgress (Utilities|Struct|BreakForgingData (.ForgingData (Utilities|Struct|BreakWeaponData _array_element_2)))) (.TotalForgeScore (Utilities|Struct|BreakForgingData (.ForgingData (Utilities|Struct|BreakWeaponData _array_element_2)))) (.TotalForgeHits (Utilities|Struct|BreakForgingData (.ForgingData (Utilities|Struct|BreakWeaponData _array_element_2)))) (.FinalForgeScore (Utilities|Struct|BreakForgingData (.ForgingData (Utilities|Struct|BreakWeaponData _array_element_2)))) (.GrainStrength (Utilities|Struct|BreakForgingData (.ForgingData (Utilities|Struct|BreakWeaponData _array_element_2)))) (.Points (Utilities|Struct|BreakNonCodeData (.AllElse (Utilities|Struct|BreakWeaponData _array_element_2)))) (.Metal (Utilities|Struct|BreakNonCodeData (.AllElse (Utilities|Struct|BreakWeaponData _array_element_2)))) (.BladeScratchStrength (Utilities|Struct|BreakNonCodeData (.AllElse (Utilities|Struct|BreakWeaponData _array_element_2)))) (.AssemblyScore (Utilities|Struct|BreakNonCodeData (.AllElse (Utilities|Struct|BreakWeaponData _array_element_2)))) (.IsAssembled (Utilities|Struct|BreakNonCodeData (.AllElse (Utilities|Struct|BreakWeaponData _array_element_2)))) (.WrappingScore (Utilities|Struct|BreakNonCodeData (.AllElse (Utilities|Struct|BreakWeaponData _array_element_2)))) (.IsWrapped (Utilities|Struct|BreakNonCodeData (.AllElse (Utilities|Struct|BreakWeaponData _array_element_2)))) (.Handle (Utilities|Struct|BreakNonCodeData (.AllElse (Utilities|Struct|BreakWeaponData _array_element_2)))) (.AcceptedHandleType (Utilities|Struct|BreakNonCodeData (.AllElse (Utilities|Struct|BreakWeaponData _array_element_2)))) (.BladeType (Utilities|Struct|BreakNonCodeData (.AllElse (Utilities|Struct|BreakWeaponData _array_element_2)))) (.Type (Utilities|Struct|BreakNonCodeData (.AllElse (Utilities|Struct|BreakWeaponData _array_element_2)))))
            (Class|ItemSlot|AttachItem (Variables|/Game/Blueprints/NoticeBoard/JobCompletion/WeaponHolder.WeaponHolder_C|GetItemSlot (Utilities|Array|Get(acopy) _outactors_2 (.HolderIndex (Utilities|Struct|BreakWeaponData _array_element_2)))) (LocalVariables|GetCurrentBlade))
            (if (.IsAssembled (Utilities|Struct|BreakNonCodeData (.AllElse (Utilities|Struct|BreakWeaponData _array_element_2))))
              (switch Utilities|FlowControl|Switch|SwitchonWeaponTypes (.Type (Utilities|Struct|BreakNonCodeData (.AllElse (Utilities|Struct|BreakWeaponData _array_element_2))))
                (:NewEnumerator0
                  (bind _returnvalue_5 (Game|SpawnActorfromClass "/Game/Blueprints/Weapons/Handles/Parent_Handle.Parent_Handle_C" (Math|Transform|MakeTransform "0, 0, 0" "0, 0, 0" "1.000000,1.000000,1.000000") "AlwaysSpawn" "MultiplyWithRoot" 0 0.0 0 :!label _label_2))
                  (Transformation|AttachComponentToComponent _returnvalue_5 (Variables|/Game/Blueprints/Weapons/BP_BladeParent.BP_BladeParent_C|GetHandlePoint (LocalVariables|GetCurrentBlade)) "None" "SnapToTarget" "SnapToTarget" "KeepWorld" true))
                (:NewEnumerator2
                  (goto _label_2))
                (:NewEnumerator1
                  (bind _returnvalue_6 (Game|SpawnActorfromClass "/Game/Blueprints/Weapons/Handles/BPAxeHandleAssembly.BPAxeHandleAssembly_C" (Math|Transform|MakeTransform "0, 0, 0" "0, 0, 0" "1.000000,1.000000,1.000000") "AlwaysSpawn" "MultiplyWithRoot" 0 0.0 0))
                  (Transformation|AttachComponentToComponent _returnvalue_6 (Variables|/Game/Blueprints/Weapons/BP_BladeParent.BP_BladeParent_C|GetHandlePoint (LocalVariables|GetCurrentBlade)) "None" "SnapToTarget" "SnapToTarget" "KeepWorld" true)))))
          (:CastFailed
            (Development|PrintString "FAILURE"))))
      (for (_array_element_3 _array_index) (Variables|/Game/Blueprints/Save/BP_GameSave.BP_GameSave_C|GetJobData (Variables|Default|GetGameSave))
        (bind _outactors_3 (Actor|GetAllActorsOfClass "/Game/Blueprints/NoticeBoard/JobCompletion/WeaponHolder.WeaponHolder_C"))
        (Variables|/Game/Blueprints/NoticeBoard/JobCompletion/WeaponHolder.WeaponHolder_C|SetRelatedJob (Utilities|Array|Get(acopy) _outactors_3 _array_index) (.Job (Utilities|Struct|BreakJobdatasaveStruct _array_element_3)))
        (Variables|/Game/Blueprints/NoticeBoard/JobCompletion/WeaponHolder.WeaponHolder_C|SetTaken (Utilities|Array|Get(acopy) _outactors_3 _array_index) true)
        (bind _returnvalue_7 (UserInterface|CreateWidget "/Game/Blueprints/NoticeBoard/WB_Poster.WB_Poster_C" 0 (.DescriptionUsed (Utilities|Struct|BreakJobdatasaveStruct _array_element_3))))
        (bind _returnvalue_8 (Actor|GetActorOfClass "/Game/Blueprints/NoticeBoard/BP_jobManager.BP_jobManager_C"))
        (Utilities|Array|Add (Variables|/Game/Blueprints/NoticeBoard/BP_jobManager.BP_jobManager_C|GetJobs _returnvalue_8) (.Job (Utilities|Struct|BreakJobdatasaveStruct _array_element_3)))
        (Utilities|Array|Add (Variables|/Game/Blueprints/NoticeBoard/BP_jobManager.BP_jobManager_C|GetJobWidgets _returnvalue_8) _returnvalue_7)
        (bind _returnvalue_9 (Game|SpawnActorfromClass "/Game/Blueprints/NoticeBoard/BP_Task.BP_Task_C" (Math|Transform|MakeTransform (.location (Transformation|GetWorldTransform (Variables|/Game/Blueprints/NoticeBoard/JobCompletion/WeaponHolder.WeaponHolder_C|GetPosterSpot (Utilities|Array|Get(acopy) _outactors_3 _array_index)))) (.rotation (Transformation|GetWorldTransform (Variables|/Game/Blueprints/NoticeBoard/JobCompletion/WeaponHolder.WeaponHolder_C|GetPosterSpot (Utilities|Array|Get(acopy) _outactors_3 _array_index)))) "1.000000,1.000000,1.000000") "AlwaysSpawn" "MultiplyWithRoot" 0 _returnvalue_8 (.DescriptionUsed (Utilities|Struct|BreakJobdatasaveStruct _array_element_3)) true (Utilities|Array|Get(acopy) _outactors_3 _array_index) 0))
        (Utilities|Array|Add (Variables|/Game/Blueprints/NoticeBoard/BP_jobManager.BP_jobManager_C|GetJobPosters _returnvalue_8) _returnvalue_9))
      (if (> _amethistammount 0)
        (for _index_2 (range 1 _amethistammount)
          (bind _returnvalue_10 (Game|SpawnActorfromClass "/Game/Blueprints/Crystal_.Crystal__C" (Math|Transform|MakeTransform "0, 0, 0" "0, 0, 0" "1.000000,1.000000,1.000000") "AlwaysSpawn" "MultiplyWithRoot" 0 0))
          (bind _returnvalue_11 (Actor|GetActorOfClass "/Game/Blueprints/CrystalContainer.CrystalContainer_C"))
          (Class|ItemSlot|AttachItem (Variables|/Game/Blueprints/CrystalContainer.CrystalContainer_C|GetAs%20Box%20Slot _returnvalue_11) _returnvalue_10)))
      (bind _outactors_4 (Actor|GetAllActorsOfClass "/Game/Blueprints/MouldHoulder.MouldHoulder_C"))
      (LocalVariables|SetMouldStorage _outactors_4)
      (bind (_keypin_2 _valuepin_2) (Utilities|Map|ForEachLoop(Map) (Variables|/Game/Blueprints/Save/BP_GameSave.BP_GameSave_C|GetMouldsInStorage (Variables|Default|GetGameSave)))
        (:then
          (if (> _valuepin_2 0)
            (bind _array_element_4 (Utilities|Array|ForEachLoopwithBreak (LocalVariables|GetMouldStorage) :!label _label_3)
              (:LoopBody
                (if (Utilities|Enum|Equal(Enum) _keypin_2 (Variables|/Game/Blueprints/MouldHoulder.MouldHoulder_C|GetAccepted%20Specific%20Type _array_element_4))
                  (for _index_3 (range 1 _valuepin_2)
                    (switch Utilities|FlowControl|Switch|SwitchonESpecificTypes (Variables|/Game/Blueprints/MouldHoulder.MouldHoulder_C|GetAccepted%20Specific%20Type _array_element_4)
                      (:AxeMould
                        (LocalVariables|SetMouldType "NewEnumerator1"))
                      (:SwordMould
                        (LocalVariables|SetMouldType "NewEnumerator0"))
                      (:DaggerMould
                        (LocalVariables|SetMouldType "NewEnumerator2")))
                    (bind _returnvalue_12 (Game|SpawnActorfromClass "/Game/Blueprints/BP_Mould.BP_Mould_C" (Math|Transform|MakeTransform "0, 0, 0" "0, 0, 0" "1.000000,1.000000,1.000000") "AlwaysSpawn" "MultiplyWithRoot" 0 (LocalVariables|GetMouldType) "NewEnumerator0" 0 0))
                    (Class|ItemSlot|AttachItem (Variables|/Game/Blueprints/MouldHoulder.MouldHoulder_C|GetAs%20Box%20Slot _array_element_4) _returnvalue_12))
                  (goto _label_3 Break))))))
        (:CompletedPin
          (bind _outactors_5 (Actor|GetAllActorsOfClass "/Game/Blueprints/HandlesBox.HandlesBox_C"))
          (LocalVariables|SetHandleStorage _outactors_5)
          (bind (_keypin_3 _valuepin_3) (Utilities|Map|ForEachLoop(Map) (Variables|/Game/Blueprints/Save/BP_GameSave.BP_GameSave_C|GetHandlesInStorage (Variables|Default|GetGameSave)))
            (:then
              (if (> _valuepin_3 0)
                (bind _array_element_5 (Utilities|Array|ForEachLoopwithBreak (LocalVariables|GetHandleStorage) :!label _label_4)
                  (:LoopBody
                    (if (Utilities|Enum|Equal(Enum) _keypin_3 (Variables|/Game/Blueprints/HandlesBox.HandlesBox_C|GetAccepted%20Specific%20Type _array_element_5))
                      (for _index_4 (range 1 _valuepin_3)
                        (switch Utilities|FlowControl|Switch|SwitchonESpecificTypes (Variables|/Game/Blueprints/HandlesBox.HandlesBox_C|GetAccepted%20Specific%20Type _array_element_5)
                          (:SwordHandle
                            (bind _returnvalue_13 (Game|SpawnActorfromClass "/Game/Blueprints/Weapons/Handles/Sword_And_Dagger_Handle_BP.Sword_And_Dagger_Handle_BP_C" (Math|Transform|MakeTransform "0, 0, 0" "0, 0, 0" "1.000000,1.000000,1.000000") "AlwaysSpawn" "MultiplyWithRoot" 0 0))
                            (Class|ItemSlot|AttachItem (Variables|/Game/Blueprints/HandlesBox.HandlesBox_C|GetAs%20Box%20Slot _array_element_5) _returnvalue_13))
                          (:AxeHandle
                            (bind _returnvalue_14 (Game|SpawnActorfromClass "/Game/Blueprints/Weapons/Handles/Axe_Handle.Axe_Handle_C" (Math|Transform|MakeTransform "0, 0, 0" "0, 0, 0" "1.000000,1.000000,1.000000") "AlwaysSpawn" "MultiplyWithRoot" 0 0))
                            (Class|ItemSlot|AttachItem (Variables|/Game/Blueprints/HandlesBox.HandlesBox_C|GetAs%20Box%20Slot _array_element_5) _returnvalue_14))))
                      (goto _label_4 Break))))))
            (:CompletedPin
              (bind _returnvalue_15 (Actor|GetActorOfClass "/Game/Blueprints/BP_AlloyPoster.BP_AlloyPoster_C"))
              (Variables|/Game/Blueprints/BP_AlloyPoster.BP_AlloyPoster_C|SetAlloys _returnvalue_15 (Variables|/Game/Blueprints/Save/BP_GameSave.BP_GameSave_C|GetPosterAlloy (Variables|Default|GetGameSave)))
              (if (not (Utilities|Array|IsEmpty _deliverydata))
                (bind _returnvalue_16 (Actor|GetActorOfClass "/Game/Blueprints/Workstations/Ordering/UI/DeliveryPoint.DeliveryPoint_C"))
                (Variables|/Game/Blueprints/Workstations/Ordering/UI/DeliveryPoint.DeliveryPoint_C|SetDeliveries _returnvalue_16 _deliverydata)
                (Default|Deliver _returnvalue_16)))))))))

(fn SetWeaponStats
  (params (Target :type BP%20Blade%20Parent%20Object%20Reference) (IsForged :type Boolean) (ForgingProgress :type Float%20%28double-precision%29) (TotalForgeScore :type Float%20%28double-precision%29) (TotalForgeHits :type Integer) (FinalForgeScore :type Float%20%28double-precision%29) (GrainStrength :type Float%20%28double-precision%29) (Points :type Array%20of%20Floats%20%28double-precision%29) (Metal :type E_MetalType%20Enum :default "NewEnumerator0") (BladeScratchStrength :type Float%20%28double-precision%29) (AssemblyScore :type Integer) (IsAssembled :type Boolean) (WrappingScore :type Integer) (IsWrapped :type Boolean) (Handle :type Actor%20Class%20Reference) (AcceptedHandleType :type HandleTypes%20Enum :default "NewEnumerator0") (BladeType :type Actor%20Class%20Reference) (WeaponType :type WeaponTypes%20Enum :default "NewEnumerator0"))
  (Variables|/Game/Blueprints/Weapons/BP_BladeParent.BP_BladeParent_C|SetWeaponType Target WeaponType)
  (Variables|/Script/TeamA.Project|SetbIsForged Target IsForged)
  (Variables|/Script/TeamA.Project|SetforgingProgress Target ForgingProgress)
  (Variables|/Script/TeamA.Project|SetTotalForgeScore Target TotalForgeScore)
  (Variables|/Script/TeamA.Project|SetTotalForgeHits Target TotalForgeHits)
  (Variables|/Script/TeamA.Project|SetFinalForgeScore Target FinalForgeScore)
  (Variables|/Script/TeamA.Project|SetGrainStrength Target GrainStrength)
  (Variables|/Game/Blueprints/Weapons/BP_BladeParent.BP_BladeParent_C|SetPoints Target Points)
  (Variables|/Game/Blueprints/Weapons/BP_BladeParent.BP_BladeParent_C|SetMetal%20Type Target Metal)
  (Variables|/Game/Blueprints/Weapons/BP_BladeParent.BP_BladeParent_C|SetBlade%20Scratch%20Strength Target BladeScratchStrength)
  (Variables|/Game/Blueprints/Weapons/BP_BladeParent.BP_BladeParent_C|SetAssemblyScore Target AssemblyScore)
  (Variables|/Game/Blueprints/Weapons/BP_BladeParent.BP_BladeParent_C|SetIsBladeAttached? Target IsAssembled)
  (Variables|/Game/Blueprints/Weapons/BP_BladeParent.BP_BladeParent_C|SetWrappingScore Target WrappingScore)
  (Variables|/Game/Blueprints/Weapons/BP_BladeParent.BP_BladeParent_C|SetIsBladeWrapped? Target IsWrapped)
  (Variables|/Game/Blueprints/Weapons/BP_BladeParent.BP_BladeParent_C|SetAcceptableHandleType Target AcceptedHandleType))