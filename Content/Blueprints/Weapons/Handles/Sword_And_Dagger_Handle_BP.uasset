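; Sword and dagger handle for the assembly minigame, with two nails that are driven in one after the other.
; NailAnimation raises a clamped Alpha by the minigame's Points divided by its Handle's PointProgress, then lerps the active nail between start and end markers.
; When the first nail reaches full Alpha, Alpha restarts and later calls move the second nail.
; ResetAnimation returns both nails to their start positions.
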(event Custom|ResetAnimation
  (Variables|Default|SetIsNail1Done? false)
  (Variables|Default|SetAlpha 0.0)
  (Transformation|SetWorldLocation (Variables|Default|GetNail_01) (Math|Vector|Lerp(Vector) (Transformation|GetWorldLocation (Variables|Default|GetNailStart_01)) (Transformation|GetWorldLocation (Variables|Default|GetNailEnd_01)) 0.0) false false)
  (Transformation|SetWorldLocation (Variables|Default|GetNail_02) (Math|Vector|Lerp(Vector) (Transformation|GetWorldLocation (Variables|Default|GetNailStart_02)) (Transformation|GetWorldLocation (Variables|Default|GetNailEnd_02)) 0.0) false false))

(event Collision|EventActorBeginOverlap
  (params (OtherActor :type Actor%20Object%20Reference)))

(event EventTick
  (params (DeltaSeconds :type Float%20%28single-precision%29)))

(fn ConstructionScript)

(fn NailAnimation
  ;[0.15 0.15 0.15 0.5] First Nail
  (if (Variables|Default|GetIsNail1Done?)
    ;[0.15 0.15 0.15 0.5] Second Nail
    (bind _returnvalue (Actor|GetActorOfClass "/Game/Blueprints/Workstations/Assembly/BP_AssemblyMinigame.BP_AssemblyMinigame_C"))
    (bind _output_get (Variables|Default|SetAlpha (Math|Float|Clamp(Float) (+ (Variables|Default|GetAlpha) (/ (Variables|/Game/Blueprints/Workstations/Assembly/BP_AssemblyMinigame.BP_AssemblyMinigame_C|GetPoints _returnvalue) (Variables|Sword_And_Dagger_Handle_BP_C|GetPointProgress (Variables|/Game/Blueprints/Workstations/Assembly/BP_AssemblyMinigame.BP_AssemblyMinigame_C|GetHandle _returnvalue)))))))
    (Development|PrintString (Utilities|String|ToString(Float) _output_get))
    (Transformation|SetWorldLocation (Variables|Default|GetNail_02) (Math|Vector|Lerp(Vector) (Transformation|GetWorldLocation (Variables|Default|GetNailStart_02)) (Transformation|GetWorldLocation (Variables|Default|GetNailEnd_02)) (Variables|Default|GetAlpha)) false false)
    (else
      (Development|PrintString "P is being pressed from handle_BP")
      (bind _returnvalue_2 (Actor|GetActorOfClass "/Game/Blueprints/Workstations/Assembly/BP_AssemblyMinigame.BP_AssemblyMinigame_C"))
      (bind _output_get_2 (Variables|Default|SetAlpha (Math|Float|Clamp(Float) (+ (Variables|Default|GetAlpha) (/ (Variables|/Game/Blueprints/Workstations/Assembly/BP_AssemblyMinigame.BP_AssemblyMinigame_C|GetPoints _returnvalue_2) (Variables|Sword_And_Dagger_Handle_BP_C|GetPointProgress (Variables|/Game/Blueprints/Workstations/Assembly/BP_AssemblyMinigame.BP_AssemblyMinigame_C|GetHandle _returnvalue_2)))))))
      (Development|PrintString (Utilities|String|ToString(Float) _output_get_2))
      (Transformation|SetWorldLocation (Variables|Default|GetNail_01) (Math|Vector|Lerp(Vector) (Transformation|GetWorldLocation (Variables|Default|GetNailStart_01)) (Transformation|GetWorldLocation (Variables|Default|GetNailEnd_01)) (Variables|Default|GetAlpha)) false false)
      (if (== (Variables|Default|GetAlpha) 1.0)
        (Variables|Default|SetIsNail1Done? true)
        (Variables|Default|SetAlpha 0.0)
        (else
          (Variables|Default|SetIsNail1Done? false))))))