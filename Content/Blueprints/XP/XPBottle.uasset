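; XPBottle is a Blueprint actor that visualizes reputation XP as a fill level.
; On BeginPlay it finds and caches the BP_RepPlaque actor in the level.
; The XPchange event, after a tiny retriggerable delay, scales the Cylinder002 mesh along Z from empty to full by the plaque's XP over RequiredXP ratio.
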(event Custom|XP%20change
  (bind _repplaque (Variables|Default|GetRepPlaque))
  (Utilities|FlowControl|RetriggerableDelay 0.001)
  (Transformation|SetRelativeScale3D (Variables|Default|GetCylinder_002) (Math|Vector|Lerp(Vector) "1.000000,1.000000,0.000000" "1.000000,1.000000,1.000000" (/ (Variables|/Game/Blueprints/XP/BP_RepPlaque.BP_RepPlaque_C|GetXP _repplaque) (Variables|/Game/Blueprints/XP/BP_RepPlaque.BP_RepPlaque_C|GetRequiredXP _repplaque)))))

(event EventBeginPlay
  (bind _returnvalue (Actor|GetActorOfClass "/Game/Blueprints/XP/BP_RepPlaque.BP_RepPlaque_C"))
  (Variables|Default|SetRepPlaque _returnvalue))

(fn ConstructionScript)