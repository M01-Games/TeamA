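; BP_DayQuestLog is an actor that settles the day's completed jobs and awards XP for those that were won.
; On BeginPlay it caches the BP_RepPlaque actor, which holds the XP total.
; Its Who? event prints each job's name as lived or died in green or red, summing monster XP worth for wins.
; It then clears the list, adds double that sum to the plaque and refreshes its title and level.
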(event Custom|Who?
  (bind _repandxp (Variables|Default|GetRepAndXP))
  (Variables|Default|SetXPAmmount 0)
  (for _array_element (Variables|Default|GetJobs%20Completed)
    (if (.won? _array_element)
      (Development|PrintString (Utilities|String|Append (.name _array_element) " Lived") true true "(R=0.083213,G=1.000000,B=0.000000,A=1.000000)" 11111.0)
      (Variables|Default|SetXPAmmount (+ (Variables|Default|GetXPAmmount) (.XPworth (Utilities|Struct|BreakMonsterInfo (.monster _array_element)))))
      (else
        (Development|PrintString (Utilities|String|Append (.name _array_element) " Died") true true "(R=1.000000,G=0.000000,B=0.000000,A=1.000000)" 1111.0))))
  (Utilities|Array|Clear (Variables|Default|GetJobs%20Completed))
  (Variables|/Game/Blueprints/XP/BP_RepPlaque.BP_RepPlaque_C|SetXP _repandxp (+ (Variables|/Game/Blueprints/XP/BP_RepPlaque.BP_RepPlaque_C|GetXP _repandxp) (* (Variables|Default|GetXPAmmount) 2)))
  (Default|SetTitleandLevel (Variables|Default|GetRepAndXP)))

(event EventBeginPlay
  (bind _returnvalue (Actor|GetActorOfClass "/Game/Blueprints/XP/BP_RepPlaque.BP_RepPlaque_C"))
  (Variables|Default|SetRepAndXP _returnvalue))

(event Collision|EventActorBeginOverlap
  (params (OtherActor :type Actor%20Object%20Reference)))

(event EventTick
  (params (DeltaSeconds :type Float%20%28single-precision%29)))

(fn ConstructionScript)