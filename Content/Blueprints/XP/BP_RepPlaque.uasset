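; Reputation plaque actor that displays the player's rank title and level on two text renders and finds an XPBottle in the level.
; SetTitleAndLevel recursively spends XP against the requirement to level up, refreshing the text and calling the bottle's XPChange each time.
; SetRequired maps levels to thresholds and rank titles from Novice to Grand Master, using an incremental formula beyond the hand-set levels.
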(event Custom|SetTitleAndLevel
  (if (>= (Variables|Default|GetXP) (Variables|Default|GetRequiredXP))
    (Variables|Default|SetXP (- (Variables|Default|GetXP) (Variables|Default|GetRequiredXP)))
    (Math|Integer|IncrementInt (Variables|Default|GetLevel)
      (:%20%20
        (CallFunction|SetRequired)
        (Rendering|Components|TextRender|SetText (Variables|Default|GetTextRender) (Utilities|Text|ToText(String) (Variables|Default|GetTitle)))
        (Rendering|Components|TextRender|SetText (Variables|Default|GetTextRender1) (Utilities|Text|ToText(String) (Utilities|String|Append "Level: " (Utilities|String|ToString(Integer) (Variables|Default|GetLevel)))))
        (Default|XPChange (Variables|Default|Getbottle))
        (CallFunction|SetTitleandLevel)))))

(event EventBeginPlay
  (bind _returnvalue (Actor|GetActorOfClass "/Game/Blueprints/XP/XPBottle.XPBottle_C"))
  (bind _output_get (Variables|Default|Setbottle _returnvalue))
  (Default|XPChange _output_get)
  (CallFunction|SetRequired)
  (Rendering|Components|TextRender|SetText (Variables|Default|GetTextRender) (Utilities|Text|ToText(String) (Variables|Default|GetTitle)))
  (CallFunction|SetTitleandLevel)
  (Rendering|Components|TextRender|SetText (Variables|Default|GetTextRender1) (Utilities|Text|ToText(String) (Utilities|String|Append "Level: " (Utilities|String|ToString(Integer) (Variables|Default|GetLevel))))))

(event Collision|EventActorBeginOverlap
  (params (OtherActor :type Actor%20Object%20Reference)))

(event EventTick
  (params (DeltaSeconds :type Float%20%28single-precision%29)))

(fn ConstructionScript)

(fn SetRequired
  (switch int (Variables|Default|GetLevel)
    (:Default
      (Variables|Default|SetRequiredXP (+ (Variables|Default|GetRequiredXP) (* (- (Variables|Default|GetLevel) 12) 5)))
      (if (>= (Variables|Default|GetLevel) 100)
        (Variables|Default|SetTitle "Grand Master")
        (else
          (Variables|Default|SetTitle "Master"))))
    (:1
      (Variables|Default|SetRequiredXP 2)
      (Variables|Default|SetTitle "Novice"))
    (:2
      (Variables|Default|SetRequiredXP 4))
    (:3
      (Variables|Default|SetRequiredXP 6))
    (:4
      (Variables|Default|SetRequiredXP 8)
      (Variables|Default|SetTitle "Beginner"))
    (:5
      (Variables|Default|SetRequiredXP 10))
    (:6
      (Variables|Default|SetRequiredXP 12)
      (Variables|Default|SetTitle "Intermediate"))
    (:7
      (Variables|Default|SetRequiredXP 15))
    (:8
      (Variables|Default|SetRequiredXP 18)
      (Variables|Default|SetTitle "Advanced"))
    (:9
      (Variables|Default|SetRequiredXP 21))
    (:10
      (Variables|Default|SetRequiredXP 24)
      (Variables|Default|SetTitle "Expert"))
    (:11
      (Variables|Default|SetRequiredXP 27))
    (:12
      (Variables|Default|SetRequiredXP 30)
      (Variables|Default|SetTitle "Master"))))