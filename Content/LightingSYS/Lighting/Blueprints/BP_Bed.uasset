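; BP_Bed is an interactable bed that lets the player end the day once the time manager's clock passes a sleep threshold.
; A trigger box toggles input and a prompt, and interacting locks movement, fades the camera and shows a newspaper widget.
; Depending on the widget's News result, it continues immediately or awaits another interact through a DoOnce gate.
; It then skips to morning, updates the day quest log, saves and opens the Connor level.
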(event OnComponentBeginOverlap(TriggerBox)
  (params (OverlappedComponent :type Primitive%20Component%20Object%20Reference) (OtherActor :type Actor%20Object%20Reference) (OtherComp :type Primitive%20Component%20Object%20Reference) (OtherBodyIndex :type Integer) (bFromSweep :type Boolean) (SweepResult :type Hit%20Result%20Structure%20%28by%20ref%29))
  (Utilities|Casting|CastToCharacter OtherActor)
  (Input|EnableInput (Game|GetPlayerController 0))
  (Rendering|SetVisibility (Variables|Default|GetPromptText) true false))

(event OnComponentEndOverlap(TriggerBox)
  (params (OverlappedComponent :type Primitive%20Component%20Object%20Reference) (OtherActor :type Actor%20Object%20Reference) (OtherComp :type Primitive%20Component%20Object%20Reference) (OtherBodyIndex :type Integer))
  (Utilities|Casting|CastToCharacter OtherActor)
  (Input|DisableInput (Game|GetPlayerController 0))
  (Rendering|SetVisibility (Variables|Default|GetPromptText) false false))

(event Custom|Save
  (bind _returnvalue (Actor|GetActorOfClass "/Game/Blueprints/Save/BP_GameSaver.BP_GameSaver_C"))
  (Utilities|IsValid _returnvalue
    (:Is%20Valid
      (Default|SaveGame _returnvalue))))

(event Input|EnhancedActionEvents|EnhancedInputActionIA_Interact
  (params (ActionValue :type Boolean) (ElapsedSeconds :type Float%20%28double-precision%29) (TriggeredSeconds :type Float%20%28double-precision%29) (InputAction :type Input%20Action%20Object%20Reference :default "/Game/Input/Actions/IA_Interact.IA_Interact"))
  (:Started
    (Utilities|FlowControl|DoOnce true
      (:Completed
        (Widget|RemovefromParent (Variables|Default|GetNewsPaper))
        (Default|SkiptoMorning (Variables|Default|GetTimeManagerRef))
        (bind _returnvalue (Actor|GetActorOfClass "/Game/Blueprints/XP/BP_DayQuestLog.BP_DayQuestLog_C"))
        (Default|Who? _returnvalue)
        (CallFunction|Save)
        (Utilities|FlowControl|Delay 0.2)
        (Game|OpenLevel(byObjectReference) "/Game/Levels/Connor/Connor.Connor")))))

(event Input|EnhancedActionEvents|EnhancedInputActionIA_Interact
  (params (ActionValue :type Boolean) (ElapsedSeconds :type Float%20%28double-precision%29) (TriggeredSeconds :type Float%20%28double-precision%29) (InputAction :type Input%20Action%20Object%20Reference :default "/Game/Input/Actions/IA_Interact.IA_Interact"))
  (:Started
    (Utilities|FlowControl|DoOnce false :!label _label
      (:Completed
        (if (and (> (Variables|/Game/LightingSYS/Lighting/Blueprints/BP_TimeManager.BP_TimeManager_C|GetCurrentTime (Variables|Default|GetTimeManagerRef)) (Variables|Default|GetSleepThreshold)) (not (Variables|Default|GetIsSleeping)))
          (Variables|Default|SetIsSleeping true)
          (bind _returnvalue (Class|InputDeviceLibrary|GetPlayerControllerfromInputDevice))
          (Input|SetIgnoreMoveInput (Game|GetPlayerController 0) true)
          (CameraFades|StartCameraFade :self (Variables|/Script/Engine.PlayerController|GetPlayerCameraManager _returnvalue) :ToAlpha 1.0 :Duration 1.5 :bShouldFadeAudio true :bHoldWhenFinished true)
          (Utilities|FlowControl|Delay 2.0)
          (bind _returnvalue_2 (UserInterface|CreateWidget "/Game/Blueprints/Newspaper/WBP_Newspaper.WBP_Newspaper_C"))
          (Variables|Default|SetNewsPaper _returnvalue_2)
          (UserInterface|Viewport|AddtoViewport (Variables|Default|GetNewsPaper) 9999)
          (bind _newparam (Default|News (Variables|Default|GetNewsPaper)))
          (if _newparam
            (Widget|RemovefromParent (Variables|Default|GetNewsPaper))
            (Default|SkiptoMorning (Variables|Default|GetTimeManagerRef))
            (bind _returnvalue_3 (Actor|GetActorOfClass "/Game/Blueprints/XP/BP_DayQuestLog.BP_DayQuestLog_C"))
            (Default|Who? _returnvalue_3)
            (CallFunction|Save)
            (Utilities|FlowControl|Delay 0.2)
            (Game|OpenLevel(byObjectReference) "/Game/Levels/Connor/Connor.Connor")
            (else
              (Utilities|FlowControl|DoOnce true) ; enters at Reset
            ))
          (else
            (Development|PrintString "It is too early to sleep." true true "(R=1.000000,G=0.000000,B=0.000000,A=1.000000)")
            (goto _label Reset)))))))

(event EventBeginPlay
  (bind _returnvalue (Actor|GetActorOfClass "/Game/LightingSYS/Lighting/Blueprints/BP_TimeManager.BP_TimeManager_C"))
  (Variables|Default|SetTimeManagerRef _returnvalue))

(event Collision|EventActorBeginOverlap
  (params (OtherActor :type Actor%20Object%20Reference)))

(event EventTick
  (params (DeltaSeconds :type Float%20%28single-precision%29)))

(fn ConstructionScript)