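; Medieval light actor that turns on at night and flickers like a flame in a draft.
; It binds to the first BP_TimeManager's day/night event, toggling the PointLight and actor Tick together.
; Tick uses randomly seeded Perlin noise to flicker around base intensity, with a slower-or-faster draft noise causing deep dips.
; FInterpTo feeds the light intensity, but CurrentSmoothedIntensity is never written back.
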(event Custom|ToggleLight
  (params (CurrentIsNight :type Boolean))
  (if CurrentIsNight
    (Rendering|SetVisibility (Variables|Default|GetPointLight) true false)
    (Actor|Tick|SetActorTickEnabled true)
    (else
      (Rendering|SetVisibility (Variables|Default|GetPointLight) false false)
      (Actor|Tick|SetActorTickEnabled false))))

(event EventBeginPlay
  (Variables|Default|SetRandomSeed (Math|Random|RandomFloatinRange 0.0 1e+03))
  (bind _outactors (Actor|GetAllActorsOfClass "/Game/LightingSYS/Lighting/Blueprints/BP_TimeManager.BP_TimeManager_C"))
  (bind _output_get (Variables|Default|SetTimeManagerRef (Utilities|Array|Get(acopy) _outactors)))
  (EventDispatchers|BindEventtoOnDayNightStateChanged _output_get (delegate Custom|ToggleLight))
  (CallFunction|ToggleLight (Variables|/Game/LightingSYS/Lighting/Blueprints/BP_TimeManager.BP_TimeManager_C|GetCurrentIsNight (Variables|Default|GetTimeManagerRef))))

(event Collision|EventActorBeginOverlap
  (params (OtherActor :type Actor%20Object%20Reference)))

(event EventTick
  (params (DeltaSeconds :type Float%20%28single-precision%29))
  (bind _returnvalue (Utilities|Time|GetGameTimeinSeconds))
  (bind _flickerspeed (Variables|Default|GetFlickerSpeed))
  (bind _baseintensity (Variables|Default|GetBaseIntensity))
  (bind _randomseed (Variables|Default|GetRandomSeed))
  (bind _returnvalue_2 (+ _returnvalue _randomseed))
  (bind _returnvalue_3 (* _returnvalue_2 _flickerspeed))
  (bind _returnvalue_4 (Class|KismetMathLibrary|PerlinNoise1D _returnvalue_3))
  (bind _returnvalue_5 (Math|Float|MapRangeClamped _returnvalue_4 -1.0 1.0 0.8 1.2))
  (bind _returnvalue_6 (* _returnvalue_5 _baseintensity))
  (Rendering|Components|Light|SetIntensity (Variables|Default|GetPointLight) (Math|Interpolation|FInterpTo (Variables|Default|GetCurrentSmoothedIntensity) (Math|Float|SelectFloat (* _returnvalue_6 0.02) _returnvalue_6 (< (Class|KismetMathLibrary|PerlinNoise1D (* (+ (Utilities|Time|GetGameTimeinSeconds) (Variables|Default|GetRandomSeed)) (Variables|Default|GetDraftSpeed))) -0.5)) (Utilities|Time|GetWorldDeltaSeconds) 1e+01)))

(fn ConstructionScript)