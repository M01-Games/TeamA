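; BP_TimeManager runs the game's day/night clock, advancing scaled time up to a freeze limit and counting days.
; Tick rotates the sun, tints it from a color curve and feeds the custom sky's Material Parameter Collection.
; It also updates a debug HUD, triggers deliveries at midnight rollover and broadcasts night state, though only while the night flag is already true.
; SkipToMorning jumps to 6:00, increments the day and reuses the sun update.
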(event Custom|SkipToMorning
  (bind _sunlight (Variables|Default|GetSunLight))
  (bind _lightcomponent (Variables|/Script/Engine.Light|GetLightComponent _sunlight))
  (bind _returnvalue (Math|Vector|GetForwardVector _lightcomponent))
  (bind _returnvalue_2 (* _returnvalue -1.0))
  ;[0.15 0.15 0.15 0.5] SKIP TO MORNING FUNC
  (Variables|Default|SetCurrentTime 6.0)
  (bind _result (Math|Integer|IncrementInt (Variables|Default|GetDayCount))
    (:%20%20
      ;[0.15 0.15 0.15 0.5] ROTATE SUN DEPENDANT ON TIME OF DAY
      (Transformation|SetActorRotation (Variables|Default|GetSunLight) (Math|Rotator|MakeRotator 0.0 (* (- (Variables|Default|GetCurrentTime) -6.0) 15.0) 0.0))
      ;[0.15 0.15 0.15 0.5] FOR THE CUSTOM SKY
      (Rendering|Material|SetVectorParameterValue "/Game/LightingSYS/Lighting/Sky/MPC_SkyData.MPC_SkyData" "SunDirection" (Math|Conversions|ToLinearColor(Vector) _returnvalue_2) :!class /Script/Engine.KismetMaterialLibrary)
      (Rendering|Material|SetScalarParameterValue "/Game/LightingSYS/Lighting/Sky/MPC_SkyData.MPC_SkyData" "SunHeight" (Math|Float|MapRangeClamped (.Z (Math|Vector|BreakVector _returnvalue_2)) -1.0 1.0 0.0 1.0) :!class /Script/Engine.KismetMaterialLibrary)
      (Utilities|FlowControl|Sequence
        (:then_0
          (Rendering|Components|Light|SetLightColor (Variables|/Script/Engine.Light|GetLightComponent (Variables|Default|GetSunLight)) (Math|Curves|GetLinearColorValue (Variables|Default|GetHorizonCurve) (/ (Variables|Default|GetCurrentTime) 24.0)) false)
          (Rendering|Material|SetVectorParameterValue "/Game/LightingSYS/Lighting/Sky/MPC_SkyData.MPC_SkyData" "SunColor" (Math|Curves|GetLinearColorValue (Variables|Default|GetHorizonCurve) (/ (Variables|Default|GetCurrentTime) 24.0)) :!class /Script/Engine.KismetMaterialLibrary))
        (:then_1
          ;[0.15 0.15 0.15 0.5] UPDATE DEBUG INFO
          (Default|UpdateDebugInfo (Variables|Default|GetMyHUD) (Variables|Default|GetCurrentTime) (Variables|Default|GetDayCount)))
        (:then_2
          ;[0.15 0.15 0.15 0.5] NIGHT CHECK FOR LIGHTS
          (if (!= false (Variables|Default|GetCurrentIsNight))
            (bind _output_get (Variables|Default|SetCurrentIsNight (or (> (Variables|Default|GetCurrentTime) 18.0) (< (Variables|Default|GetCurrentTime) 6.0))))
            (Default|CallOnDayNightStateChanged _output_get)))))))

(event EventBeginPlay
  ;[0.15 0.15 0.15 0.5] SETUP DEBUG WIDGET
  (bind _returnvalue (UserInterface|CreateWidget "/Game/LightingSYS/Lighting/Blueprints/W_DebugHUD.W_DebugHUD_C"))
  (bind _output_get (Variables|Default|SetMyHUD _returnvalue))
  (UserInterface|Viewport|AddtoViewport _output_get 0))

(event Collision|EventActorBeginOverlap
  (params (OtherActor :type Actor%20Object%20Reference)))

(event EventTick
  (params (DeltaSeconds :type Float%20%28single-precision%29))
  (bind _sunlight (Variables|Default|GetSunLight))
  (bind _lightcomponent (Variables|/Script/Engine.Light|GetLightComponent _sunlight))
  (bind _returnvalue (Math|Vector|GetForwardVector _lightcomponent))
  (bind _returnvalue_2 (* _returnvalue -1.0))
  ;[0.15 0.15 0.15 0.5] CALCULATE CURRENT TIME USING EVENT TICK
  (if (< (+ (* DeltaSeconds (Variables|Default|GetTimeSpeed)) (Variables|Default|GetCurrentTime)) (Variables|Default|GetFreezeTime))
    (Variables|Default|SetCurrentTime (+ (* DeltaSeconds (Variables|Default|GetTimeSpeed)) (Variables|Default|GetCurrentTime)))
    (if (>= (Variables|Default|GetCurrentTime) 24.0)
      ;[0.15 0.15 0.15 0.5] ADD TO DAY COUNT WHEN CLOCK GOES OVER 24
      (Variables|Default|SetCurrentTime 0.0)
      (bind _result (Math|Integer|IncrementInt (Variables|Default|GetDayCount))
        (:%20%20
          (Development|PrintString "NEW DAY!" true true "(R=1.000000,G=0.000000,B=0.000000,A=1.000000)")
          (CallFunction|FindDelivery))))
    ;[0.15 0.15 0.15 0.5] ROTATE SUN DEPENDANT ON TIME OF DAY
    (Transformation|SetActorRotation (Variables|Default|GetSunLight) (Math|Rotator|MakeRotator 0.0 (* (- (Variables|Default|GetCurrentTime) -6.0) 15.0) 0.0))
    ;[0.15 0.15 0.15 0.5] FOR THE CUSTOM SKY
    (Rendering|Material|SetVectorParameterValue "/Game/LightingSYS/Lighting/Sky/MPC_SkyData.MPC_SkyData" "SunDirection" (Math|Conversions|ToLinearColor(Vector) _returnvalue_2) :!class /Script/Engine.KismetMaterialLibrary)
    (Rendering|Material|SetScalarParameterValue "/Game/LightingSYS/Lighting/Sky/MPC_SkyData.MPC_SkyData" "SunHeight" (Math|Float|MapRangeClamped (.Z (Math|Vector|BreakVector _returnvalue_2)) -1.0 1.0 0.0 1.0) :!class /Script/Engine.KismetMaterialLibrary)
    (Utilities|FlowControl|Sequence
      (:then_0
        (Rendering|Components|Light|SetLightColor (Variables|/Script/Engine.Light|GetLightComponent (Variables|Default|GetSunLight)) (Math|Curves|GetLinearColorValue (Variables|Default|GetHorizonCurve) (/ (Variables|Default|GetCurrentTime) 24.0)) false)
        (Rendering|Material|SetVectorParameterValue "/Game/LightingSYS/Lighting/Sky/MPC_SkyData.MPC_SkyData" "SunColor" (Math|Curves|GetLinearColorValue (Variables|Default|GetHorizonCurve) (/ (Variables|Default|GetCurrentTime) 24.0)) :!class /Script/Engine.KismetMaterialLibrary))
      (:then_1
        ;[0.15 0.15 0.15 0.5] UPDATE DEBUG INFO
        (Default|UpdateDebugInfo (Variables|Default|GetMyHUD) (Variables|Default|GetCurrentTime) (Variables|Default|GetDayCount)))
      (:then_2
        ;[0.15 0.15 0.15 0.5] NIGHT CHECK FOR LIGHTS
        (if (!= false (Variables|Default|GetCurrentIsNight))
          (bind _output_get (Variables|Default|SetCurrentIsNight (or (> (Variables|Default|GetCurrentTime) 18.0) (< (Variables|Default|GetCurrentTime) 6.0))))
          (Default|CallOnDayNightStateChanged _output_get))))
    (else
      (Variables|Default|SetCurrentTime (Variables|Default|GetFreezeTime)))))

(fn ConstructionScript)

(fn FindDelivery
  (bind _returnvalue (Actor|GetActorOfClass "/Game/Blueprints/Workstations/Ordering/UI/DeliveryPoint.DeliveryPoint_C"))
  (Default|Deliver _returnvalue))